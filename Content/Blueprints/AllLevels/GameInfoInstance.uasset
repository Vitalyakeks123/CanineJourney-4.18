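; Game-wide info instance that manages the main, play, pause, options and death screens, plus player settings.
; Widgets are created once and cached, with index-driven hover, select and left/right events for navigation without mouse clicks.
; Character or dog death opens the death screen after a short delay, while pause and options freeze play through zero time dilation.
; Music settings act on every AmbientSound actor; two E-key options are simple toggles.
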(event Custom|SelectOptions
  ;[1 1 1] Select options Widget
  (if (Variables|OptionsWidget|GetisOptionsWidget)
    (switch int (Variables|OptionsWidget|GetOptionsWidgetIndex)
      (:0
        (CallFunction|OptionsChangeMusicon))
      (:2
        (CallFunction|OpenMenuWidget)
        (CallFunction|CloseOptionsWidget)))))

(event Custom|OptionsTurnRight
  ;[1 1 1] Options Turn Right
  (if (Variables|OptionsWidget|GetisOptionsWidget)
    (switch int (Variables|OptionsWidget|GetOptionsWidgetIndex)
      (:0
        (CallFunction|OptionsChangeMusicon))
      (:1
        (CallFunction|OptionsChangeMusicVolume 0.1)))))

(event Custom|DieCharacter
  ;[1 1 1] Death Handlers
  (Development|PrintString "You Died!")
  (Utilities|FlowControl|Delay 0.5)
  (CallFunction|OpenDeathWindow))

(event Custom|Close%20Main%20Menu
  (bind _mainmenuwidget (Variables|Default|GetMainMenuWidget))
  ;[1 1 1] Close Main Menu
  (Utilities|IsValid _mainmenuwidget
    (:Is%20Valid
      (Widget|RemovefromParent _mainmenuwidget))))

(event Custom|DeathWidgetHover
  (bind _deathwidget (Variables|Default|GetDeathWidget))
  ;[1 1 1] Death Widget Hover
  (if (Variables|DeathWidget|GetisDeadthWidget)
    (switch int (Variables|DeathWidget|GetDeathWidgetIndex)
      (:0
        (Default|HoverRestart _deathwidget))
      (:1
        (Default|HoverMainMenu _deathwidget))
      (:2
        (Default|HoverExit _deathwidget)))))

(event Custom|OpenOptionsWidget
  ;[1 1 1] Open options Widget
  (Utilities|IsValid (Variables|Default|GetOptionsWidget)
    (:Is%20Valid
      (UserInterface|Viewport|AddtoViewport (Variables|Default|GetOptionsWidget) 0))
    (:Is%20Not%20Valid
      (bind _returnvalue (UserInterface|CreateWidget "/Game/UI/OptionsWidget.OptionsWidget_C"))
      (bind _output_get (Variables|Default|SetOptionsWidget _returnvalue))
      (UserInterface|Viewport|AddtoViewport _output_get 0)))
  (Variables|OptionsWidget|SetOptionsWidgetIndex 0)
  (Variables|OptionsWidget|SetisOptionsWidget true)
  (CallFunction|HoverOptions)
  (Utilities|Time|SetGlobalTimeDilation 0.0))

(event Custom|OptionsChangeMusicVolume
  (params (delta :type Float%20%28single-precision%29))
  ;[1 1 1] Options change music volume [0;1]
  (Variables|Options|SetMusicVolume (Math|Float|Clamp(Float) (+ (Variables|Options|GetMusicVolume) delta) 0.1))
  (bind _outactors (Actor|GetAllActorsOfClass "/Script/Engine.AmbientSound"))
  (for _array_element _outactors
    (Audio|Components|Audio|SetVolumeMultiplier (Variables|/Script/Engine.AmbientSound|GetAudioComponent _array_element) (Variables|Options|GetMusicVolume) :!class /Script/Engine.AudioComponent)
    (Default|VolumeChange (Variables|Default|GetOptionsWidget))))

(event Custom|DieDog
  ;[1 1 1] Death Handlers
  (Development|PrintString "Dog died")
  (bind _ashuman_character (Utilities|Casting|CastToHumanCharacter (Game|GetPlayerCharacter 0)))
  (Variables|/Game/Blueprints/Characters/HumanCharacter.HumanCharacter_C|SetisDead _ashuman_character true)
  (Utilities|FlowControl|Delay 0.5)
  (CallFunction|OpenDeathWindow))

(event Custom|OpenDeathWindow
  ;[1 1 1] Open Death Widget
  (Utilities|IsValid (Variables|Default|GetDeathWidget)
    (:Is%20Valid
      (UserInterface|Viewport|AddtoViewport (Variables|Default|GetDeathWidget) 0))
    (:Is%20Not%20Valid
      (bind _returnvalue (UserInterface|CreateWidget "/Game/UI/DeathWidget.DeathWidget_C"))
      (bind _output_get (Variables|Default|SetDeathWidget _returnvalue))
      (UserInterface|Viewport|AddtoViewport _output_get 0)))
  (Variables|DeathWidget|SetisDeadthWidget true)
  (Variables|DeathWidget|SetDeathWidgetIndex 0)
  (CallFunction|DeathWidgetHover))

(event Custom|DeathWidgetSelect
  ;[1 1 1] Death Widget Select
  (if (Variables|DeathWidget|GetisDeadthWidget)
    (switch int (Variables|DeathWidget|GetDeathWidgetIndex)
      (:0
        (bind _returnvalue (Game|GetCurrentLevelName true))
        (Game|OpenLevel(byName) (Utilities|String|StringToName _returnvalue))
        (CallFunction|CloseDeathWidget))
      (:1
        (Game|OpenLevel(byName) "MainMenu")
        (CallFunction|CloseDeathWidget))
      (:2
        (Game|QuitGame 0 "Quit")))))

(event Custom|ExitGame
  ;[1 1 1] Exit the game
  (Game|QuitGame 0 "Quit"))

(event Custom|OpenMainMenu
  ;[1 1 1] Open Main Menu
  (Utilities|IsValid (Variables|Default|GetMainMenuWidget)
    (:Is%20Valid
      (UserInterface|Viewport|AddtoViewport (Variables|Default|GetMainMenuWidget) 0))
    (:Is%20Not%20Valid
      (bind _returnvalue (UserInterface|CreateWidget "/Game/UI/MainMenuWidget.MainMenuWidget_C"))
      (bind _output_get (Variables|Default|SetMainMenuWidget _returnvalue))
      (UserInterface|Viewport|AddtoViewport _output_get 0)))
  (Variables|/Script/Engine.PlayerController|SetbShowMouseCursor (Game|GetPlayerController 0) false))

(event Custom|OpenMenuWidget
  ;[1 1 1] Open menu Widget
  (Utilities|IsValid (Variables|Default|GetMenuWidget)
    (:Is%20Valid
      (UserInterface|Viewport|AddtoViewport (Variables|Default|GetMenuWidget) 0))
    (:Is%20Not%20Valid
      (bind _returnvalue (UserInterface|CreateWidget "/Game/UI/MenuWidget.MenuWidget_C"))
      (bind _output_get (Variables|Default|SetMenuWidget _returnvalue))
      (UserInterface|Viewport|AddtoViewport _output_get 0)))
  (Variables|MenuWidget|SetMenuWidgetIndex 0)
  (Variables|MenuWidget|SetisMenuWidget true)
  (CallFunction|MenuHover)
  (Utilities|Time|SetGlobalTimeDilation 0.0))

(event Custom|CloseDeathWidget
  (bind _deathwidget (Variables|Default|GetDeathWidget))
  ;[1 1 1] Close Death Widget
  (Utilities|IsValid _deathwidget
    (:Is%20Valid
      (Widget|RemovefromParent _deathwidget)
      (Variables|DeathWidget|SetisDeadthWidget false))))

(event Custom|CloseOptionsWidget
  (bind _optionswidget (Variables|Default|GetOptionsWidget))
  ;[1 1 1] Close options Widget
  (Utilities|IsValid _optionswidget
    (:Is%20Valid
      (Widget|RemovefromParent _optionswidget)
      (Variables|OptionsWidget|SetisOptionsWidget false))))

(event Custom|OptionsChangeMusicOn
  ;[1 1 1] Options turn music on/off
  (if (Variables|Options|GetisMusicOn?)
    (Variables|Options|SetisMusicOn? false)
    (bind _outactors (Actor|GetAllActorsOfClass "/Script/Engine.AmbientSound"))
    (for _array_element _outactors
      (Class|AudioComponent|SetPaused (Variables|/Script/Engine.AmbientSound|GetAudioComponent _array_element) true)
      (Default|MusicChange (Variables|Default|GetOptionsWidget)))
    (else
      (Variables|Options|SetisMusicOn? true)
      (bind _outactors_2 (Actor|GetAllActorsOfClass "/Script/Engine.AmbientSound"))
      (for _array_element_2 _outactors_2
        (Class|AudioComponent|SetPaused (Variables|/Script/Engine.AmbientSound|GetAudioComponent _array_element_2) false)
        (Default|MusicChange (Variables|Default|GetOptionsWidget))))))

(event Custom|HoverOptions
  (bind _optionswidget (Variables|Default|GetOptionsWidget))
  ;[1 1 1] Hover menu widget
  (if (Variables|OptionsWidget|GetisOptionsWidget)
    (switch int (Variables|OptionsWidget|GetOptionsWidgetIndex)
      (:0
        (Default|HoverMusic _optionswidget))
      (:1
        (Default|HoverVolume _optionswidget))
      (:2
        (Default|HoverBack _optionswidget)))))

(event Custom|OptionsTurnLeft
  ;[1 1 1] Options Turn Left
  (if (Variables|OptionsWidget|GetisOptionsWidget)
    (switch int (Variables|OptionsWidget|GetOptionsWidgetIndex)
      (:0
        (CallFunction|OptionsChangeMusicon))
      (:1
        (CallFunction|OptionsChangeMusicVolume -0.1)))))

(event Custom|OptionsChangeHoldE
  ;[1 1 1] Options Hold E
  (if (Variables|Options|GetoptionsHoldE)
    (Variables|Options|SetoptionsHoldE false)
    (else
      (Variables|Options|SetoptionsHoldE true))))

(event Custom|OptionsChangeCloseE
  ;[1 1 1] Options Close E After Throw
  (if (Variables|Options|GetoptionsCloseE)
    (Variables|Options|SetoptionsCloseE false)
    (else
      (Variables|Options|SetoptionsCloseE true))))

(event Custom|CloseMenuWidget
  (bind _menuwidget (Variables|Default|GetMenuWidget))
  ;[1 1 1] Close menu Widget
  (Utilities|IsValid _menuwidget
    (:Is%20Valid
      (Widget|RemovefromParent _menuwidget)
      (Variables|MenuWidget|SetisMenuWidget false)
      (Utilities|Time|SetGlobalTimeDilation 1.0)
      (bind _ashuman_character (Utilities|Casting|CastToHumanCharacter (Game|GetPlayerCharacter 0)))
      (Default|CloseMenu _ashuman_character))))

(event Custom|OpenPlay
  ;[1 1 1] Open Play Widget
  (Utilities|IsValid (Variables|Default|GetPlayWidget)
    (:Is%20Valid
      (UserInterface|Viewport|AddtoViewport (Variables|Default|GetPlayWidget) 0))
    (:Is%20Not%20Valid
      (bind _returnvalue (UserInterface|CreateWidget "/Game/UI/PlayWidget.PlayWidget_C"))
      (bind _output_get (Variables|Default|SetPlayWidget _returnvalue))
      (UserInterface|Viewport|AddtoViewport _output_get 0))))

(event Custom|MenuHover
  (bind _menuwidget (Variables|Default|GetMenuWidget))
  ;[1 1 1] Hover menu widget
  (if (Variables|MenuWidget|GetisMenuWidget)
    (switch int (Variables|MenuWidget|GetMenuWidgetIndex)
      (:0
        (Default|HoverResume _menuwidget))
      (:1
        (Default|HoverOptions _menuwidget))
      (:2
        (Default|HoverRestart _menuwidget))
      (:3
        (Default|HoverMainMenu _menuwidget))
      (:4
        (Default|HoverExit _menuwidget)))))

(event Custom|SelectMenu
  ;[1 1 1] Select menu Widget
  (if (and (Variables|MenuWidget|GetisMenuWidget) (not (Variables|OptionsWidget|GetisOptionsWidget)))
    (switch int (Variables|MenuWidget|GetMenuWidgetIndex)
      (:0
        (CallFunction|CloseMenuWidget))
      (:1
        (CallFunction|CloseMenuWidget)
        (CallFunction|OpenOptionsWidget))
      (:2
        (CallFunction|CloseMenuWidget)
        (bind _returnvalue (Game|GetCurrentLevelName true))
        (Game|OpenLevel(byName) (Utilities|String|StringToName _returnvalue)))
      (:3
        (Game|OpenLevel(byName) "MainMenu")
        (CallFunction|CloseMenuWidget))
      (:4
        (Game|QuitGame 0 "Quit")))))

(event Custom|ClosePlayWidget
  (bind _playwidget (Variables|Default|GetPlayWidget))
  ;[1 1 1] Close Play Widget
  (Utilities|IsValid _playwidget
    (:Is%20Valid
      (Widget|RemovefromParent _playwidget))))