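; Player controller for the main menu that drives keyboard navigation through the main screen and level-select screen.
; BeginPlay opens the menu via GameInfoInstance, then W/S or arrow keys cycle HoveredIndex with wraparound per MenuState, updating widget highlights through HoverButton.
; Enter or Space acts on the selection: switching screens, exiting the game or opening one of eight levels by name.
; Options can be highlighted but has no select action.
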(event Custom|HoverButton
  (bind _gameinfoinstance (Variables|Default|GetGameInfoInstance))
  (bind _gameinfoinstance_2 (Variables|Default|GetGameInfoInstance))
  (bind _mainmenuwidget (Variables|/Game/Blueprints/AllLevels/GameInfoInstance.GameInfoInstance_C|GetMainMenuWidget _gameinfoinstance_2))
  (bind _playwidget (Variables|/Game/Blueprints/AllLevels/GameInfoInstance.GameInfoInstance_C|GetPlayWidget _gameinfoinstance))
  ;[1 1 1] HoverButton
  (switch int (Variables|Default|GetMenuState)
    (:0
      (switch int (Variables|Default|GetHoveredIndex)
        (:0
          (Default|HoverPlay _mainmenuwidget))
        (:1
          (Default|HoverOptions _mainmenuwidget))
        (:2
          (Default|HoverExit _mainmenuwidget))))
    (:1
      (switch int (Variables|Default|GetHoveredIndex)
        (:0
          (Default|SelectLevel1 _playwidget))
        (:1
          (Default|SelectLevel2 _playwidget))
        (:2
          (Default|SelectLevel3 _playwidget))
        (:3
          (Default|SelectLevel4 _playwidget))
        (:4
          (Default|SelectLevel5 _playwidget))
        (:5
          (Default|SelectLevel6 _playwidget))
        (:6
          (Default|SelectLevel7 _playwidget))
        (:7
          (Default|SelectLevel8 _playwidget))
        (:8
          (Default|SelectBack _playwidget))))))

(event EventBeginPlay
  (bind _asgame_info_instance (Utilities|Casting|CastToGameInfoInstance (Game|GetGameInstance)))
  (bind _output_get (Variables|Default|SetGameInfoInstance _asgame_info_instance))
  (Default|OpenMainMenu _output_get)
  (Variables|Default|SetHoveredIndex 0)
  (CallFunction|HoverButton))

(event EventTick
  (params (DeltaSeconds :type Float%20%28single-precision%29)))

(event Input|KeyboardEvents|S
  (params (Key :type Key%20Structure))
  ;[1 1 1] Down
  (:Pressed
    (bind _result (Math|Integer|IncrementInt (Variables|Default|GetHoveredIndex))
      (:%20%20
        (if (>= _result (Utilities|Array|Get(acopy) (Variables|Default|GetMaxButtons) (Variables|Default|GetMenuState)))
          (Variables|Default|SetHoveredIndex 0))
        (CallFunction|HoverButton)))))

(event Input|KeyboardEvents|Down
  (params (Key :type Key%20Structure))
  ;[1 1 1] Down
  (:Pressed
    (bind _result (Math|Integer|IncrementInt (Variables|Default|GetHoveredIndex))
      (:%20%20
        (if (>= _result (Utilities|Array|Get(acopy) (Variables|Default|GetMaxButtons) (Variables|Default|GetMenuState)))
          (Variables|Default|SetHoveredIndex 0))
        (CallFunction|HoverButton)))))

(event Input|KeyboardEvents|Enter
  (params (Key :type Key%20Structure))
  (bind _gameinfoinstance (Variables|Default|GetGameInfoInstance))
  ;[1 1 1] Select
  (:Pressed
    (switch int (Variables|Default|GetMenuState)
      (:0
        (switch int (Variables|Default|GetHoveredIndex)
          (:0
            (Default|CloseMainMenu _gameinfoinstance)
            (Default|OpenPlay _gameinfoinstance)
            (Variables|Default|SetHoveredIndex 0)
            (Variables|Default|SetMenuState 1)
            (CallFunction|HoverButton))
          (:2
            (Default|ExitGame _gameinfoinstance))))
      (:1
        (Default|ClosePlayWidget (Variables|Default|GetGameInfoInstance))
        (switch int (Variables|Default|GetHoveredIndex)
          (:0
            (Game|OpenLevel(byName) "pervii_yroven1_bez_lishnego_musora"))
          (:1
            (Game|OpenLevel(byName) "misha_3"))
          (:2
            (Game|OpenLevel(byName) "misha_4"))
          (:3
            (Game|OpenLevel(byName) "misha_1"))
          (:4
            (Game|OpenLevel(byName) "misha_2_2"))
          (:5
            (Game|OpenLevel(byName) "misha_5"))
          (:6
            (Game|OpenLevel(byName) "misha_6"))
          (:7
            (Game|OpenLevel(byName) "misha_7"))
          (:8
            (Default|OpenMainMenu (Variables|Default|GetGameInfoInstance))
            (Variables|Default|SetHoveredIndex 0)
            (Variables|Default|SetMenuState 0)
            (CallFunction|HoverButton)))))))

(event Input|KeyboardEvents|SpaceBar
  (params (Key :type Key%20Structure))
  (bind _gameinfoinstance (Variables|Default|GetGameInfoInstance))
  ;[1 1 1] Select
  (:Pressed
    (switch int (Variables|Default|GetMenuState)
      (:0
        (switch int (Variables|Default|GetHoveredIndex)
          (:0
            (Default|CloseMainMenu _gameinfoinstance)
            (Default|OpenPlay _gameinfoinstance)
            (Variables|Default|SetHoveredIndex 0)
            (Variables|Default|SetMenuState 1)
            (CallFunction|HoverButton))
          (:2
            (Default|ExitGame _gameinfoinstance))))
      (:1
        (Default|ClosePlayWidget (Variables|Default|GetGameInfoInstance))
        (switch int (Variables|Default|GetHoveredIndex)
          (:0
            (Game|OpenLevel(byName) "pervii_yroven1_bez_lishnego_musora"))
          (:1
            (Game|OpenLevel(byName) "misha_3"))
          (:2
            (Game|OpenLevel(byName) "misha_4"))
          (:3
            (Game|OpenLevel(byName) "misha_1"))
          (:4
            (Game|OpenLevel(byName) "misha_2_2"))
          (:5
            (Game|OpenLevel(byName) "misha_5"))
          (:6
            (Game|OpenLevel(byName) "misha_6"))
          (:7
            (Game|OpenLevel(byName) "misha_7"))
          (:8
            (Default|OpenMainMenu (Variables|Default|GetGameInfoInstance))
            (Variables|Default|SetHoveredIndex 0)
            (Variables|Default|SetMenuState 0)
            (CallFunction|HoverButton)))))))

(event Input|KeyboardEvents|W
  (params (Key :type Key%20Structure))
  ;[1 1 1] Up
  (:Pressed
    (bind _result (Math|Integer|DecrementInt (Variables|Default|GetHoveredIndex))
      (:%20%20
        (if (<= _result -1)
          (Variables|Default|SetHoveredIndex (- (Utilities|Array|Get(acopy) (Variables|Default|GetMaxButtons) (Variables|Default|GetMenuState)) 1)))
        (CallFunction|HoverButton)))))

(event Input|KeyboardEvents|Up
  (params (Key :type Key%20Structure))
  ;[1 1 1] Up
  (:Pressed
    (bind _result (Math|Integer|DecrementInt (Variables|Default|GetHoveredIndex))
      (:%20%20
        (if (<= _result -1)
          (Variables|Default|SetHoveredIndex (- (Utilities|Array|Get(acopy) (Variables|Default|GetMaxButtons) (Variables|Default|GetMenuState)) 1)))
        (CallFunction|HoverButton)))))

(fn ConstructionScript)