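; Ladder actor that lets a HumanCharacter climb while inside its trigger box.
; Box begin overlap sets the character's CanClimb flag.
; On end overlap, it checks every Ladder actor in the level and only clears CanClimb and calls ClimbingEnd when the character overlaps none, so moving between adjacent ladders keeps climbing active.
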(event OnComponentBeginOverlap(Box)
  (params (OverlappedComponent :type Primitive%20Component%20Object%20Reference) (OtherActor :type Actor%20Object%20Reference) (OtherComp :type Primitive%20Component%20Object%20Reference) (OtherBodyIndex :type Integer) (bFromSweep :type Boolean) (SweepResult :type Hit%20Result%20Structure%20%28by%20ref%29))
  (bind _ashuman_character (Utilities|Casting|CastToHumanCharacter OtherActor))
  (Variables|/Game/Blueprints/Characters/HumanCharacter.HumanCharacter_C|SetCanClimb? _ashuman_character true))

(event OnComponentEndOverlap(Box)
  (params (OverlappedComponent :type Primitive%20Component%20Object%20Reference) (OtherActor :type Actor%20Object%20Reference) (OtherComp :type Primitive%20Component%20Object%20Reference) (OtherBodyIndex :type Integer))
  (bind _ashuman_character (Utilities|Casting|CastToHumanCharacter OtherActor))
  (Variables|Default|SetisOverlap false)
  (bind _outactors (Actor|GetAllActorsOfClass "Ladder_C"))
  (for _array_element _outactors
    (if (Collision|IsOverlappingActor _ashuman_character _array_element :!class /Script/Engine.Actor)
      (Variables|Default|SetisOverlap true)))
  (if (not (Variables|Default|GetisOverlap))
    (Variables|/Game/Blueprints/Characters/HumanCharacter.HumanCharacter_C|SetCanClimb? _ashuman_character false)
    (Default|ClimbingEnd _ashuman_character)))

(event EventBeginPlay)

(event Collision|EventActorBeginOverlap
  (params (OtherActor :type Actor%20Object%20Reference)))

(event EventTick
  (params (DeltaSeconds :type Float%20%28single-precision%29)))

(fn ConstructionScript)