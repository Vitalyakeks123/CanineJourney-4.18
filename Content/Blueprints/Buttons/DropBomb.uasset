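; DropBomb is an actor that periodically spawns bombs at its Arrow component.
; A Tick-driven countdown starts at FirstDelay, then resets to Interval each time it reaches zero and fires a spawn.
; Each bomb always spawns regardless of collision and receives the arrow's rotation as its move rotation, along with the spawner's Speed.
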(event EventBeginPlay
  (Variables|Default|SetTime (Variables|Bomb|GetFirstDelay)))

(event EventTick
  (params (DeltaSeconds :type Float%20%28single-precision%29))
  (CallFunction|ChangeTime DeltaSeconds))

(fn ConstructionScript)

(fn ChangeTime
  (params (Delta%20Time :type Float%20%28single-precision%29))
  (bind _output_get (Variables|Default|SetTime (Math|Float|Clamp(Float) (- (Variables|Default|GetTime) Delta%20Time) 0.0 123.0)))
  (if (<= _output_get 0.0)
    (Variables|Default|SetTime (Variables|Bomb|GetInterval))
    (CallFunction|SpawnBomb)))

(fn SpawnBomb
  (bind _arrow (Variables|Default|GetArrow))
  (bind _returnvalue (Transformation|GetWorldTransform _arrow))
  (bind _returnvalue_2 (Game|SpawnActorfromClass "/Game/Blueprints/Buttons/DropBomb/Bomb.Bomb_C" (Math|Transform|MakeTransform (.location _returnvalue) "0, 0, 0" "1,1,1") "AlwaysSpawn" 0 0))
  (Utilities|IsValid _returnvalue_2
    (:Is%20Valid
      (Variables|/Game/Blueprints/Buttons/DropBomb/Bomb.Bomb_C|SetMoveRotation _returnvalue_2 (.rotation _returnvalue))
      (Variables|/Game/Blueprints/Buttons/DropBomb/Bomb.Bomb_C|SetSpeed _returnvalue_2 (Variables|Bomb|GetSpeed)))))