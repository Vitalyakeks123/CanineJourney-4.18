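; Paper2D gate actor with Open and Close events that teleport it between OpenedLocation and the location captured at start.
; First opening plays the flipbook once, disables sprite and box collision, and plays a sound.
; Paired DoOnce nodes re-arm each other so sounds don't repeat; Close leaves collision and animation untouched.
; Construction script applies the configurable sprite, flipbook, offset, rotation and box size.
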(event Custom|Open
  (bind _paperflipbook (Variables|Default|GetPaperFlipbook))
  (Transformation|Teleport (Variables|Default|GetOpenedLocation) (Transformation|GetActorRotation))
  (Utilities|FlowControl|DoOnce false
    (:Completed
      (Audio|Components|Audio|Play _paperflipbook)
      (Components|Timeline|SetPlayRate _paperflipbook 1.0)
      (Components|Timeline|SetLooping _paperflipbook false)
      (Collision|SetCollisionEnabled (Variables|Default|GetPaperSprite) "NoCollision")
      (Collision|SetCollisionEnabled (Variables|Default|GetBox) "NoCollision")
      (Audio|PlaySound2D "/Game/StarterContent/Audio/zvuki_dlya_igri/dveriotkritie.dveriotkritie")
      (Utilities|FlowControl|DoOnce false) ; enters at Reset
    )))

(event Custom|Close
  (bind _paperflipbook (Variables|Default|GetPaperFlipbook))
  (Transformation|Teleport (Variables|Default|GetClosedLocation) (Transformation|GetActorRotation))
  (Utilities|FlowControl|DoOnce false
    (:Completed
      (Audio|PlaySound2D "/Game/StarterContent/Audio/zvuki_dlya_igri/dverizakritie.dverizakritie")
      (Utilities|FlowControl|DoOnce false) ; enters at Reset
    )))

(event EventBeginPlay
  (Variables|Default|SetClosedLocation (Transformation|GetActorLocation)))

(event EventTick
  (params (DeltaSeconds :type Float%20%28single-precision%29)))

(fn ConstructionScript
  (bind _papersprite (Variables|Default|GetPaperSprite))
  (bind _paperflipbook (Variables|Default|GetPaperFlipbook))
  (bind _gaterotation (Variables|Door|GetGateRotation))
  (bind _gateoffset (Variables|Door|GetGateOffset))
  (Variables|Default|SetClosedLocation (Transformation|GetActorLocation))
  (Rendering|Components|Sprite|SetSprite _papersprite (Variables|Door|GetGateSprite))
  (Sprite|SetFlipbook _paperflipbook (Variables|Door|GetGateAnimation))
  (Transformation|SetRelativeTransform _papersprite (Math|Transform|MakeTransform (Math|Vector|MakeVector (.x _gateoffset) 7.0 (.z _gateoffset)) _gaterotation (Transformation|GetWorldScale _papersprite)) false false)
  (Transformation|SetRelativeTransform _paperflipbook (Math|Transform|MakeTransform (Math|Vector|MakeVector (.x _gateoffset) -5.0 (.z _gateoffset)) _gaterotation (Transformation|GetWorldScale _paperflipbook)) false false)
  (Components|Box|SetBoxExtent (Variables|Default|GetBox) (Variables|Door|GetGateSize) true))