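; Spinner hazard: a rotating arm of spheres that damages the player character or their dog on overlap.
; The construction script builds the arm by chaining Number sphere components upward from RootCircle, spaced by Radius.
; Each tick, Spin steps a wrapping Angle by Speed, with IsAlarm setting the direction, and derives actor rotation from a look-at toward a Y-axis-rotated vector.
; DamageCheck then applies damage every overlapping frame, checking the player before the dog.
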(event EventBeginPlay
  (Development|PrintString (Utilities|String|ToString(Float) (Variables|SpinnerStats|GetAngle))))

(event Collision|EventActorBeginOverlap
  (params (OtherActor :type Actor%20Object%20Reference)))

(event EventTick
  (params (DeltaSeconds :type Float%20%28single-precision%29))
  (CallFunction|Spin)
  (CallFunction|DamageCheck))

(fn ConstructionScript
  (Components|Sphere|SetSphereRadius (Variables|Default|GetRootCircle) (Variables|SpinnerStats|GetRadius) true)
  (Utilities|Array|AddUnique (Variables|Default|GetParts) (Variables|Default|GetRootCircle))
  (for _index (range 1 (Variables|SpinnerStats|GetNumber))
    (LocalVariables|SetCurrentIndex _index)
    (bind _returnvalue (AddComponent|AddSphereComponent false (Math|Transform|MakeTransform (Math|Vector|MakeVector 0.0 0.0 (* (Variables|SpinnerStats|GetRadius) 2.0 (Math|Conversions|ToFloat(Integer) (LocalVariables|GetCurrentIndex)))) "0, 0, 0" "1,1,1")))
    (Utilities|Array|AddUnique (Variables|Default|GetParts) _returnvalue)
    (Components|Sphere|SetSphereRadius _returnvalue (Variables|SpinnerStats|GetRadius) true)
    (Transformation|AttachComponentToComponent _returnvalue (Utilities|Array|Get(acopy) (Variables|Default|GetParts) (- (LocalVariables|GetCurrentIndex) 1)) "None" "KeepWorld" "SnapToTarget" "KeepRelative" true)
    (Development|SetHiddeninGame _returnvalue false false)))

(fn Spin
  (bind _returnvalue (Transformation|GetActorLocation))
  (Utilities|FlowControl|Sequence
    (:then_0
      (if (Variables|SpinnerStats|GetisAlarm)
        (Variables|SpinnerStats|SetAngle (Math|Float|Clamp(Float) (+ (Variables|SpinnerStats|GetAngle) (* (Variables|SpinnerStats|GetSpeed) (Utilities|Time|GetWorldDeltaSeconds) 3e+01)) -1.0 3.6e+02))
        (else
          (Variables|SpinnerStats|SetAngle (Math|Float|Clamp(Float) (- (Variables|SpinnerStats|GetAngle) (* (Variables|SpinnerStats|GetSpeed) (Utilities|Time|GetWorldDeltaSeconds) 3e+01)) -1.0 3.6e+02)))))
    (:then_1
      (Utilities|FlowControl|Sequence
        (:then_0
          (if (>= (Variables|SpinnerStats|GetAngle) 3.6e+02)
            (Variables|SpinnerStats|SetAngle 0.0)))
        (:then_1
          (if (< (Variables|SpinnerStats|GetAngle) 0.0)
            (Variables|SpinnerStats|SetAngle 3.6e+02)))
        (:then_2
          (Transformation|SetActorRotation (Math|Rotator|MakeRotator (.Yaw (Math|Rotator|BreakRotator (Math|Rotator|FindLookatRotation _returnvalue (+ _returnvalue (Math|Vector|RotateVectorAroundAxis "100.000000, 0,100.000000" (Variables|SpinnerStats|GetAngle) "0.0,1,0.0"))))) (.Pitch (Math|Rotator|BreakRotator (Math|Rotator|FindLookatRotation _returnvalue (+ _returnvalue (Math|Vector|RotateVectorAroundAxis "100.000000, 0,100.000000" (Variables|SpinnerStats|GetAngle) "0.0,1,0.0"))))) (.Yaw (Math|Rotator|BreakRotator (Math|Rotator|FindLookatRotation _returnvalue (+ _returnvalue (Math|Vector|RotateVectorAroundAxis "100.000000, 0,100.000000" (Variables|SpinnerStats|GetAngle) "0.0,1,0.0")))))) true))))))

(fn DamageCheck
  (bind _returnvalue (Game|GetPlayerCharacter 0))
  (bind _returnvalue_2 (Game|GetPlayerCharacter 0))
  (bind _ashuman_character (Utilities|Casting|CastToHumanCharacter _returnvalue))
  (bind _dogreference (Variables|/Game/Blueprints/Characters/HumanCharacter.HumanCharacter_C|GetDogReference _ashuman_character))
  (if (Collision|IsOverlappingActor _returnvalue_2 :!class /Script/Engine.Actor)
    (Game|Damage|ApplyDamage _returnvalue_2 1.0 0 self)
    (elif (Collision|IsOverlappingActor _dogreference :!class /Script/Engine.Actor)
      (Game|Damage|ApplyDamage _dogreference 1.0 0 self))))