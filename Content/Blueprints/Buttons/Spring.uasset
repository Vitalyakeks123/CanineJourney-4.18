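; Spring pad that launches the player character and their companion dog along its arrow's direction.
; Tick counts down a cooldown, then polls overlaps with both characters, applying SpringForce with Z-velocity override, playing a sound and restarting the delay.
; A button event toggles IsTurnedOn, but the launch check never reads it.
; ChangeAnim, which swaps spike flipbooks, is never called here.
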(event Custom|ChangeTurnOn
  ;[1 1 1] Button change on/off
  (if (Variables|Default|GetIsTurnedOn?)
    (Variables|Default|SetIsTurnedOn? false)
    (else
      (Variables|Default|SetIsTurnedOn? true))))

(event EventBeginPlay)

(event EventTick
  (params (DeltaSeconds :type Float%20%28single-precision%29))
  (CallFunction|ChangeTime)
  (CallFunction|CheckCollision))

(fn ConstructionScript)

(fn ChangeAnim
  (if (== (Class|PaperFlipbookComponent|GetFlipbook (Variables|Default|GetPaperFlipbook)) "/Game/Sprites/Spike/spike.spike")
    (Sprite|SetFlipbook (Variables|Default|GetPaperFlipbook) "/Game/Sprites/Spike/spike_opened.spike_opened")
    (else
      (Sprite|SetFlipbook (Variables|Default|GetPaperFlipbook) "/Game/Sprites/Spike/spike_closed.spike_closed"))))

(fn CheckCollision
  (bind _returnvalue (Game|GetPlayerCharacter 0))
  (bind _arrow (Variables|Default|GetArrow))
  (bind _springforce (Variables|FanWind|GetSpringForce))
  (bind _returnvalue_2 (Transformation|GetWorldRotation _arrow))
  (bind _returnvalue_3 (Math|Vector|GetForwardVector _returnvalue_2))
  (bind _returnvalue_4 (* _returnvalue_3 _springforce))
  (if (<= (Variables|Default|GetTime) 0.0)
    (bind _ashuman_character (Utilities|Casting|CastToHumanCharacter _returnvalue))
    (Utilities|FlowControl|Sequence
      (:then_0
        (if (Collision|IsOverlappingActor _returnvalue :!class /Script/Engine.Actor)
          (Character|LaunchCharacter _returnvalue _returnvalue_4 false true)
          (Variables|Default|SetTime (Variables|Default|GetTimeDelay) :!label _label)
          (Audio|PlaySound2D "/Game/StarterContent/Audio/zvuki_dlya_igri/prugina3.prugina3")))
      (:then_1
        (if (Collision|IsOverlappingActor (Variables|/Game/Blueprints/Characters/HumanCharacter.HumanCharacter_C|GetDogReference _ashuman_character) :!class /Script/Engine.Actor)
          (Character|LaunchCharacter (Variables|/Game/Blueprints/Characters/HumanCharacter.HumanCharacter_C|GetDogReference _ashuman_character) _returnvalue_4 false true)
          (goto _label))))))

(fn ChangeTime
  (Variables|Default|SetTime (Math|Float|Clamp(Float) (- (Variables|Default|GetTime) (Utilities|Time|GetWorldDeltaSeconds)) 0.0 123.0)))