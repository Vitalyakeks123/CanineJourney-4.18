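; 2D spike hazard that damages the human and dog characters and destroys Balls on overlap.
; Tick either holds static spikes open or runs a countdown toggling Opened and Closed, with timers swapping transition flipbooks to idle ones.
; Box and flipbook overlaps handle contact, while DamageCheck re-applies damage every tick to an overlapping player or their dog while open.
; Transitional states are overwritten immediately, so damage switches as each animation starts.
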(event OnComponentBeginOverlap(Box)
  (params (OverlappedComponent :type Primitive%20Component%20Object%20Reference) (OtherActor :type Actor%20Object%20Reference) (OtherComp :type Primitive%20Component%20Object%20Reference) (OtherBodyIndex :type Integer) (bFromSweep :type Boolean) (SweepResult :type Hit%20Result%20Structure%20%28by%20ref%29))
  (if (Utilities|Enum|Equal(Enum) (Variables|Default|GetState) "NewEnumerator1")
    (bind _asball (Utilities|Casting|CastToBall OtherActor)
      (:then
        (Actor|DestroyActor _asball))
      (:CastFailed
        (bind _ashuman_character (Utilities|Casting|CastToHumanCharacter OtherActor)
          (:then
            (Game|Damage|ApplyDamage _ashuman_character (Variables|Default|GetDamage) 0 self))
          (:CastFailed
            (bind _asdog_character (Utilities|Casting|CastToDogCharacter OtherActor))
            (Game|Damage|ApplyDamage _asdog_character (Variables|Default|GetDamage) 0 self)))))))

(event OnComponentBeginOverlap(PaperFlipbook)
  (params (OverlappedComponent :type Primitive%20Component%20Object%20Reference) (OtherActor :type Actor%20Object%20Reference) (OtherComp :type Primitive%20Component%20Object%20Reference) (OtherBodyIndex :type Integer) (bFromSweep :type Boolean) (SweepResult :type Hit%20Result%20Structure%20%28by%20ref%29))
  (if (not (Utilities|Enum|Equal(Enum) (Variables|Default|GetState) "NewEnumerator0"))
    (bind _asball (Utilities|Casting|CastToBall OtherActor)
      (:then
        (Actor|DestroyActor _asball))
      (:CastFailed
        (bind _ashuman_character (Utilities|Casting|CastToHumanCharacter OtherActor)
          (:then
            (Game|Damage|ApplyDamage _ashuman_character (Variables|Default|GetDamage) 0 self))
          (:CastFailed
            (bind _asdog_character (Utilities|Casting|CastToDogCharacter OtherActor))
            (Game|Damage|ApplyDamage _asdog_character (Variables|Default|GetDamage) 0 self)))))))

(event EventBeginPlay
  (Variables|Default|SetTime (Variables|Constants|GetOpenedTime)))

(event Collision|EventActorBeginOverlap
  (params (OtherActor :type Actor%20Object%20Reference)))

(event EventTick
  (params (DeltaSeconds :type Float%20%28single-precision%29))
  (if (Variables|Constants|GetIsStatic?)
    (Variables|Default|SetState "NewEnumerator1")
    (else
      (CallFunction|ChangeTime DeltaSeconds)))
  (CallFunction|DamageCheck))

(fn ConstructionScript)

(fn ChangeTime
  (params (Delta%20Time :type Float%20%28single-precision%29))
  (bind _output_get (Variables|Default|SetTime (Math|Float|Clamp(Float) (- (Variables|Default|GetTime) Delta%20Time) 0.0 123.0)))
  (if (<= _output_get 0.0)
    (switch Utilities|FlowControl|Switch|SwitchonSpikeState (Variables|Default|GetState)
      (:NewEnumerator0
        (CallFunction|OpenSpike)
        (Variables|Default|SetTime (Variables|Constants|GetOpenedTime))
        (Variables|Default|SetState "NewEnumerator1"))
      (:NewEnumerator1
        (CallFunction|CloseSpike)
        (Variables|Default|SetTime (Variables|Constants|GetClosedTime))
        (Variables|Default|SetState "NewEnumerator0")))))

(fn OpenSpike
  (Sprite|SetFlipbook (Variables|Default|GetPaperFlipbook) "/Game/Sprites/Spike/spike.spike")
  (Utilities|Time|SetTimerbyFunctionName 0 "ChangeAnim" (- (Class|PaperFlipbookComponent|GetFlipbookLength (Variables|Default|GetPaperFlipbook)) 0.05))
  (Variables|Default|SetState "NewEnumerator2"))

(fn CloseSpike
  (Sprite|SetFlipbook (Variables|Default|GetPaperFlipbook) "/Game/Sprites/Spike/spike_close.spike_close")
  (Utilities|Time|SetTimerbyFunctionName 0 "ChangeAnim" (- (Class|PaperFlipbookComponent|GetFlipbookLength (Variables|Default|GetPaperFlipbook)) 0.05))
  (Variables|Default|SetState "NewEnumerator3"))

(fn ChangeAnim
  (if (== (Class|PaperFlipbookComponent|GetFlipbook (Variables|Default|GetPaperFlipbook)) "/Game/Sprites/Spike/spike.spike")
    (Sprite|SetFlipbook (Variables|Default|GetPaperFlipbook) "/Game/Sprites/Spike/spike_opened.spike_opened")
    (else
      (Sprite|SetFlipbook (Variables|Default|GetPaperFlipbook) "/Game/Sprites/Spike/spike_closed.spike_closed"))))

(fn DamageCheck
  (bind _returnvalue (Game|GetPlayerCharacter 0))
  (bind _returnvalue_2 (Game|GetPlayerCharacter 0))
  (bind _ashuman_character (Utilities|Casting|CastToHumanCharacter _returnvalue))
  (bind _dogreference (Variables|/Game/Blueprints/Characters/HumanCharacter.HumanCharacter_C|GetDogReference _ashuman_character))
  (if (Utilities|Enum|Equal(Enum) (Variables|Default|GetState) "NewEnumerator1")
    (if (Collision|IsOverlappingActor _returnvalue_2 :!class /Script/Engine.Actor)
      (Game|Damage|ApplyDamage _returnvalue_2 (Variables|Default|GetDamage) 0 self)
      (elif (Collision|IsOverlappingActor _dogreference :!class /Script/Engine.Actor)
        (Game|Damage|ApplyDamage _dogreference (Variables|Default|GetDamage) 0 self)))))