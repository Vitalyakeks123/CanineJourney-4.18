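; Spike hazard actor that damages human and dog characters and destroys balls touching its box or flipbook.
; Tick forces its state to the same damaging value, so it never cycles, and damages player character 0 every frame while overlapping.
; When IsBytilka is set, a per-tick sphere trace finds nearby pawns and destroys any EnemyBase overlapping the box.
; The construction script applies the configured sprite.
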(event OnComponentBeginOverlap(Box)
  (params (OverlappedComponent :type Primitive%20Component%20Object%20Reference) (OtherActor :type Actor%20Object%20Reference) (OtherComp :type Primitive%20Component%20Object%20Reference) (OtherBodyIndex :type Integer) (bFromSweep :type Boolean) (SweepResult :type Hit%20Result%20Structure%20%28by%20ref%29))
  (if (Utilities|Enum|Equal(Enum) (Variables|Default|GetState) "NewEnumerator1")
    (bind _asball (Utilities|Casting|CastToBall OtherActor)
      (:then
        (Actor|DestroyActor _asball))
      (:CastFailed
        (bind _ashuman_character (Utilities|Casting|CastToHumanCharacter OtherActor)
          (:then
            (Game|Damage|ApplyDamage _ashuman_character (Variables|Default|GetDamage) 0 self))
          (:CastFailed
            (bind _asdog_character (Utilities|Casting|CastToDogCharacter OtherActor))
            (Game|Damage|ApplyDamage _asdog_character (Variables|Default|GetDamage) 0 self)))))))

(event OnComponentBeginOverlap(PaperFlipbook)
  (params (OverlappedComponent :type Primitive%20Component%20Object%20Reference) (OtherActor :type Actor%20Object%20Reference) (OtherComp :type Primitive%20Component%20Object%20Reference) (OtherBodyIndex :type Integer) (bFromSweep :type Boolean) (SweepResult :type Hit%20Result%20Structure%20%28by%20ref%29))
  (if (not (Utilities|Enum|Equal(Enum) (Variables|Default|GetState) "NewEnumerator0"))
    (bind _asball (Utilities|Casting|CastToBall OtherActor)
      (:then
        (Actor|DestroyActor _asball))
      (:CastFailed
        (bind _ashuman_character (Utilities|Casting|CastToHumanCharacter OtherActor)
          (:then
            (Game|Damage|ApplyDamage _ashuman_character (Variables|Default|GetDamage) 0 self))
          (:CastFailed
            (bind _asdog_character (Utilities|Casting|CastToDogCharacter OtherActor))
            (Game|Damage|ApplyDamage _asdog_character (Variables|Default|GetDamage) 0 self)))))))

(event EventBeginPlay
  (Variables|Default|SetTime (Variables|Constants|GetOpenedTime)))

(event Collision|EventActorBeginOverlap
  (params (OtherActor :type Actor%20Object%20Reference)))

(event EventTick
  (params (DeltaSeconds :type Float%20%28single-precision%29))
  (Variables|Default|SetState "NewEnumerator1")
  (CallFunction|DamageCheck)
  (CallFunction|CheckEnemy))

(fn ConstructionScript
  (Rendering|Components|Sprite|SetSprite (Variables|Default|GetPaperSprite) (Variables|Default|GetSprite)))

(fn DamageCheck
  (bind _returnvalue (Game|GetPlayerCharacter 0))
  (if (Utilities|Enum|Equal(Enum) (Variables|Default|GetState) "NewEnumerator1")
    (if (Collision|IsOverlappingActor _returnvalue :!class /Script/Engine.Actor)
      (Game|Damage|ApplyDamage _returnvalue (Variables|Default|GetDamage) 0 self))))

(fn CheckEnemy
  (bind _returnvalue (Transformation|GetActorLocation))
  (if (Variables|Constants|GetIsBytilka?)
    (bind _outhits (Collision|MultiSphereTraceForObjects _returnvalue _returnvalue 3e+02 (Utilities|Array|MakeArray "ObjectTypeQuery3") false (Utilities|Array|MakeArray self) "None"))
    (for _array_element _outhits
      (bind _asenemy_base (Utilities|Casting|CastToEnemyBase (.HitActor (Collision|BreakHitResult _array_element))))
      (if (Collision|IsOverlappingActor (Variables|Default|GetBox) _asenemy_base :!class /Script/Engine.PrimitiveComponent)
        (Actor|DestroyActor _asenemy_base)))))