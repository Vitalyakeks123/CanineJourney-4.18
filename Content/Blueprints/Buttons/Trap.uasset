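; Trap actor with a Paper2D flipbook that stays hidden until triggered, then damages the player.
; Each Tick polls Box1 for a grounded player and starts an activation timer unless the trap is active or cooling down.
; Named function timers chain the states: show the flipbook, hide it after the active time, then re-arm after cooldown.
; While the flipbook is visible, damage applies every tick to a player overlapping DamageBox.
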(event EventBeginPlay)

(event EventTick
  (params (DeltaSeconds :type Float%20%28single-precision%29))
  (CallFunction|CheckCollision)
  (CallFunction|CheckDamage))

(fn ConstructionScript
  (Development|SetHiddeninGame (Variables|Default|GetPaperFlipbookTrap) true false))

(fn CheckCollision
  (bind _returnvalue (Game|GetPlayerCharacter 0))
  (if (Math|Boolean|ANDBoolean (Collision|IsOverlappingActor (Variables|Default|GetBox1) _returnvalue :!class /Script/Engine.PrimitiveComponent) (not (AI|Components|NavMovement|IsFalling (Variables|/Script/Engine.Character|GetCharacterMovement _returnvalue))) (not (Variables|Default|GetIsActive?)) (not (Variables|Default|GetisCooldown?)))
    (if (not (Class|KismetSystemLibrary|IsTimerActive 0 "SetActive"))
      (Utilities|Time|SetTimerbyFunctionName 0 "SetActive" (Variables|TrapStats|GetActivationTime)))))

(fn SetActive
  (Utilities|Time|SetTimerbyFunctionName 0 "SetNotActive" (Variables|TrapStats|GetActiveTime))
  (Development|SetHiddeninGame (Variables|Default|GetPaperFlipbookTrap) false false)
  (Variables|Default|SetIsActive? true))

(fn SetNotActive
  (Development|SetHiddeninGame (Variables|Default|GetPaperFlipbookTrap) true false)
  (Variables|Default|SetIsActive? false)
  (Variables|Default|SetisCooldown? true)
  (Utilities|Time|SetTimerbyFunctionName 0 "ResetCooldown" (Variables|TrapStats|GetCooldown)))

(fn CheckDamage
  (if (Collision|IsOverlappingActor (Variables|Default|GetDamageBox) (Game|GetPlayerCharacter 0) :!class /Script/Engine.PrimitiveComponent)
    (if (not (Variables|/Script/Engine.SceneComponent|GetbHiddenInGame (Variables|Default|GetPaperFlipbookTrap)))
      (Game|Damage|ApplyDamage (Game|GetPlayerCharacter 0) 1.0 0 self))))

(fn ResetCooldown
  (Variables|Default|SetisCooldown? false))