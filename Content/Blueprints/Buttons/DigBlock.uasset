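; A 2D diggable block that wears down while it is being dug and destroys itself when its dig timer runs out.
; DigBlock subtracts the passed-in delta time from a countdown, while DigPlaySound swaps the Paper2D sprite at three progress thresholds.
; A bool array makes each stage's sound play only once, and the same sound plays again on destruction.
; ResetTime restores the timer, first sprite and stage flags.
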(event Custom|ResetTime
  (bind _digsound (Variables|Default|GetDigSound))
  ;[1 1 1] Reset
  (Variables|Default|SetTime (Variables|DIG|GetDigTime))
  (Rendering|Components|Sprite|SetSprite (Variables|Default|GetPaperSprite) (Utilities|Array|Get(acopy) (Variables|DIG|GetSprites)))
  (for (_ _array_index) _digsound
    (Utilities|Array|SetArrayElem _digsound _array_index false)))

(event Custom|DigBlock
  (params (deltaTime :type Float%20%28single-precision%29))
  (CallFunction|DigPlaySound)
  (bind _output_get (Variables|Default|SetTime (- (Variables|Default|GetTime) deltaTime)))
  (if (<= _output_get 0.0)
    (Actor|DestroyActor)))

(event EventBeginPlay
  (Variables|Default|SetTime (Variables|DIG|GetDigTime)))

(event EventDestroyed
  ;[1 1 1] Event on destroyed
  (Audio|PlaySound2D "/Game/Sounds/zvuki_dlya_igri/kopat.kopat"))

(fn ConstructionScript
  (Rendering|Components|Sprite|SetSprite (Variables|Default|GetPaperSprite) (Utilities|Array|Get(acopy) (Variables|DIG|GetSprites))))

(fn DigPlaySound
  (Utilities|FlowControl|Sequence
    (:then_0
      (if (and (<= (Variables|Default|GetTime) (Variables|DIG|GetDigTime)) (not (Utilities|Array|Get(acopy) (Variables|Default|GetDigSound))))
        (Utilities|Array|SetArrayElem (Variables|Default|GetDigSound) 0 true)
        (Rendering|Components|Sprite|SetSprite (Variables|Default|GetPaperSprite) (Utilities|Array|Get(acopy) (Variables|DIG|GetSprites)))
        (Audio|PlaySound2D "/Game/Sounds/zvuki_dlya_igri/kopat.kopat" :!label _label)))
    (:then_1
      (if (and (<= (Variables|Default|GetTime) (/ (Variables|DIG|GetDigTime) 1.5)) (not (Utilities|Array|Get(acopy) (Variables|Default|GetDigSound) 1)))
        (Utilities|Array|SetArrayElem (Variables|Default|GetDigSound) 1 true)
        (Rendering|Components|Sprite|SetSprite (Variables|Default|GetPaperSprite) (Utilities|Array|Get(acopy) (Variables|DIG|GetSprites) 1))
        (goto _label)))
    (:then_2
      (if (and (<= (Variables|Default|GetTime) (/ (Variables|DIG|GetDigTime) 3.0)) (not (Utilities|Array|Get(acopy) (Variables|Default|GetDigSound) 2)))
        (Utilities|Array|SetArrayElem (Variables|Default|GetDigSound) 2 true)
        (Rendering|Components|Sprite|SetSprite (Variables|Default|GetPaperSprite) (Utilities|Array|Get(acopy) (Variables|DIG|GetSprites) 2))
        (goto _label)))))