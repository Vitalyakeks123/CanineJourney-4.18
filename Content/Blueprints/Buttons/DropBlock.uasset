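; DropBlock is a spawner that launches DroppigBlock actors from its Arrow, either on a repeating timer or on button activation.
; When IsAlways is set, Tick counts down from an initial delay and spawns at each interval; otherwise it counts down a cooldown that gates ButtonActivate.
; Each block receives the arrow's rotation plus speed, lifetime, size and damage radius.
; The construction script scales Box1's extent to the block size.
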(event Custom|ButtonActivate
  (if (<= (Variables|Default|GetTimeDelay) 0.0)
    (CallFunction|SpawnBomb)
    (Variables|Default|SetTimeDelay (Variables|Bomb|GetDelay))))

(event EventBeginPlay
  (Variables|Default|SetTime (Variables|Bomb|GetFirstDelay)))

(event EventTick
  (params (DeltaSeconds :type Float%20%28single-precision%29))
  (if (Variables|Bomb|GetIsAlways?)
    (CallFunction|ChangeTime DeltaSeconds)
    (else
      (CallFunction|DelayChange DeltaSeconds))))

(fn ConstructionScript
  (bind _size (Variables|Bomb|GetSize))
  (Components|Box|SetBoxExtent (Variables|Default|GetBox1) (Math|Vector|MakeVector _size 1e+01 _size) true))

(fn ChangeTime
  (params (Delta%20Time :type Float%20%28single-precision%29))
  (bind _output_get (Variables|Default|SetTime (Math|Float|Clamp(Float) (- (Variables|Default|GetTime) Delta%20Time) 0.0 123.0)))
  (if (<= _output_get 0.0)
    (Variables|Default|SetTime (Variables|Bomb|GetInterval))
    (CallFunction|SpawnBomb)))

(fn SpawnBomb
  (bind _arrow (Variables|Default|GetArrow))
  (bind _returnvalue (Transformation|GetWorldTransform _arrow))
  (bind _returnvalue_2 (Game|SpawnActorfromClass "/Game/Blueprints/Buttons/DropBomb/DroppigBlock.DroppigBlock_C" (Math|Transform|MakeTransform (.location _returnvalue) "0, 0, 0" "1,1,1") "AlwaysSpawn" 0 0))
  (Utilities|IsValid _returnvalue_2
    (:Is%20Valid
      (Variables|/Game/Blueprints/Buttons/DropBomb/DroppigBlock.DroppigBlock_C|SetMoveRotation _returnvalue_2 (.rotation _returnvalue))
      (Variables|/Game/Blueprints/Buttons/DropBomb/DroppigBlock.DroppigBlock_C|SetSpeed _returnvalue_2 (Variables|Bomb|GetSpeed))
      (Variables|/Game/Blueprints/Buttons/DropBomb/DroppigBlock.DroppigBlock_C|SetDropTime _returnvalue_2 (Variables|Bomb|GetLifeTime))
      (Variables|/Game/Blueprints/Buttons/DropBomb/DroppigBlock.DroppigBlock_C|SetSize _returnvalue_2 (Variables|Bomb|GetSize))
      (Default|ChangeSize _returnvalue_2)
      (Variables|/Game/Blueprints/Buttons/DropBomb/DroppigBlock.DroppigBlock_C|SetDamageRadius _returnvalue_2 (Variables|Bomb|GetSizeCheck)))))

(fn DelayChange
  (params (Delta%20Time :type Float%20%28single-precision%29))
  (Variables|Default|SetTimeDelay (Math|Float|Clamp(Float) (- (Variables|Default|GetTimeDelay) Delta%20Time) 0.0 123.0)))