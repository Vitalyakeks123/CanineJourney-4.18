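; Floor button that, when a HumanCharacter overlaps it, changes sprite and drives linked spikes, fans, conveyors, drop blocks and a Gate.
; Pressing disables spike cycling, toggles fans, stops conveyors, triggers drop blocks and opens the Gate.
; Unless OneUse, emptying the tracked-actor array on exit toggles fans and closes the Gate; other changes persist.
; ActivateButtonViaBall repeats the press for OneUse buttons only.
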(event OnComponentBeginOverlap(Box)
  (params (OverlappedComponent :type Primitive%20Component%20Object%20Reference) (OtherActor :type Actor%20Object%20Reference) (OtherComp :type Primitive%20Component%20Object%20Reference) (OtherBodyIndex :type Integer) (bFromSweep :type Boolean) (SweepResult :type Hit%20Result%20Structure%20%28by%20ref%29))
  (Utilities|Casting|CastToHumanCharacter OtherActor)
  (CallFunction|ChangeSprite "/Game/Sprites/LandscapeNEW/button_on_Sprite_0.button_on_Sprite_0")
  (CallFunction|SpikesChange)
  (Utilities|FlowControl|Sequence
    (:then_0
      (CallFunction|FansChangeEvent)
      (CallFunction|ConveyorsOff)
      (CallFunction|DropBlocksActivate))
    (:then_1
      (Utilities|IsValid (Variables|Default|GetGate)
        (:Is%20Valid
          (Default|Open (Variables|Default|GetGate))
          (Utilities|Array|AddUnique (Variables|Default|Getactors_array) OtherActor))))))

(event OnComponentEndOverlap(Box)
  (params (OverlappedComponent :type Primitive%20Component%20Object%20Reference) (OtherActor :type Actor%20Object%20Reference) (OtherComp :type Primitive%20Component%20Object%20Reference) (OtherBodyIndex :type Integer))
  (bind _gate (Variables|Default|GetGate))
  (bind _actors_array (Variables|Default|Getactors_array))
  (if (not (Variables|Default|GetOneUse?))
    (Utilities|Array|RemoveItem _actors_array OtherActor)
    (if (<= (Utilities|Array|Length _actors_array) 0)
      (CallFunction|FansChangeEvent)
      (if (Utilities|IsValid _gate)
        (Default|Close _gate)))))

(event Custom|FansChangeEvent
  (Utilities|FlowControl|DoOnce false :!label _label
    (:Completed
      (CallFunction|FansChange)
      (if (not (Variables|Default|GetOneUse?))
        (goto _label Reset)))))

(event EventBeginPlay)

(event Collision|EventActorBeginOverlap
  (params (OtherActor :type Actor%20Object%20Reference)))

(event EventTick
  (params (DeltaSeconds :type Float%20%28single-precision%29)))

(fn ConstructionScript
  (Rendering|Components|Sprite|SetSprite (Variables|Default|GetPaperSprite) (Variables|Default|GetSprite)))

(fn SpikesChange
  (Utilities|FlowControl|DoOnce false
    (:Completed
      (for _array_element (Variables|Default|GetSpikes)
        (Variables|/Game/Blueprints/Buttons/Spike.Spike_C|SetIsStatic? _array_element false)
        (Variables|/Game/Blueprints/Buttons/Spike.Spike_C|SetClosedTime _array_element 123123123.0)
        (Variables|/Game/Blueprints/Buttons/Spike.Spike_C|SetOpenedTime _array_element 0.0)))))

(fn FansChange
  (for _array_element (Variables|Default|GetFans)
    (Default|ChangeTurnon _array_element)))

(fn ConveyorsOff
  (for _array_element (Variables|Default|GetConveyors)
    (Variables|/Game/Blueprints/Platforms/Conveyor1.Conveyor1_C|SetIsOn? _array_element false)))

(fn ActivateButtonViaBall
  (if (Variables|Default|GetOneUse?)
    (CallFunction|ChangeSprite "/Game/Sprites/LandscapeNEW/button_on_Sprite_0.button_on_Sprite_0")
    (CallFunction|SpikesChange)
    (Utilities|FlowControl|Sequence
      (:then_0
        (CallFunction|FansChangeEvent)
        (CallFunction|ConveyorsOff)
        (CallFunction|DropBlocksActivate))
      (:then_1
        (Utilities|IsValid (Variables|Default|GetGate)
          (:Is%20Valid
            (Default|Open (Variables|Default|GetGate))))))))

(fn DropBlocksActivate
  (for _array_element (Variables|Default|GetDropBlocks)
    (Default|ButtonActivate _array_element)))

(fn ChangeSprite
  (params (Sprite :type Paper%20Sprite%20Object%20Reference))
  (Rendering|Components|Sprite|SetSprite (Variables|Default|GetPaperSprite) Sprite))