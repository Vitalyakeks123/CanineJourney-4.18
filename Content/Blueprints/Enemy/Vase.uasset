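; Breakable vase built as an enemy subclass that takes damage and can drop a coin or heart when destroyed.
; BeginPlay sets low health and damage timings, while empty Tick and UpdateAnimation events override the parent's per-frame behavior.
; The AnyDamage override sets knockback by ranged or melee type, then launches it, briefly stops movement and subtracts health.
; If shielded, it ignores damage until a charged HumanProjectile removes the shield.
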(event EventBeginPlay
  (|CallParentFunction)
  (Variables|Default|SetDamageDelay 9999.0)
  (Variables|Default|SetHealth 2.0)
  (Variables|Default|SetDamageTime_const 0.01))

(event Collision|EventActorBeginOverlap
  (params (OtherActor :type Actor%20Object%20Reference))
  (|CallParentFunction OtherActor) ; This node is disabled and will not be called.\nDrag off pins to build functionality.
)

(event Game|Damage|EventAnyDamage
  (params (Damage :type Float%20%28single-precision%29) (DamageType :type Damage%20Type%20Object%20Reference) (InstigatedBy :type Controller%20Object%20Reference) (DamageCauser :type Actor%20Object%20Reference))
  ;[1 1 1] ApplyDamage overrite
  (Utilities|FlowControl|Sequence
    (:then_0
      (Utilities|Casting|CastToHumanDamageRanged DamageType)
      (Variables|Default|SetPushX 0.0)
      (Variables|Default|SetPushZ 2e+02))
    (:then_1
      (Utilities|Casting|CastToHumanDamageMelee DamageType)
      (Variables|Default|SetPushX 4e+02)
      (Variables|Default|SetPushZ 3e+02))
    (:then_2
      (if (not (Variables|Default|GethasShield?))
        (if (and (> Damage 0.0) (<= (Variables|Default|GetDamageTime) 0.0))
          (CallFunction|LaunchEnemyonHit DamageCauser)
          (Variables|/Script/Engine.CharacterMovementComponent|SetMaxWalkSpeed (Variables|Character|GetCharacterMovement) 0.0)
          (Utilities|Time|SetTimerbyFunctionName 0 "ResetMovement" (Variables|Default|GetDamageStun))
          (bind _output_get (Variables|Default|SetHealth (- (Variables|Default|GetHealth) Damage)))
          (if (<= _output_get 0.0)
            (Actor|DestroyActor)))
        (else
          (bind _ashuman_projectile (Utilities|Casting|CastToHumanProjectile DamageCauser))
          (if (Variables|/Game/Blueprints/Characters/Projectile/HumanProjectile.HumanProjectile_C|GetisCharged? _ashuman_projectile)
            (Variables|Default|SethasShield? false)
            (CallFunction|LaunchEnemyonHit DamageCauser)))))))

(event EventDestroyed
  (if (Variables|Vase_|GetDropCoin?)
    (Game|SpawnActorfromClass "/Game/Blueprints/Pickables/Coin.Coin_C" (Math|Transform|MakeTransform (Transformation|GetActorLocation) "0, 0, 0" "1,1,1") "AlwaysSpawn" 0 0))
  (if (Variables|Vase_|GetDropHealth?)
    (Game|SpawnActorfromClass "/Game/Blueprints/Pickables/Heart.Heart_C" (Math|Transform|MakeTransform (Transformation|GetActorLocation) "0, 0, 0" "1,1,1") "AlwaysSpawn" 0 0)))

(event EventTick
  (params (DeltaSeconds :type Float%20%28single-precision%29)))

(event EventUpdateAnimation)

(fn ConstructionScript
  (|CallParentFunction)
  (Sprite|SetFlipbook (Variables|Default|GetSprite) (Variables|Vase|GetSprite_)))