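; Side-scrolling charger enemy that winds up, then dashes a fixed range, damaging any human it overlaps.
; Tick drives cooldown, cast and swept-offset charge while in the camera block, plus timer-delayed turning.
; Outside a charge, hits cause knockback, stun and health loss, though elites only take damage from behind.
; Mid-charge it takes no health damage, but a charged human projectile cuts the dash short and knocks it back.
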(event EventBeginPlay
  (|CallParentFunction) ; This node is disabled and will not be called.\nDrag off pins to build functionality.
)

(event Game|Damage|EventAnyDamage
  (params (Damage :type Float%20%28single-precision%29) (DamageType :type Damage%20Type%20Object%20Reference) (InstigatedBy :type Controller%20Object%20Reference) (DamageCauser :type Actor%20Object%20Reference))
  ;[1 1 1] ApplyDamage
  (Utilities|FlowControl|Sequence
    (:then_0
      (Utilities|Casting|CastToHumanDamageRanged DamageType)
      (Variables|Default|SetPushX 2e+02)
      (Variables|Default|SetPushZ 2e+02))
    (:then_1
      (Utilities|Casting|CastToHumanDamageMelee DamageType)
      (Variables|Default|SetPushX 4e+02)
      (Variables|Default|SetPushZ 3e+02))
    (:then_2
      (if (not (Variables|Charge|GetisInCharge?))
        (if (and (> Damage 0.0) (<= (Variables|Default|GetDamageTime) 0.0))
          (if (not (Variables|Default|GetisElite?))
            (CallFunction|LaunchEnemyonHit DamageCauser :!label _label)
            (Variables|Default|SetDamageTime (Variables|Default|GetDamageTime_const))
            (Variables|/Script/Engine.CharacterMovementComponent|SetMaxWalkSpeed (Variables|Character|GetCharacterMovement) 0.0)
            (Utilities|Time|SetTimerbyFunctionName 0 "ResetMovement" (Variables|Default|GetDamageStun))
            (bind _output_get (Variables|Default|SetHealth (- (Variables|Default|GetHealth) Damage)))
            (if (<= _output_get 0.0)
              (Actor|DestroyActor))
            (else
              (bind _canbedamaged_ (CallFunction|EliteChargerCanbeDamaged? DamageCauser))
              (if _canbedamaged_
                (goto _label)))))
        (else
          (bind _ashuman_projectile (Utilities|Casting|CastToHumanProjectile DamageCauser))
          (if (Variables|/Game/Blueprints/Characters/Projectile/HumanProjectile.HumanProjectile_C|GetisCharged? _ashuman_projectile)
            (Variables|Charge|SetChargeRange 0.0)
            (CallFunction|LaunchEnemyonHit _ashuman_projectile)))))))

(event EventSetElite
  ;[1 1 1] Override SetElite
)

(event EventTick
  (params (DeltaSeconds :type Float%20%28single-precision%29))
  (|CallParentFunction DeltaSeconds)
  (CallFunction|TimeChange)
  (CallFunction|CheckforRotationCharge)
  (CallFunction|CheckforDamage))

(event EventChaseHuman
  ;[1 1 1] Overrided functions
)

(event EventDamageHuman
  ;[1 1 1] Overrided functions
)

(event EventUpdateAnimation
  (bind _sprite (Variables|Default|GetSprite))
  ;[1 1 1] Handle Animation
  (Utilities|FlowControl|Sequence
    (:then_0
      ;[1 1 1] State machine
      (if (> (Math|Vector|VectorLength (Transformation|GetVelocity)) 0.0)
        (Variables|Default|SetState "NewEnumerator0")
        (else
          (Variables|Default|SetState "NewEnumerator0"))))
    (:then_1
      (if (Variables|Charge|GetisInCharge?)
        (Variables|Default|SetState "NewEnumerator1")))
    (:then_2
      (switch Utilities|FlowControl|Switch|SwitchonHumanState (Variables|Default|GetState)
        (:NewEnumerator0
          (Sprite|SetFlipbook _sprite "/Game/Sprites/Enemy/Charger/charger_idle_anim.charger_idle_anim"))
        (:NewEnumerator1
          (Sprite|SetFlipbook _sprite "/Game/Sprites/Enemy/Charger/charger_attack_anim.charger_attack_anim"))))))

(fn ConstructionScript
  (|CallParentFunction))

(fn TimeChange
  (bind _incamerablock_ (CallFunction|IsinCameraBlock))
  (if _incamerablock_
    (Utilities|FlowControl|Sequence
      (:then_0
        ;[1 1 1] ChargeCD update
        (bind _output_get (Variables|Charge|SetChargeCD (- (Variables|Charge|GetChargeCD) (Utilities|Time|GetWorldDeltaSeconds))))
        (if (Math|Boolean|ANDBoolean (<= _output_get 0.0) (Utilities|Enum|Equal(Enum) (Variables|Default|GetEnemyState) "NewEnumerator2") (not (Variables|Charge|GetisInCharge?)) (not (Variables|Charge|GetisCharging?)))
          (if (Math|Boolean|Equal(Boolean) (Variables|Default|GetbisMovingRight) (Variables|Default|GetisEnemyRight?))
            (Variables|Charge|SetisCharging? true)
            (Variables|Charge|SetChargeCast (Variables|Charge|GetChargeCast_const))
            (Variables|Charge|SetChargeCD (Variables|Charge|GetChargeCD_const)))))
      (:then_1
        ;[1 1 1] Charge Casting
        (bind _output_get_2 (Variables|Charge|SetChargeCast (- (Variables|Charge|GetChargeCast) (Utilities|Time|GetWorldDeltaSeconds))))
        (if (and (<= _output_get_2 0.0) (Variables|Charge|GetisCharging?))
          (Variables|Charge|SetisCharging? false)
          (Variables|Charge|SetisInCharge? true)
          (Variables|Charge|SetChargeRange (Variables|Charge|GetChargeRange_const))
          (Variables|/Script/Engine.CharacterMovementComponent|SetMaxWalkSpeed (Variables|Character|GetCharacterMovement) 0.0)))
      (:then_2
        ;[1 1 1] In Charge
        (if (Variables|Charge|GetisInCharge?)
          (bind _output_get_3 (LocalVariables|SetdeltaX (* (Variables|Charge|GetChargeSpeed) (Utilities|Time|GetWorldDeltaSeconds))))
          (if (> _output_get_3 (Variables|Charge|GetChargeRange))
            (Transformation|AddActorLocalOffset (Math|Vector|MakeVector (Variables|Charge|GetChargeRange) 0.0 0.0) true true)
            (Variables|Charge|SetChargeRange 0.0)
            (else
              (Variables|Charge|SetChargeRange (- (Variables|Charge|GetChargeRange) (LocalVariables|GetdeltaX)))
              (Transformation|AddActorLocalOffset (Math|Vector|MakeVector (LocalVariables|GetdeltaX) 0.0 0.0) true true)))
          (if (<= (Variables|Charge|GetChargeRange) 0.0)
            (Variables|/Script/Engine.CharacterMovementComponent|SetMaxWalkSpeed (Variables|Character|GetCharacterMovement) (Variables|Default|GetMoveSpeed))
            (Variables|Charge|SetisInCharge? false)
            (Variables|Charge|SetChargeCD (Variables|Charge|GetChargeCD_const))
            (CallFunction|CheckforRotation)))))))

(fn ChargeStartCasting
  (bind _chargerange_const (Variables|Charge|GetChargeRange_const))
  (bind _chargespeed (Variables|Charge|GetChargeSpeed))
  (Variables|Charge|SetChargeCD (Variables|Charge|GetChargeCD_const))
  (if (Variables|Default|GetbisMovingRight)
    (Character|LaunchCharacter (Math|Vector|MakeVector _chargerange_const 0.0 _chargespeed) true true)
    (else
      (Character|LaunchCharacter (Math|Vector|MakeVector (* _chargerange_const -1.0) 0.0 _chargespeed) true true)))
  (Variables|Charge|SetisInCharge? true))

(fn RotateCharge
  (if (Utilities|Enum|Equal(Enum) (Variables|Default|GetEnemyState) "NewEnumerator2")
    (Utilities|FlowControl|Sequence
      (:then_0
        (if (and (Variables|Default|GetbisMovingRight) (not (Variables|Default|GetisEnemyRight?)))
          (Transformation|SetActorRotation "0,180.000000, 0")
          (Variables|Default|SetbisMovingRight false)))
      (:then_1
        (if (and (not (Variables|Default|GetbisMovingRight)) (Variables|Default|GetisEnemyRight?))
          (Transformation|SetActorRotation "0, 0, 0")
          (Variables|Default|SetbisMovingRight true))))))

(fn CheckforDamage
  (if (Variables|Charge|GetisInCharge?)
    (for _array_element (Collision|GetOverlappingActors (Variables|Default|GetDamageCollision) 0 :!class /Script/Engine.PrimitiveComponent)
      (bind _ashuman_character (Utilities|Casting|CastToHumanCharacter _array_element))
      (Game|Damage|ApplyDamage _ashuman_character 1.0 0 self))))

(fn EliteChargerCanbeDamaged?
  (params (DamageSource :type Actor%20Object%20Reference))
  (bind _returnvalue (Transformation|GetActorLocation))
  (bind _returnvalue_2 (Transformation|GetActorLocation DamageSource))
  (if (Variables|Default|GetbisMovingRight)
    (return (< (.x _returnvalue_2) (.x _returnvalue)))
    (else
      (return (> (.x _returnvalue_2) (.x _returnvalue))))))

(fn CheckforRotationCharge
  (if (Utilities|Enum|Equal(Enum) (Variables|Default|GetEnemyState) "NewEnumerator2")
    (Utilities|FlowControl|Sequence
      (:then_0
        (if (and (Variables|Default|GetbisMovingRight) (not (Variables|Default|GetisEnemyRight?)))
          (if (not (Class|KismetSystemLibrary|IsTimerActive 0 "RotateCharge")) :!label _label
            (Utilities|Time|SetTimerbyFunctionName 0 "RotateCharge" (Variables|Default|GetChangeRotationTime)))))
      (:then_1
        (if (and (not (Variables|Default|GetbisMovingRight)) (Variables|Default|GetisEnemyRight?))
          (goto _label))))))