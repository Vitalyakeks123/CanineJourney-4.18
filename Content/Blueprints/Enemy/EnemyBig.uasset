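; Big slime enemy that patrols between two points and chases the human player within DetectRange.
; Tick picks the state by distance and moves through EnemyBigController without pathfinding; a timer swaps patrol targets after a wait.
; DamageCollision overlap starts and clears a repeating DamageHuman timer, while UpdateAnimation selects flipbooks from movement.
; Dog chase and damage functions respect playing dead but are not called here, and BarkTime is disconnected.
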(event OnComponentBeginOverlap(DamageCollision)
  (params (OverlappedComponent :type Primitive%20Component%20Object%20Reference) (OtherActor :type Actor%20Object%20Reference) (OtherComp :type Primitive%20Component%20Object%20Reference) (OtherBodyIndex :type Integer) (bFromSweep :type Boolean) (SweepResult :type Hit%20Result%20Structure%20%28by%20ref%29))
  (Utilities|Casting|CastToHumanCharacter OtherActor)
  (if (not (Class|KismetSystemLibrary|TimerExists 0 "DamageHuman"))
    (Utilities|Time|SetTimerbyFunctionName 0 "DamageHuman" (Variables|Enemy|GetDamageDelay) true)))

(event OnComponentEndOverlap(DamageCollision)
  (params (OverlappedComponent :type Primitive%20Component%20Object%20Reference) (OtherActor :type Actor%20Object%20Reference) (OtherComp :type Primitive%20Component%20Object%20Reference) (OtherBodyIndex :type Integer))
  (Utilities|Casting|CastToHumanCharacter OtherActor)
  (Utilities|Time|ClearTimerbyFunctionName 0 "DamageHuman"))

(event EventBeginPlay
  (|CallParentFunction)
  (Variables|Default|SetcurrentMoveLocation (Variables|Default|GetPatrolPoint))
  (Variables|Default|SetnextMoveLocation (Variables|Default|GetPatrolDefPosition))
  (Variables|Default|SetEnemyState "NewEnumerator0"))

(event Collision|EventActorBeginOverlap
  (params (OtherActor :type Actor%20Object%20Reference)))

(event EventTick
  (params (DeltaSeconds :type Float%20%28single-precision%29))
  (|CallParentFunction DeltaSeconds)
  (CallFunction|ChangeState)
  (switch Utilities|FlowControl|Switch|SwitchonEnemyState (Variables|Default|GetEnemyState)
    (:NewEnumerator0
      (if (Variables|Enemy|GetisPatroling?)
        (CallFunction|StatePatroling)))
    (:NewEnumerator2
      (CallFunction|ChaseHuman))))

(event EventUpdateAnimation
  (bind _sprite (Variables|Default|GetSprite))
  ;[1 1 1] Handle Animation
  (Utilities|FlowControl|Sequence
    (:then_0
      ;[1 1 1] State machine
      (if (> (Math|Vector|VectorLength (Transformation|GetVelocity)) 0.0)
        (Variables|Default|SetState "NewEnumerator1")
        (else
          (Variables|Default|SetState "NewEnumerator0"))))
    (:then_1
      (if (AI|Components|NavMovement|IsFalling (Variables|Character|GetCharacterMovement))
        (Variables|Default|SetState "NewEnumerator2")
        (Variables|Default|SetIsThrowing? false)))
    (:then_2
      (switch Utilities|FlowControl|Switch|SwitchonHumanState (Variables|Default|GetState)
        (:NewEnumerator0
          (Sprite|SetFlipbook _sprite "/Game/Sprites/Slime/Slimeboi_idle.Slimeboi_idle"))
        (:NewEnumerator1
          (Sprite|SetFlipbook _sprite "/Game/Sprites/Slime/Slimeboi.Slimeboi"))
        (:NewEnumerator2
          (Sprite|SetFlipbook (Variables|Default|GetSprite) "/Game/Sprites/Slime/Slimeboi.Slimeboi"))))))

(fn ConstructionScript
  (|CallParentFunction))

(fn PatrolCheck
  (if (<= (Math|Float|Absolute(Float) (- (.x (Transformation|GetActorLocation)) (.x (Variables|Default|GetcurrentMoveLocation)))) 25.0)
    (if (not (Class|KismetSystemLibrary|IsTimerActive 0 "changePatrol"))
      (Utilities|Time|SetTimerbyFunctionName 0 "changePatrol" (Variables|Enemy|GetPatrolWaitDelay)))))

(fn ChangePatrol
  (LocalVariables|SetTempLocation (Variables|Default|GetcurrentMoveLocation))
  (Variables|Default|SetcurrentMoveLocation (Variables|Default|GetnextMoveLocation))
  (Variables|Default|SetnextMoveLocation (LocalVariables|GetTempLocation))
  (Utilities|Time|ClearTimerbyFunctionName 0 "changePatrol"))

(fn StatePatroling
  (bind _currentmovelocation (Variables|Default|GetcurrentMoveLocation))
  (bind _asenemy_big_controller (Utilities|Casting|CastToEnemyBigController (AI|GetAIController self)))
  (AI|Navigation|MovetoLocation _asenemy_big_controller (Math|Vector|MakeVector (.x _currentmovelocation) (.y _currentmovelocation) (.z _currentmovelocation)) 1.0 true false false)
  (CallFunction|PatrolCheck))

(fn ChangeState
  (bind _ashuman_character (Utilities|Casting|CastToHumanCharacter (Game|GetPlayerCharacter 0)))
  (if (<= (Math|Vector|VectorLength (- (Transformation|GetActorLocation _ashuman_character) (Transformation|GetActorLocation))) (Variables|enemy|GetDetectRange))
    (Variables|Default|SetEnemyState "NewEnumerator2")
    (else
      (Variables|Default|SetEnemyState "NewEnumerator0"))))

(fn ChaseDog
  (bind _returnvalue (Game|GetPlayerCharacter 0))
  (bind _ashuman_character (Utilities|Casting|CastToHumanCharacter _returnvalue))
  (bind _dogreference (Variables|/Game/Blueprints/Characters/HumanCharacter.HumanCharacter_C|GetDogReference _ashuman_character))
  (bind _returnvalue_2 (Transformation|GetActorLocation _dogreference))
  (if (not (Variables|/Game/Blueprints/Characters/DogCharacter.DogCharacter_C|GetisPlayingDead _dogreference))
    (bind _asenemy_big_controller (Utilities|Casting|CastToEnemyBigController (AI|GetAIController self)))
    (AI|Navigation|MovetoLocation _asenemy_big_controller (Math|Vector|MakeVector (.x _returnvalue_2) 0.0 (.z _returnvalue_2)) 1.0 true false false)))

(fn ChaseHuman
  (bind _returnvalue (Game|GetPlayerCharacter 0))
  (bind _ashuman_character (Utilities|Casting|CastToHumanCharacter _returnvalue))
  (bind _returnvalue_2 (Transformation|GetActorLocation _ashuman_character))
  (bind _asenemy_big_controller (Utilities|Casting|CastToEnemyBigController (AI|GetAIController self)))
  (AI|Navigation|MovetoLocation _asenemy_big_controller (Math|Vector|MakeVector (.x _returnvalue_2) (.y _returnvalue_2) (.z _returnvalue_2)) 1.0 true false false))

(fn BarkTime
  (params (DeltaTime :type Float%20%28single-precision%29)))

(fn DamageHuman
  (if (<= (Variables|Default|GetDamageTime) 0.0)
    (Game|Damage|ApplyDamage (Game|GetPlayerCharacter 0) 1.0 0 self)
    (Utilities|Time|SetTimerbyFunctionName 0 "DamageHuman" (Variables|Enemy|GetDamageDelay))
    (else
      (Utilities|Time|SetTimerbyFunctionName 0 "DamageHuman" (Variables|Default|GetDamageTime)))))

(fn DamageDog
  (bind _returnvalue (Game|GetPlayerCharacter 0))
  (bind _ashuman_character (Utilities|Casting|CastToHumanCharacter _returnvalue))
  (bind _dogreference (Variables|/Game/Blueprints/Characters/HumanCharacter.HumanCharacter_C|GetDogReference _ashuman_character))
  (if (not (Variables|/Game/Blueprints/Characters/DogCharacter.DogCharacter_C|GetisPlayingDead _dogreference))
    (Game|Damage|ApplyDamage _dogreference 1.0 0 self)
    (Utilities|Time|SetTimerbyFunctionName 0 "DamageDog" (Variables|Enemy|GetDamageDelay))))