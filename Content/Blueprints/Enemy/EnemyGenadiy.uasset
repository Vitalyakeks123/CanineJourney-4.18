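; Genadiy is an armored skeleton side-scroller enemy that patrols, chases the player, leaps and fires projectiles.
; Tick updates the flipbook and runs the patrol/chase state logic from inherited helpers.
; Self-rescheduling timers randomly trigger jumps and timed casts while chasing, and pounce-collision overlaps mid-jump reverse the leap.
; Its shield blocks damage until a charged human projectile breaks it; later hits stun it and reduce health until destruction.
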(event OnComponentBeginOverlap(PounceCollision)
  (params (OverlappedComponent :type Primitive%20Component%20Object%20Reference) (OtherActor :type Actor%20Object%20Reference) (OtherComp :type Primitive%20Component%20Object%20Reference) (OtherBodyIndex :type Integer) (bFromSweep :type Boolean) (SweepResult :type Hit%20Result%20Structure%20%28by%20ref%29))
  (bind _jumpforce (Variables|Genadiy|GetJumpForce))
  ;[1 1 1] Pounce
  (if (and (Variables|Genadiy|GetisJumping?) (not (Variables|Genadiy|GetisPouncing?)))
    (Utilities|Casting|CastToEnemyBigController (AI|GetAIController self))
    (Variables|Genadiy|SetisPouncing? true)
    (if (Variables|Genadiy|GetJumpingRight?)
      (Variables|Genadiy|SetJumpingRight? false)
      (Character|LaunchCharacter (Math|Vector|MakeVector -3e+02 0.0 _jumpforce) true true)
      (Pawn|SetControlRotation (Pawn|GetController) (Math|Rotator|MakeRotator 0.0 0.0 1.8e+02))
      (else
        (Variables|Genadiy|SetJumpingRight? true)
        (Character|LaunchCharacter (Math|Vector|MakeVector 3e+02 0.0 _jumpforce) true true)
        (Pawn|SetControlRotation (Pawn|GetController) (Math|Rotator|MakeRotator 0.0 0.0 0.0))))
    (Utilities|Time|SetTimerbyFunctionName 0 "ResetPounceCooldown" 0.5)))

(event EventBeginPlay
  (|CallParentFunction)
  (Utilities|Time|SetTimerbyFunctionName 0 "TryJump" (Variables|Genadiy|GetJumpCooldown))
  (Utilities|Time|SetTimerbyFunctionName 0 "TryCast" (Variables|Genadiy|GetProjectileCooldown)))

(event Collision|EventActorBeginOverlap
  (params (OtherActor :type Actor%20Object%20Reference))
  (|CallParentFunction OtherActor))

(event Game|Damage|EventAnyDamage
  (params (Damage :type Float%20%28single-precision%29) (DamageType :type Damage%20Type%20Object%20Reference) (InstigatedBy :type Controller%20Object%20Reference) (DamageCauser :type Actor%20Object%20Reference))
  ;[1 1 1] ApplyDamage overrite
  (Utilities|FlowControl|Sequence
    (:then_0
      (Utilities|Casting|CastToHumanDamageRanged DamageType)
      (Variables|Default|SetPushX 2e+02)
      (Variables|Default|SetPushZ 2e+02))
    (:then_1
      (Utilities|Casting|CastToHumanDamageMelee DamageType)
      (Variables|Default|SetPushX 4e+02)
      (Variables|Default|SetPushZ 3e+02))
    (:then_2
      (if (not (Variables|Default|GethasShield?))
        (if (and (> Damage 0.0) (<= (Variables|Default|GetDamageTime) 0.0))
          (Variables|Default|SetDamageTime (Variables|Default|GetDamageTime_const))
          (Variables|/Script/Engine.CharacterMovementComponent|SetMaxWalkSpeed (Variables|Character|GetCharacterMovement) 0.0)
          (Utilities|Time|SetTimerbyFunctionName 0 "ResetMovement" (Variables|Default|GetDamageStun))
          (bind _output_get (Variables|Default|SetHealth (- (Variables|Default|GetHealth) Damage)))
          (if (<= _output_get 0.0)
            (Actor|DestroyActor)))
        (else
          (bind _ashuman_projectile (Utilities|Casting|CastToHumanProjectile DamageCauser))
          (if (Variables|/Game/Blueprints/Characters/Projectile/HumanProjectile.HumanProjectile_C|GetisCharged? _ashuman_projectile)
            (Variables|Default|SethasShield? false)))))))

(event EventUpdateAnimation
  ;[1 1 1] Update Animation Overrided
  (if (Variables|Genadiy|GetisCasting?)
    (Sprite|SetFlipbook (Variables|Default|GetSprite) "/Game/Sprites/Enemy/Genadiy/skeleton_armor_cast.skeleton_armor_cast")
    (elif (Variables|Genadiy|GetisUsingAttack?)
      (Sprite|SetFlipbook (Variables|Default|GetSprite) "/Game/Sprites/Enemy/Genadiy/skeleton_armor_attack.skeleton_armor_attack")
      (else
        (Sprite|SetFlipbook (Variables|Default|GetSprite) "/Game/Sprites/Enemy/Genadiy/skeleton_armor_walk.skeleton_armor_walk")))))

(event EventTick
  (params (DeltaSeconds :type Float%20%28single-precision%29))
  ;[1 1 1] Event Tick
  (CallFunction|UpdateAnimation)
  (CallFunction|TickVariables)
  (Utilities|FlowControl|Sequence
    (:then_0
      (if (Utilities|Enum|Equal(Enum) (Variables|Default|GetEnemyState) "NewEnumerator2")
        (if (>= (.x (Transformation|GetActorLocation (Game|GetPlayerCharacter 0))) (.x (Transformation|GetActorLocation)))
          (Variables|Default|SetbisMovingRight true)
          (else
            (Variables|Default|SetbisMovingRight false)))))
    (:then_1
      (CallFunction|ChangeState)
      (switch Utilities|FlowControl|Switch|SwitchonEnemyState (Variables|Default|GetEnemyState)
        (:NewEnumerator0
          (if (Variables|Default|GetisPatroling?)
            (CallFunction|StatePatroling)))
        (:NewEnumerator2
          (if (Math|Boolean|ANDBoolean (not (Variables|Genadiy|GetisJumping?)) (not (Variables|Genadiy|GetisCasting?)) (not (Variables|Genadiy|GetisUsingAttack?)))
            (CallFunction|ChaseHuman)
            (CallFunction|CheckforRotation)))))))

(event EventOnLanded
  (params (Hit :type Hit%20Result%20Structure%20%28by%20ref%29))
  ;[1 1 1] Event OnLanded - Reset Jump Cooldown if was in Jump
  (if (Variables|Genadiy|GetisJumping?)
    (Variables|Genadiy|SetisJumping? false)
    (Utilities|Time|SetTimerbyFunctionName 0 "ResetJumpCooldown" (Variables|Genadiy|GetJumpCooldown))))

(fn ConstructionScript
  (|CallParentFunction))

(fn ResetJumpCooldown
  (Variables|Genadiy|SetcanJump? true)
  (CallFunction|TryJump))

(fn TryJump
  (bind _jumpforce (Variables|Genadiy|GetJumpForce))
  (bind _jumpforcerandomize (Variables|Genadiy|GetJumpForceRandomize))
  (bind _jumprange (Variables|Genadiy|GetJumpRange))
  (bind _returnvalue (Math|Random|RandomFloatinRange 0.0 _jumpforcerandomize))
  (bind _returnvalue_2 (+ _jumpforce _returnvalue))
  (if (<= (Math|Random|RandomIntegerinRange 0 10) 4)
    (if (Math|Boolean|ANDBoolean (Variables|Genadiy|GetcanJump?) (not (AI|Components|NavMovement|IsFalling (Variables|Character|GetCharacterMovement))) (not (Variables|Genadiy|GetisJumping?)) (Utilities|Enum|Equal(Enum) (Variables|Default|GetEnemyState) "NewEnumerator2") (not (Variables|Genadiy|GetisCasting?)) (not (Variables|Genadiy|GetisUsingAttack?)))
      (Variables|Genadiy|SetcanJump? false)
      (Variables|Genadiy|SetisJumping? true)
      (Components|Movement|StopMovementImmediately (Variables|Character|GetCharacterMovement))
      (if (Variables|Default|GetisEnemyRight?)
        (Character|LaunchCharacter (Math|Vector|MakeVector _jumprange 0.0 _returnvalue_2) true true)
        (Variables|Genadiy|SetJumpingRight? true)
        (else
          (Character|LaunchCharacter (Math|Vector|MakeVector (* _jumprange -1.0) 0.0 _returnvalue_2) true true)
          (Variables|Genadiy|SetJumpingRight? false)))
      (else
        (Utilities|Time|SetTimerbyFunctionName 0 "TryJump" (Variables|Genadiy|GetJumpCooldown) :!label _label)))
    (else
      (goto _label))))

(fn ResetPounceCooldown
  (Variables|Genadiy|SetisPouncing? false))

(fn TryCast
  (if (<= (Math|Random|RandomIntegerinRange 0 10) 3)
    (if (Math|Boolean|ANDBoolean (Variables|Genadiy|GetcanCast?) (not (AI|Components|NavMovement|IsFalling (Variables|Character|GetCharacterMovement))) (Utilities|Enum|Equal(Enum) (Variables|Default|GetEnemyState) "NewEnumerator2") (not (Variables|Genadiy|GetisCasting?)))
      (Variables|Genadiy|SetcanCast? false)
      (Variables|Genadiy|SetisCasting? true)
      (Utilities|Time|SetTimerbyFunctionName 0 "RangeAttack" (Variables|Genadiy|GetCastingDuration))
      (Components|Movement|StopMovementImmediately (Variables|Character|GetCharacterMovement))
      (else
        (Utilities|Time|SetTimerbyFunctionName 0 "TryCast" (Variables|Genadiy|GetProjectileCooldown) :!label _label)))
    (else
      (goto _label))))

(fn RangeAttack
  (Variables|Genadiy|SetisUsingAttack? true)
  (Variables|Genadiy|SetisCasting? false)
  (Utilities|Time|SetTimerbyFunctionName 0 "EndRangeAttack" 0.3))

(fn EndRangeAttack
  (Variables|Genadiy|SetisUsingAttack? false)
  (Variables|Genadiy|SetcanCast? true)
  (Utilities|Time|SetTimerbyFunctionName 0 "TryCast" (Variables|Genadiy|GetProjectileCooldown))
  (Game|SpawnActorfromClass "/Game/Blueprints/Enemy/Projectiles/EnemyGenadyiProjectile.EnemyGenadyiProjectile_C" (Transformation|GetWorldTransform (Variables|Default|GetProjectileArrow)) "AlwaysSpawn" 0 0)
  (Audio|PlaySound2D "/Game/StarterContent/Audio/zvuki_dlya_igri/ydar_vraga.ydar_vraga"))