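; Big helmeted slime enemy (Kaska) Blueprint that sets its sprite flipbook to match its movement.
; UpdateAnimation derives an Idle or Running state from velocity, then overrides it to Jumping and clears IsThrowing while falling.
; The state selects the flipbook, with Running and Jumping sharing the same animation.
; BeginPlay, overlap and Tick are disabled stubs, and the construction script only calls its parent.
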(event EventBeginPlay
  (|CallParentFunction) ; This node is disabled and will not be called.\nDrag off pins to build functionality.
)

(event Collision|EventActorBeginOverlap
  (params (OtherActor :type Actor%20Object%20Reference))
  (|CallParentFunction OtherActor) ; This node is disabled and will not be called.\nDrag off pins to build functionality.
)

(event EventTick
  (params (DeltaSeconds :type Float%20%28single-precision%29))
  (|CallParentFunction DeltaSeconds) ; This node is disabled and will not be called.\nDrag off pins to build functionality.
)

(event EventUpdateAnimation
  (bind _sprite (Variables|Default|GetSprite))
  ;[1 1 1] Handle Animation
  (Utilities|FlowControl|Sequence
    (:then_0
      ;[1 1 1] State machine
      (if (> (Math|Vector|VectorLength (Transformation|GetVelocity)) 0.0)
        (Variables|Default|SetState "NewEnumerator1")
        (else
          (Variables|Default|SetState "NewEnumerator0"))))
    (:then_1
      (if (AI|Components|NavMovement|IsFalling (Variables|Character|GetCharacterMovement))
        (Variables|Default|SetState "NewEnumerator2")
        (Variables|Default|SetIsThrowing? false)))
    (:then_2
      (switch Utilities|FlowControl|Switch|SwitchonHumanState (Variables|Default|GetState)
        (:NewEnumerator0
          (Sprite|SetFlipbook _sprite "/Game/Sprites/Slime/Slimeboi_kaska_idle.Slimeboi_kaska_idle"))
        (:NewEnumerator1
          (Sprite|SetFlipbook _sprite "/Game/Sprites/Slime/Slimeboi_kaska.Slimeboi_kaska"))
        (:NewEnumerator2
          (Sprite|SetFlipbook (Variables|Default|GetSprite) "/Game/Sprites/Slime/Slimeboi_kaska.Slimeboi_kaska"))))))

(fn ConstructionScript
  (|CallParentFunction))