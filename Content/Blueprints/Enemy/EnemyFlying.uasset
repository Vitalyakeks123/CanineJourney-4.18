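; Flying side-scroller enemy that patrols or chases the human and is destroyed by any damage.
; Each tick it faces left or right from X velocity, then runs ChangeState and the matching state behavior.
; Chasing only moves inside the camera block, issuing short straight AI moves along X, without pathfinding, at the Z height saved on BeginPlay.
; Overrides UpdateAnimation with an empty event.
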(event EventBeginPlay
  ;[1 1 1] Begin Play
  (|CallParentFunction)
  (Variables|/Script/Engine.CharacterMovementComponent|SetMaxFlySpeed (Variables|Character|GetCharacterMovement) (Variables|Default|GetMoveSpeed))
  (Variables|Default|SetDefaultLocation (Transformation|GetActorLocation)))

(event Collision|EventActorBeginOverlap
  (params (OtherActor :type Actor%20Object%20Reference))
  (|CallParentFunction OtherActor))

(event EventTick
  (params (DeltaSeconds :type Float%20%28single-precision%29))
  ;[1 1 1] Event Tick
  (Utilities|FlowControl|Sequence
    (:then_0
      (Math|Float|CompareFloat (.X (Math|Vector|BreakVector (Variables|/Script/Engine.MovementComponent|GetVelocity (Pawn|GetMovementComponent)))) 0.0
        (:>
          (Pawn|SetControlRotation (Pawn|GetController) (Math|Rotator|MakeRotator 0.0 0.0 0.0) :!label _label))
        (:==
          (if (Variables|Default|GetbisMovingRight)
            (goto _label)
            (else
              (Pawn|SetControlRotation (Pawn|GetController) (Math|Rotator|MakeRotator 0.0 0.0 1.8e+02) :!label _label_2))))
        (:<
          (goto _label_2))))
    (:then_1
      (CallFunction|ChangeState)
      (switch Utilities|FlowControl|Switch|SwitchonEnemyState (Variables|Default|GetEnemyState)
        (:NewEnumerator0
          (if (Variables|Default|GetisPatroling?)
            (CallFunction|StatePatroling)))
        (:NewEnumerator2
          (CallFunction|ChaseHuman)
          (CallFunction|CheckforRotation))))))

(event Game|Damage|EventAnyDamage
  (params (Damage :type Float%20%28single-precision%29) (DamageType :type Damage%20Type%20Object%20Reference) (InstigatedBy :type Controller%20Object%20Reference) (DamageCauser :type Actor%20Object%20Reference))
  ;[1 1 1] Take damage Overrided
  (Actor|DestroyActor))

(event EventUpdateAnimation
  ;[1 1 1] Update Animation Overrided
)

(event EventChaseHuman
  (bind _returnvalue (Transformation|GetActorLocation))
  (bind _defaultlocation (Variables|Default|GetDefaultLocation))
  ;[1 1 1] Moving Left/Right when in range
  (bind _incamerablock_ (CallFunction|IsinCameraBlock))
  (if _incamerablock_
    (bind _asenemy_big_controller (Utilities|Casting|CastToEnemyBigController (AI|GetAIController self)))
    (if (Variables|Default|GetisEnemyRight?)
      (AI|Navigation|MovetoLocation _asenemy_big_controller (Math|Vector|MakeVector (+ (.x _returnvalue) 1e+02) (.y _returnvalue) (.z _defaultlocation)) 0.0 true false false false 0 false)
      (else
        (AI|Navigation|MovetoLocation _asenemy_big_controller (Math|Vector|MakeVector (- (.x _returnvalue) 1e+02) (.y _returnvalue) (.z _defaultlocation)) 0.0 true false false false 0 false)))))

(fn ConstructionScript
  (|CallParentFunction))

(fn SetCurrentHeight)