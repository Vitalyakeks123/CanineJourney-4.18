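; EnemyRunner is an enemy Blueprint that overrides the inherited chase and damage events with empty bodies, so it adds no response to them.
; Its RunRight function casts its AI controller to EnemyBigController and issues a MoveToLocation to a point far along world +X.
; The move bypasses pathfinding, sending the runner in a straight line.
; Nothing in this Blueprint calls RunRight.
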(event EventBeginPlay
  (|CallParentFunction) ; This node is disabled and will not be called.\nDrag off pins to build functionality.
)

(event Collision|EventActorBeginOverlap
  (params (OtherActor :type Actor%20Object%20Reference))
  (|CallParentFunction OtherActor) ; This node is disabled and will not be called.\nDrag off pins to build functionality.
)

(event EventTick
  (params (DeltaSeconds :type Float%20%28single-precision%29))
  (|CallParentFunction DeltaSeconds) ; This node is disabled and will not be called.\nDrag off pins to build functionality.
)

(event EventChaseDog
  ;[1 1 1] Overrided functions
)

(event EventDamageHuman
  ;[1 1 1] Overrided functions
)

(event EventChaseHuman
  ;[1 1 1] Overrided functions
)

(event EventDamageDog
  ;[1 1 1] Overrided functions
)

(event Game|Damage|EventAnyDamage
  (params (Damage :type Float%20%28single-precision%29) (DamageType :type Damage%20Type%20Object%20Reference) (InstigatedBy :type Controller%20Object%20Reference) (DamageCauser :type Actor%20Object%20Reference))
  ;[1 1 1] Overrided functions
)

(fn ConstructionScript
  (|CallParentFunction))

(fn RunRight
  (bind _returnvalue (Transformation|GetActorLocation))
  (bind _asenemy_big_controller (Utilities|Casting|CastToEnemyBigController (AI|GetAIController self)))
  (AI|Navigation|MovetoLocation _asenemy_big_controller (Math|Vector|MakeVector (+ (.x _returnvalue) 99999.0) (.y _returnvalue) (.z _returnvalue)) 1.0 true false false))