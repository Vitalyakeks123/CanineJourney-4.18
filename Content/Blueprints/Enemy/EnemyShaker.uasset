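; Paper2D enemy Shaker that attacks with a ground shockwave instead of chasing, extending a base enemy with empty chase and damage overrides.
; Tick turns it toward its target and, on cooldown while grounded and in the camera block, starts a brief attack animation.
; EndWaving then spawns a line of ShakerWave actors with staggered lifespans, stopping where ground ends.
; Hits apply knockback by melee or ranged type, stun, and health loss.
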(event EventBeginPlay
  (|CallParentFunction) ; This node is disabled and will not be called.\nDrag off pins to build functionality.
)

(event Game|Damage|EventAnyDamage
  (params (Damage :type Float%20%28single-precision%29) (DamageType :type Damage%20Type%20Object%20Reference) (InstigatedBy :type Controller%20Object%20Reference) (DamageCauser :type Actor%20Object%20Reference))
  ;[1 1 1] ApplyDamage
  (Utilities|FlowControl|Sequence
    (:then_0
      (Utilities|Casting|CastToHumanDamageRanged DamageType)
      (Variables|Default|SetPushX 2e+02)
      (Variables|Default|SetPushZ 2e+02))
    (:then_1
      (Utilities|Casting|CastToHumanDamageMelee DamageType)
      (Variables|Default|SetPushX 1.5e+02)
      (Variables|Default|SetPushZ 3e+02))
    (:then_2
      (if (and (> Damage 1.0) (<= (Variables|Default|GetDamageTime) 0.0))
        (CallFunction|LaunchEnemyonHit DamageCauser)
        (Variables|Default|SetDamageTime (Variables|Default|GetDamageTime_const))
        (Variables|/Script/Engine.CharacterMovementComponent|SetMaxWalkSpeed (Variables|Character|GetCharacterMovement) 0.0)
        (Utilities|Time|SetTimerbyFunctionName 0 "ResetMovement" (Variables|Default|GetDamageStun))
        (bind _output_get (Variables|Default|SetHealth (- (Variables|Default|GetHealth) Damage)))
        (if (<= _output_get 0.0)
          (Actor|DestroyActor))))))

(event EventTick
  (params (DeltaSeconds :type Float%20%28single-precision%29))
  (|CallParentFunction DeltaSeconds)
  (CallFunction|TimeChange)
  (CallFunction|RotateCharge))

(event EventUpdateAnimation
  (bind _sprite (Variables|Default|GetSprite))
  ;[1 1 1] Handle Animation
  (Utilities|FlowControl|Sequence
    (:then_0
      ;[1 1 1] State machine
      (if (> (Math|Vector|VectorLength (Transformation|GetVelocity)) 0.0)
        (Variables|Default|SetState "NewEnumerator0")
        (else
          (Variables|Default|SetState "NewEnumerator0"))))
    (:then_1
      (if (Variables|Shaker|GetisWaving?)
        (Variables|Default|SetState "NewEnumerator6")))
    (:then_2
      (switch Utilities|FlowControl|Switch|SwitchonHumanState (Variables|Default|GetState)
        (:NewEnumerator0
          (Sprite|SetFlipbook _sprite "/Game/Sprites/Enemy/Shaker/shaker_idle_anim.shaker_idle_anim"))
        (:NewEnumerator1
          (Sprite|SetFlipbook _sprite "/Game/Sprites/Enemy/Shaker/shaker_idle_anim.shaker_idle_anim"))
        (:NewEnumerator2
          (Sprite|SetFlipbook (Variables|Default|GetSprite) "/Game/Sprites/Enemy/Shaker/shaker_idle_anim.shaker_idle_anim"))
        (:NewEnumerator6
          (Sprite|SetFlipbook (Variables|Default|GetSprite) "/Game/Sprites/Enemy/Shaker/shaker_attack_anim.shaker_attack_anim"))))))

(event EventChaseHuman
  ;[1 1 1] Overrided functions
)

(event EventDamageHuman
  ;[1 1 1] Overrided functions
)

(fn ConstructionScript
  (|CallParentFunction))

(fn TimeChange
  (Utilities|FlowControl|Sequence
    (:then_0
      ;[1 1 1] ChargeCD update
      (bind _output_get (Variables|Shaker|SetShakeCD (- (Variables|Shaker|GetShakeCD) (Utilities|Time|GetWorldDeltaSeconds))))
      (if (Math|Boolean|ANDBoolean (<= _output_get 0.0) (Utilities|Enum|Equal(Enum) (Variables|Default|GetEnemyState) "NewEnumerator2") (not (AI|Components|NavMovement|IsFalling (Variables|Character|GetCharacterMovement))))
        (if (Math|Boolean|Equal(Boolean) (Variables|Default|GetbisMovingRight) (Variables|Default|GetisEnemyRight?))
          (Variables|Shaker|SetShakeCD (Variables|Shaker|GetShakeCD_const))
          (CallFunction|SpawnWave))))))

(fn ChargeStartCasting
  (Variables|Shaker|SetShakeCD (Variables|Shaker|GetShakeCD_const))
  (if (Variables|Default|GetbisMovingRight)
    (Character|LaunchCharacter (Math|Vector|MakeVector 0.0 0.0 0.0) true true)
    (else
      (Character|LaunchCharacter (Math|Vector|MakeVector (* 0.0 -1.0) 0.0 0.0) true true))))

(fn RotateCharge
  (if (Utilities|Enum|Equal(Enum) (Variables|Default|GetEnemyState) "NewEnumerator2")
    (Utilities|FlowControl|Sequence
      (:then_0
        (if (and (Variables|Default|GetbisMovingRight) (not (Variables|Default|GetisEnemyRight?)))
          (Transformation|SetActorRotation "0,180.000000, 0")
          (Variables|Default|SetbisMovingRight false)))
      (:then_1
        (if (and (not (Variables|Default|GetbisMovingRight)) (Variables|Default|GetisEnemyRight?))
          (Transformation|SetActorRotation "0, 0, 0")
          (Variables|Default|SetbisMovingRight true))))))

(fn SpawnWave
  (bind _incamerablock_ (CallFunction|IsinCameraBlock))
  (if _incamerablock_
    (Variables|Shaker|SetisWaving? true)
    (Utilities|Time|SetTimerbyFunctionName 0 "EndWaving" 0.35)))

(fn EndWaving
  (bind _returnvalue (Transformation|GetActorLocation))
  (Variables|Shaker|SetisWaving? false)
  (bind _index (Utilities|FlowControl|ForLoopwithBreak 1 (Variables|Shaker|GetWaveCount) :!label _label)
    (:LoopBody
      (if (Variables|Default|GetisEnemyRight?)
        (LocalVariables|SetSpawnX (+ (.x _returnvalue) (* _index 64.0)))
        (else
          (LocalVariables|SetSpawnX (- (.x _returnvalue) (* _index 64.0)))))
      ;[1 1 1] Spawn Wave
      (bind _returnvalue_2 (Game|SpawnActorfromClass "/Game/Blueprints/Enemy/Projectiles/ShakerWave.ShakerWave_C" (Math|Transform|MakeTransform (Math|Vector|MakeVector (LocalVariables|GetSpawnX) 0.0 (- (.z _returnvalue) 32.0)) "0, 0, 0" "1,1,1") "AlwaysSpawn" 0 0))
      (Actor|SetLifeSpan _returnvalue_2 (* (- _index 1) (Variables|Shaker|GetExplosiondDelay)))
      (bind _onground_ (Default|CheckIsonGround _returnvalue_2))
      (if _onground_
        (if (== _index 1)
          (Actor|DestroyActor _returnvalue_2))
        (else
          (goto _label Break))))))