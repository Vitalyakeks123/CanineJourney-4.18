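; EnemyArkadiy is a Paper2D side-scrolling enemy that extends a parent enemy, patrolling or running between left and right positions when the player gets close.
; Self-rescheduling timers randomly trigger projectile casts, jumps, and leaps that drop a GamblingBomb.
; Tick drives state and flipbooks and lets it rise through WorldStatic geometry, while zone events redirect or launch it.
; Human ranged and melee damage briefly stuns it, with a hit cooldown.
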(event Custom|EndZone
  (params (isRight? :type Boolean))
  ;[1 1 1] Change Location in the End
  (Variables|Running|SetisRunning? true)
  (if isRight?
    (Variables|Running|SetMovingLocation (Transformation|GetActorLocation (Variables|Running|GetRightPosition)))
    (else
      (Variables|Running|SetMovingLocation (Transformation|GetActorLocation (Variables|Running|GetLeftPosition)))))
  (bind _asenemy_big_controller (Utilities|Casting|CastToEnemyBigController (AI|GetAIController self)))
  (AI|Navigation|MovetoLocation _asenemy_big_controller (Variables|Running|GetMovingLocation) 1.0 true false false)
  (Utilities|Time|SetTimerbyFunctionName 0 "ResetRunningCooldown" (Variables|Running|GetRunningCooldown)))

(event Custom|JumpZone
  (params (JumpForce :type Vector))
  (if (not (AI|Components|NavMovement|IsFalling (Variables|Character|GetCharacterMovement)))
    (if (<= (Math|Random|RandomIntegerinRange 0 10) 5)
      (Components|Movement|StopMovementImmediately (Variables|Character|GetCharacterMovement))
      (Collision|SetCollisionResponsetoChannel (Variables|Default|GetCapsuleComponent) "ECC_WorldStatic" "ECR_Ignore")
      (Character|LaunchCharacter JumpForce true true))))

(event EventBeginPlay
  (|CallParentFunction)
  (Utilities|Time|SetTimerbyFunctionName 0 "TryLeap" (Variables|Leap|GetLeapCooldown))
  (Utilities|Time|SetTimerbyFunctionName 0 "TryCast" (Variables|Arkadiy|GetProjectileCooldown)))

(event Collision|EventActorBeginOverlap
  (params (OtherActor :type Actor%20Object%20Reference))
  (|CallParentFunction OtherActor))

(event Game|Damage|EventAnyDamage
  (params (Damage :type Float%20%28single-precision%29) (DamageType :type Damage%20Type%20Object%20Reference) (InstigatedBy :type Controller%20Object%20Reference) (DamageCauser :type Actor%20Object%20Reference))
  ;[1 1 1] ApplyDamage overrite
  (Utilities|FlowControl|Sequence
    (:then_0
      (Utilities|Casting|CastToHumanDamageRanged DamageType)
      (Variables|Default|SetPushX 2e+02)
      (Variables|Default|SetPushZ 2e+02))
    (:then_1
      (Utilities|Casting|CastToHumanDamageMelee DamageType)
      (Variables|Default|SetPushX 4e+02)
      (Variables|Default|SetPushZ 3e+02)))
  (if (and (> Damage 0.0) (<= (Variables|Default|GetDamageTime) 0.0))
    (Variables|Default|SetDamageTime (Variables|Default|GetDamageTime_const))
    (Variables|/Script/Engine.CharacterMovementComponent|SetMaxWalkSpeed (Variables|Character|GetCharacterMovement) 0.0)
    (Utilities|Time|SetTimerbyFunctionName 0 "ResetMovement" (Variables|Default|GetDamageStun))
    (bind _output_get (Variables|Default|SetHealth (- (Variables|Default|GetHealth) Damage)))
    (if (<= _output_get 0.0)
      (Actor|DestroyActor))))

(event EventUpdateAnimation
  (bind _sprite (Variables|Default|GetSprite))
  ;[1 1 1] Handle Animation
  (Utilities|FlowControl|Sequence
    (:then_0
      ;[1 1 1] State machine
      (if (> (Math|Vector|VectorLength (Transformation|GetVelocity)) 0.0)
        (Variables|Default|SetState "NewEnumerator1")
        (else
          (Variables|Default|SetState "NewEnumerator0"))))
    (:then_2
      (switch Utilities|FlowControl|Switch|SwitchonHumanState (Variables|Default|GetState)
        (:NewEnumerator0
          (Sprite|SetFlipbook _sprite "/Game/Sprites/Enemy/Arkadiy/jet_idle_anim.jet_idle_anim"))
        (:NewEnumerator1
          (Sprite|SetFlipbook _sprite "/Game/Sprites/Enemy/Arkadiy/jet_walk_anim.jet_walk_anim"))))))

(event EventTick
  (params (DeltaSeconds :type Float%20%28single-precision%29))
  (bind _capsulecomponent (Variables|Default|GetCapsuleComponent))
  ;[1 1 1] Event Tick
  (CallFunction|UpdateAnimation)
  (CallFunction|TickVariables)
  (Utilities|FlowControl|Sequence
    (:then_0
      (if (<= (.z (Transformation|GetVelocity)) 0.0)
        (Collision|SetCollisionResponsetoChannel _capsulecomponent "ECC_WorldStatic" "ECR_Block")
        (else
          (Collision|SetCollisionResponsetoChannel _capsulecomponent "ECC_WorldStatic" "ECR_Ignore"))))
    (:then_1
      (CallFunction|ChangeState)
      (switch Utilities|FlowControl|Switch|SwitchonEnemyState (Variables|Default|GetEnemyState)
        (:NewEnumerator0
          (if (Variables|Default|GetisPatroling?)
            (CallFunction|StatePatroling)))
        (:NewEnumerator2
          (if (Math|Boolean|ANDBoolean (not (Variables|Arkadiy|GetisJumping?)) (not (Variables|Arkadiy|GetisCasting?)) (not (Variables|Arkadiy|GetisUsingAttack?)))
            (CallFunction|ChaseHuman)
            (CallFunction|CheckforRotation)))))))

(event EventChaseHuman
  (bind _returnvalue (Transformation|GetActorLocation))
  (bind _returnvalue_2 (Game|GetPlayerCharacter 0))
  (bind _returnvalue_3 (Transformation|GetActorLocation _returnvalue_2))
  ;[1 1 1] Overrided Chase Human
  (bind _incamerablock_ (CallFunction|IsinCameraBlock))
  (if _incamerablock_
    (bind _asenemy_big_controller (Utilities|Casting|CastToEnemyBigController (AI|GetAIController self)))
    (if (not (Variables|Running|GetisRunning?))
      (if (and (<= (Math|Float|Absolute(Float) (- (.x _returnvalue) (.x _returnvalue_3))) 2.5e+02) (<= (Math|Float|Absolute(Float) (- (.z _returnvalue) (.z _returnvalue_3))) 1e+02))
        (if (Variables|Default|GetisEnemyRight?)
          (Variables|Running|SetMovingLocation (Transformation|GetActorLocation (Variables|Running|GetLeftPosition)))
          (else
            (Variables|Running|SetMovingLocation (Transformation|GetActorLocation (Variables|Running|GetRightPosition)))))
        (AI|Navigation|MovetoLocation _asenemy_big_controller (Variables|Running|GetMovingLocation) 1.0 true false false)
        (Variables|Running|SetisRunning? true)
        (Utilities|Time|SetTimerbyFunctionName 0 "ResetRunningCooldown" 0.5)))))

(event EventOnLanded
  (params (Hit :type Hit%20Result%20Structure%20%28by%20ref%29))
  ;[1 1 1] Event OnLanded - Reset Jump Cooldown if was in Jump
  (Utilities|FlowControl|Sequence
    (:then_0
      (if (Variables|Arkadiy|GetisJumping?)
        (Variables|Arkadiy|SetisJumping? false)
        (Utilities|Time|SetTimerbyFunctionName 0 "ResetJumpCooldown" (Variables|Arkadiy|GetJumpCooldown))))
    (:then_1
      (if (Variables|Leap|GetisLeaping?)
        (Variables|Leap|SetisLeaping? false)
        (Utilities|Time|SetTimerbyFunctionName 0 "ResetLeapCooldown" (Variables|Leap|GetLeapCooldown))))))

(fn ConstructionScript
  (|CallParentFunction))

(fn ResetJumpCooldown
  (Variables|Arkadiy|SetcanJump? true)
  (CallFunction|TryJump))

(fn TryJump
  (bind _jumpforce (Variables|Arkadiy|GetJumpForce))
  (bind _jumpforcerandomize (Variables|Arkadiy|GetJumpForceRandomize))
  (bind _jumprange (Variables|Arkadiy|GetJumpRange))
  (bind _returnvalue (Math|Random|RandomFloatinRange 0.0 _jumpforcerandomize))
  (bind _returnvalue_2 (+ _jumpforce _returnvalue))
  (if (<= (Math|Random|RandomIntegerinRange 0 10) 4)
    (if (Math|Boolean|ANDBoolean (Variables|Arkadiy|GetcanJump?) (not (AI|Components|NavMovement|IsFalling (Variables|Character|GetCharacterMovement))) (not (Variables|Arkadiy|GetisJumping?)) (Utilities|Enum|Equal(Enum) (Variables|Default|GetEnemyState) "NewEnumerator2") (not (Variables|Arkadiy|GetisCasting?)) (not (Variables|Arkadiy|GetisUsingAttack?)))
      (Variables|Arkadiy|SetcanJump? false)
      (Variables|Arkadiy|SetisJumping? true)
      (Components|Movement|StopMovementImmediately (Variables|Character|GetCharacterMovement))
      (if (Variables|Default|GetisEnemyRight?)
        (Character|LaunchCharacter (Math|Vector|MakeVector _jumprange 0.0 _returnvalue_2) true true)
        (Variables|Arkadiy|SetJumpingRight? true)
        (else
          (Character|LaunchCharacter (Math|Vector|MakeVector (* _jumprange -1.0) 0.0 _returnvalue_2) true true)
          (Variables|Arkadiy|SetJumpingRight? false)))
      (else
        (Utilities|Time|SetTimerbyFunctionName 0 "TryJump" (Variables|Arkadiy|GetJumpCooldown) :!label _label)))
    (else
      (goto _label))))

(fn TryCast
  (if (<= (Math|Random|RandomIntegerinRange 0 10) 5)
    (if (Math|Boolean|ANDBoolean (Variables|Arkadiy|GetcanCast?) (not (AI|Components|NavMovement|IsFalling (Variables|Character|GetCharacterMovement))) (Utilities|Enum|Equal(Enum) (Variables|Default|GetEnemyState) "NewEnumerator2") (not (Variables|Arkadiy|GetisCasting?)))
      (Variables|Arkadiy|SetcanCast? false)
      (Variables|Arkadiy|SetisCasting? true)
      (Utilities|Time|SetTimerbyFunctionName 0 "RangeAttack" (Variables|Arkadiy|GetCastingDuration))
      (Components|Movement|StopMovementImmediately (Variables|Character|GetCharacterMovement))
      (if (Variables|Default|GetisEnemyRight?)
        (Transformation|SetActorRotation (Math|Rotator|MakeRotator 0.0 0.0 0.0))
        (else
          (Transformation|SetActorRotation (Math|Rotator|MakeRotator 0.0 0.0 1.8e+02))))
      (else
        (Utilities|Time|SetTimerbyFunctionName 0 "TryCast" (Variables|Arkadiy|GetProjectileCooldown) :!label _label)))
    (else
      (goto _label))))

(fn RangeAttack
  (Variables|Arkadiy|SetisUsingAttack? true)
  (Variables|Arkadiy|SetisCasting? false)
  (CallFunction|EndRangeAttack))

(fn EndRangeAttack
  (Variables|Arkadiy|SetisUsingAttack? false)
  (Variables|Arkadiy|SetcanCast? true)
  (Utilities|Time|SetTimerbyFunctionName 0 "TryCast" (Variables|Arkadiy|GetProjectileCooldown))
  (Game|SpawnActorfromClass "/Game/Blueprints/Enemy/Projectiles/EnemyGenadyiProjectile.EnemyGenadyiProjectile_C" (Transformation|GetWorldTransform (Variables|Default|GetProjectileArrow)) "AlwaysSpawn" 0 0)
  (Audio|PlaySound2D "/Game/StarterContent/Audio/zvuki_dlya_igri/ydar_vraga.ydar_vraga")
  (bind _asenemy_big_controller (Utilities|Casting|CastToEnemyBigController (AI|GetAIController self)))
  (AI|Navigation|MovetoLocation _asenemy_big_controller (Variables|Running|GetMovingLocation) 1.0 true false false))

(fn TryLeap
  (bind _returnvalue (Transformation|GetActorLocation))
  (bind _leaprange (Variables|Leap|GetLeapRange))
  (bind _leapheight (Variables|Leap|GetLeapHeight))
  (if (<= (Math|Random|RandomIntegerinRange 0 10) 5)
    (if (Math|Boolean|ANDBoolean (not (AI|Components|NavMovement|IsFalling (Variables|Character|GetCharacterMovement))) (not (Variables|Leap|GetisLeaping?)) (Utilities|Enum|Equal(Enum) (Variables|Default|GetEnemyState) "NewEnumerator2") (Variables|Leap|GetcanLeap?))
      (Variables|Leap|SetcanLeap? false)
      (Variables|Leap|SetisLeaping? true)
      (Components|Movement|StopMovementImmediately (Variables|Character|GetCharacterMovement))
      (if (>= (.x (Variables|Running|GetMovingLocation)) (.x (Transformation|GetActorLocation)))
        (Character|LaunchCharacter (Math|Vector|MakeVector _leaprange 0.0 _leapheight) true true)
        (else
          (Character|LaunchCharacter (Math|Vector|MakeVector (* _leaprange -1.0) 0.0 _leapheight) true true)))
      (Game|SpawnActorfromClass "/Game/Blueprints/Gambling/GamblingBomb.GamblingBomb_C" (Math|Transform|MakeTransform (Math|Vector|MakeVector (.x _returnvalue) (.y _returnvalue) (+ (.z _returnvalue) 1e+01)) "0, 0, 0" "1,1,1") "AlwaysSpawn" 0 0)
      (else
        (Utilities|Time|SetTimerbyFunctionName 0 "TryLeap" (Variables|Leap|GetLeapCooldown) :!label _label)))
    (else
      (goto _label))))

(fn ResetLeapCooldown
  (Variables|Leap|SetcanLeap? true)
  (CallFunction|TryLeap))

(fn ResetRunningCooldown
  (Variables|Running|SetisRunning? false))