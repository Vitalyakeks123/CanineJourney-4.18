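; EnemyArc is a 2D enemy that periodically spits arcing projectiles, using Slimegril flipbooks for animation.
; Tick counts down cooldown and animation timers, scheduling a delayed throw while in the Frog Jumping or Chasing Human state.
; A moving enemy fires from Arrow2 at random speed.
; Otherwise Arrow1 faces the dog or human by state, with launch speed computed from preset left or right locations and angles.
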(event EventBeginPlay
  (|CallParentFunction) ; This node is disabled and will not be called.\nDrag off pins to build functionality.
)

(event Collision|EventActorBeginOverlap
  (params (OtherActor :type Actor%20Object%20Reference))
  (|CallParentFunction OtherActor) ; This node is disabled and will not be called.\nDrag off pins to build functionality.
)

(event EventTick
  (params (DeltaSeconds :type Float%20%28single-precision%29))
  (|CallParentFunction DeltaSeconds)
  (CallFunction|TimeChange DeltaSeconds))

(event EventUpdateAnimation
  (bind _sprite (Variables|Default|GetSprite))
  ;[1 1 1] Handle Animation
  (Utilities|FlowControl|Sequence
    (:then_0
      ;[1 1 1] State machine
      (if (<= (Variables|Default|GetThrowAnimTime) 0.0)
        (Variables|Default|SetState "NewEnumerator0")
        (else
          (Variables|Default|SetState "NewEnumerator1"))))
    (:then_1
      (if (AI|Components|NavMovement|IsFalling (Variables|Character|GetCharacterMovement))
        (Variables|Default|SetState "NewEnumerator2")
        (Variables|Default|SetIsThrowing? false)))
    (:then_2
      (switch Utilities|FlowControl|Switch|SwitchonHumanState (Variables|Default|GetState)
        (:NewEnumerator0
          (Sprite|SetFlipbook _sprite "/Game/Sprites/Slime/Slimegril.Slimegril"))
        (:NewEnumerator1
          (Sprite|SetFlipbook _sprite "/Game/Sprites/Slime/Slimegril_spit.Slimegril_spit"))
        (:NewEnumerator2
          (Sprite|SetFlipbook (Variables|Default|GetSprite) "/Game/Sprites/Slime/Slimegril.Slimegril"))))))

(event EventDamageHuman
  ;[1 1 1] Overrided damage handlers
)

(event EventDamageDog
  ;[1 1 1] Overrided damage handlers
)

(fn ConstructionScript
  (|CallParentFunction))

(fn TimeChange
  (params (Delta :type Float%20%28single-precision%29))
  (bind _output_get (Variables|Default|SetTimeThrow (Math|Float|Clamp(Float) (- (Variables|Default|GetTimeThrow) Delta) 0.0 123.0)))
  (Variables|Default|SetThrowAnimTime (Math|Float|Clamp(Float) (- (Variables|Default|GetThrowAnimTime) Delta) 0.0 123.0))
  (if (<= _output_get 0.0)
    (switch Utilities|FlowControl|Switch|SwitchonEnemyState (Variables|Default|GetEnemyState)
      (:NewEnumerator1
        _)
      (:NewEnumerator2
        _))
    (Utilities|Time|SetTimerbyFunctionName 0 "ThrowProjectile" 0.3)
    (Variables|Default|SetTimeThrow (Variables|Default|GetDamageDelay))
    (Variables|Default|SetThrowAnimTime 0.41)))

(fn ThrowProjectile
  (Audio|PlaySound2D "/Game/StarterContent/Audio/zvuki_dlya_igri/ydar_vraga_arka.ydar_vraga_arka")
  (if (Variables|Enemy|GetisMoving?)
    (Game|SpawnActorfromClass "/Game/Blueprints/Enemy/Projectiles/EnemyArcProjectile.EnemyArcProjectile_C" (Transformation|GetWorldTransform (Variables|Default|GetArrow2)) "AlwaysSpawn" 0 (Math|Random|RandomFloatinRange 325.0 425.0) 0)
    (else
      (Utilities|FlowControl|Sequence
        (:then_0
          (switch Utilities|FlowControl|Switch|SwitchonEnemyState (Variables|Default|GetEnemyState)
            (:NewEnumerator1
              (bind _ashuman_character (Utilities|Casting|CastToHumanCharacter (Game|GetPlayerCharacter 0)))
              (if (<= (.x (Transformation|GetActorLocation (Variables|/Game/Blueprints/Characters/HumanCharacter.HumanCharacter_C|GetDogReference _ashuman_character))) (.x (Transformation|GetActorLocation)))
                (Transformation|SetWorldRotation (Variables|Default|GetArrow1) (Math|Rotator|MakeRotator 1.8e+02 (Variables|Enemy|GetAngle_Left) 1.8e+02) false false :!label _label)
                (bind _speed (CallFunction|GetSpeed (Variables|Enemy|GetLocation_Left) (Variables|Enemy|GetAngle_Left)))
                (LocalVariables|SetTempSpeed _speed)
                (else
                  (Transformation|SetWorldRotation (Variables|Default|GetArrow1) (Math|Rotator|MakeRotator 0.0 (Variables|Enemy|GetAngle_Right) 0.0) false false :!label _label_2)
                  (bind _speed_2 (CallFunction|GetSpeed (Variables|Enemy|GetLocation_Right) (Variables|Enemy|GetAngle_Right)))
                  (LocalVariables|SetTempSpeed _speed_2))))
            (:NewEnumerator2
              (bind _ashuman_character_2 (Utilities|Casting|CastToHumanCharacter (Game|GetPlayerCharacter 0)))
              (if (<= (.x (Transformation|GetActorLocation _ashuman_character_2)) (.x (Transformation|GetActorLocation)))
                (goto _label)
                (else
                  (goto _label_2))))))
        (:then_1
          (Game|SpawnActorfromClass "/Game/Blueprints/Enemy/Projectiles/EnemyArcProjectile.EnemyArcProjectile_C" (Transformation|GetWorldTransform (Variables|Default|GetArrow1)) "AlwaysSpawn" 0 (LocalVariables|GetTempSpeed) 0))))))

(fn GetSpeed
  (params (Location :type Vector) (Angle :type Float%20%28single-precision%29))
  (bind _returnvalue (Transformation|GetActorLocation))
  (bind (_x _y _z) (Math|Vector|BreakVector Location))
  (bind (_x_2 _y_2 _z_2) (Math|Vector|BreakVector _returnvalue))
  (bind _output_get (LocalVariables|SetTempSpeed (Math|Float|Sqrt (/ (* (Math|Float|Absolute(Float) (- (Math|Float|Absolute(Float) (- _x _x_2)) (/ (Math|Float|Absolute(Float) (* (Math|Trig|Tan(Degrees) (- 9e+01 Angle)) (Math|Float|Absolute(Float) (- _z _z_2)))) 2.0))) 4e+04) (* Angle 2.0)))))
  (return _output_get))