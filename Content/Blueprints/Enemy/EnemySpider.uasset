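; Spider enemy that shuttles vertically between its spawn point and a lower BotLocation, and is destroyed by any damage.
; Chained timers alternate descent and climb, using randomized pauses and a travel time estimated from distance and fly speed rather than detecting arrival.
; Tick reissues a non-pathfinding AI MoveTo while the IsInCameraBlock check passes, and updates the cable's end so the web stays anchored at the top.
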(event EventBeginPlay
  ;[1 1 1] Begin Play
  (|CallParentFunction)
  (Variables|/Script/Engine.CharacterMovementComponent|SetMaxFlySpeed (Variables|Character|GetCharacterMovement) (Variables|Default|GetMoveSpeed))
  (Variables|Spider|SetTopLocation (Transformation|GetActorLocation))
  (Variables|Spider|SetMoveTime (/ (Math|Vector|VectorLength (- (Variables|Spider|GetTopLocation) (Variables|Spider|GetBotLocation))) (Variables|Default|GetMoveSpeed)))
  (Utilities|Time|SetTimerbyFunctionName 0 "Top2Down" (+ (Variables|Spider|GetTopDelay) (Math|Random|RandomFloatinRange 0.0 (Variables|Spider|GetRandomDelay)))))

(event Collision|EventActorBeginOverlap
  (params (OtherActor :type Actor%20Object%20Reference))
  (|CallParentFunction OtherActor))

(event EventTick
  (params (DeltaSeconds :type Float%20%28single-precision%29))
  ;[1 1 1] Overrided EventTick
  (CallFunction|MoveSpider)
  (CallFunction|SpiderSetWeb))

(event Game|Damage|EventAnyDamage
  (params (Damage :type Float%20%28single-precision%29) (DamageType :type Damage%20Type%20Object%20Reference) (InstigatedBy :type Controller%20Object%20Reference) (DamageCauser :type Actor%20Object%20Reference))
  ;[1 1 1] Take damage overrided
  (Actor|DestroyActor))

(event EventUpdateAnimation
  ;[1 1 1] Update animation overrided
)

(fn ConstructionScript
  (|CallParentFunction))

(fn Top2Down
  (bind _botlocation (Variables|Spider|GetBotLocation))
  (Variables|Spider|SetMovingLocation (Math|Vector|MakeVector (.x _botlocation) (.y _botlocation) (- (.z _botlocation) 45.0)))
  (Variables|Spider|SetIsMoving? true)
  (CallFunction|MoveSpider)
  (Utilities|Time|SetTimerbyFunctionName 0 "CheckForLocation" (Variables|Spider|GetMoveTime)))

(fn Down2Top
  (Variables|Spider|SetMovingLocation (Variables|Spider|GetTopLocation))
  (Variables|Spider|SetIsMoving? true)
  (CallFunction|MoveSpider)
  (Utilities|Time|SetTimerbyFunctionName 0 "CheckForLocation" (Variables|Spider|GetMoveTime)))

(fn CheckforLocation
  (if (Variables|Spider|GetIsTop?)
    (Variables|Spider|SetIsTop? false)
    (Utilities|Time|SetTimerbyFunctionName 0 "Down2Top" (+ (Variables|Spider|GetBotDelay) (Math|Random|RandomFloatinRange 0.0 (Variables|Spider|GetRandomDelay))))
    (else
      (Variables|Spider|SetIsTop? true)
      (Utilities|Time|SetTimerbyFunctionName 0 "Top2Down" (+ (Variables|Spider|GetTopDelay) (Math|Random|RandomFloatinRange 0.0 (Variables|Spider|GetRandomDelay))))))
  (return))

(fn MoveSpider
  (bind _returnvalue (Transformation|GetActorLocation))
  (if (Variables|Spider|GetIsMoving?)
    (bind _incamerablock_ (CallFunction|IsinCameraBlock))
    (if _incamerablock_
      (bind _asenemy_big_controller (Utilities|Casting|CastToEnemyBigController (AI|GetAIController self)))
      (AI|Navigation|MovetoLocation _asenemy_big_controller (Math|Vector|MakeVector (.x _returnvalue) (.y _returnvalue) (.z (Variables|Spider|GetMovingLocation))) 1.0 false false false false 0 false))))

(fn SpiderSetWeb
  (bind _returnvalue (Transformation|GetActorLocation))
  (bind _toplocation (Variables|Spider|GetTopLocation))
  (bind _returnvalue_2 (- _toplocation _returnvalue))
  (Variables|/Script/CableComponent.CableComponent|SetEndLocation (Variables|Default|GetCable) (Math|Vector|MakeVector (.x _returnvalue_2) (.y _returnvalue_2) (+ (.z _returnvalue_2) 5.0))))