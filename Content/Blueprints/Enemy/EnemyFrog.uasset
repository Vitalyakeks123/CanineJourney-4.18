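; Frog enemy that attacks by leaping horizontally in its facing direction, overriding the inherited DamageHuman and ChaseHuman events with empty ones.
; Tick runs a jump countdown and, in one EnemyState, flips facing to match IsEnemyRight and launches the frog when grounded and aligned.
; While airborne from a jump, it damages overlapping HumanCharacters every tick.
; Landing clears the jump flag and restarts the countdown.
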(event EventBeginPlay
  (|CallParentFunction) ; This node is disabled and will not be called.\nDrag off pins to build functionality.
)

(event EventTick
  (params (DeltaSeconds :type Float%20%28single-precision%29))
  (|CallParentFunction DeltaSeconds)
  (CallFunction|TimeChange)
  (CallFunction|RotateFrog)
  (CallFunction|CheckforDamage))

(event EventChaseHuman
  ;[1 1 1] Overrided functions
)

(event EventDamageHuman
  ;[1 1 1] Overrided functions
)

(event EventOnLanded
  (params (Hit :type Hit%20Result%20Structure%20%28by%20ref%29))
  (if (Variables|Frog|GetisInJump?)
    (Variables|Frog|SetisInJump? false)
    (Variables|Frog|SetFrogJump (Variables|Frog|GetFrogJump_const))))

(fn ConstructionScript
  (|CallParentFunction))

(fn TimeChange
  (bind _output_get (Variables|Frog|SetFrogJump (- (Variables|Frog|GetFrogJump) (Utilities|Time|GetWorldDeltaSeconds))))
  (if (Math|Boolean|ANDBoolean (<= _output_get 0.0) (Utilities|Enum|Equal(Enum) (Variables|Default|GetEnemyState) "NewEnumerator2") (not (Variables|Frog|GetisInJump?)))
    (if (and (Math|Boolean|Equal(Boolean) (Variables|Default|GetbisMovingRight) (Variables|Default|GetisEnemyRight?)) (not (AI|Components|NavMovement|IsFalling (Variables|Character|GetCharacterMovement))))
      (CallFunction|JumpFrog))))

(fn JumpFrog
  (bind _jumpx (Variables|Frog|GetJumpX))
  (bind _jumpz (Variables|Frog|GetJumpZ))
  (Variables|Frog|SetFrogJump (Variables|Frog|GetFrogJump_const))
  (if (Variables|Default|GetbisMovingRight)
    (Character|LaunchCharacter (Math|Vector|MakeVector _jumpx 0.0 _jumpz) true true)
    (else
      (Character|LaunchCharacter (Math|Vector|MakeVector (* _jumpx -1.0) 0.0 _jumpz) true true)))
  (Variables|Frog|SetisInJump? true))

(fn RotateFrog
  (if (Utilities|Enum|Equal(Enum) (Variables|Default|GetEnemyState) "NewEnumerator2")
    (Utilities|FlowControl|Sequence
      (:then_0
        (if (and (Variables|Default|GetbisMovingRight) (not (Variables|Default|GetisEnemyRight?)))
          (Transformation|SetActorRotation "0,180.000000, 0")
          (Variables|Default|SetbisMovingRight false)))
      (:then_1
        (if (and (not (Variables|Default|GetbisMovingRight)) (Variables|Default|GetisEnemyRight?))
          (Transformation|SetActorRotation "0, 0, 0")
          (Variables|Default|SetbisMovingRight true))))))

(fn CheckforDamage
  (if (Variables|Frog|GetisInJump?)
    (for _array_element (Collision|GetOverlappingActors (Variables|Default|GetDamageCollision) 0 :!class /Script/Engine.PrimitiveComponent)
      (bind _ashuman_character (Utilities|Casting|CastToHumanCharacter _array_element))
      (Game|Damage|ApplyDamage _ashuman_character 1.0 0 self))))