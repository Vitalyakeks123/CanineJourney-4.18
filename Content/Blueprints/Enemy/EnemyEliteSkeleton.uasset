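; Elite skeleton enemy Blueprint that overrides damage behavior and drives its Paper2D flipbook animation.
; UpdateAnimation derives idle, running, jumping or attack state from velocity, falling and the attack flag; jumping reuses the walk flipbook.
; DamageHuman directly damages player 0, halts movement during the brief attack animation and starts a cooldown.
; Function-name timers reschedule DamageHuman, restore movement speed and re-enable attacking.
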(event EventBeginPlay
  (|CallParentFunction) ; This node is disabled and will not be called.\nDrag off pins to build functionality.
)

(event Collision|EventActorBeginOverlap
  (params (OtherActor :type Actor%20Object%20Reference))
  (|CallParentFunction OtherActor) ; This node is disabled and will not be called.\nDrag off pins to build functionality.
)

(event EventTick
  (params (DeltaSeconds :type Float%20%28single-precision%29))
  (|CallParentFunction DeltaSeconds) ; This node is disabled and will not be called.\nDrag off pins to build functionality.
)

(event EventUpdateAnimation
  (bind _sprite (Variables|Default|GetSprite))
  (bind _sprite_2 (Variables|Default|GetSprite))
  ;[1 1 1] Handle Animation
  (Utilities|FlowControl|Sequence
    (:then_0
      ;[1 1 1] State machine
      (if (> (Math|Vector|VectorLength (Transformation|GetVelocity)) 0.0)
        (Variables|Default|SetState "NewEnumerator1")
        (else
          (Variables|Default|SetState "NewEnumerator0"))))
    (:then_1
      (if (AI|Components|NavMovement|IsFalling (Variables|Character|GetCharacterMovement))
        (Variables|Default|SetState "NewEnumerator2")
        (Variables|Default|SetIsThrowing? false)))
    (:then_2
      (if (Variables|Default|GetisAttackAnim?)
        (Variables|Default|SetState "NewEnumerator6")))
    (:then_3
      (switch Utilities|FlowControl|Switch|SwitchonHumanState (Variables|Default|GetState)
        (:NewEnumerator0
          (Sprite|SetFlipbook _sprite_2 "/Game/Sprites/Enemy/EliteSkeleton/elite_skeleton_idle_anim.elite_skeleton_idle_anim")
          (Components|Timeline|SetLooping _sprite_2 true)
          (Audio|Components|Audio|Play _sprite_2))
        (:NewEnumerator1
          (Sprite|SetFlipbook _sprite_2 "/Game/Sprites/Enemy/EliteSkeleton/elite_skeleton_walk_anim.elite_skeleton_walk_anim")
          (Components|Timeline|SetLooping _sprite_2 true)
          (Audio|Components|Audio|Play _sprite_2))
        (:NewEnumerator2
          (Sprite|SetFlipbook _sprite "/Game/Sprites/Enemy/EliteSkeleton/elite_skeleton_walk_anim.elite_skeleton_walk_anim")
          (Components|Timeline|SetLooping _sprite_2 true)
          (Audio|Components|Audio|Play _sprite_2))
        (:NewEnumerator6
          (Sprite|SetFlipbook _sprite "/Game/Sprites/Enemy/EliteSkeleton/elite_attack_anim.elite_attack_anim")
          (Components|Timeline|SetLooping _sprite false))))))

(event EventDamageHuman
  (bind _charactermovement (Variables|Character|GetCharacterMovement))
  ;[1 1 1] Overrited damage
  (if (Math|Boolean|ANDBoolean (<= (Variables|Default|GetDamageTime) 0.0) (not (Variables|Default|GetisAttackAnim?)) (Variables|Elite|GetcanAttack?))
    (Game|Damage|ApplyDamage (Game|GetPlayerCharacter 0) 1.0 0 self)
    (Utilities|Time|SetTimerbyFunctionName 0 "DamageHuman" (Variables|Default|GetDamageDelay))
    (Variables|Default|SetisAttackAnim? true)
    (Utilities|Time|SetTimerbyFunctionName 0 "ResetAttackAnim" 0.35)
    (Variables|/Script/Engine.CharacterMovementComponent|SetMaxWalkSpeed _charactermovement 0.0)
    (Components|Movement|StopMovementImmediately _charactermovement)
    (Utilities|Time|SetTimerbyFunctionName 0 "ResetAttackCooldown" (Variables|Elite|GetAttackCooldown))
    (Variables|Elite|SetcanAttack? false)
    (else
      (Utilities|Time|SetTimerbyFunctionName 0 "DamageHuman" (Variables|Default|GetDamageTime)))))

(fn ConstructionScript
  (|CallParentFunction))

(fn ResetAttackAnim
  (Variables|Default|SetisAttackAnim? false)
  (Variables|/Script/Engine.CharacterMovementComponent|SetMaxWalkSpeed (Variables|Character|GetCharacterMovement) (Variables|Default|GetMoveSpeed)))

(fn ResetAttackCooldown
  (Variables|Elite|SetcanAttack? true))