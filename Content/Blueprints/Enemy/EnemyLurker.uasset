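; Side-view enemy that stalks the human while hidden and immune to damage, then surfaces to leap at them.
; Tick runs a cooldown that, in one enemy state, alternates hidden AI movement with launched jumps, turns it toward its target and damages overlapped humans mid-jump.
; Landing restarts the cooldown.
; When visible, hits cause knockback scaled by ranged or melee damage type, a brief stun and death at zero health.
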(event EventBeginPlay
  (|CallParentFunction) ; This node is disabled and will not be called.\nDrag off pins to build functionality.
)

(event Game|Damage|EventAnyDamage
  (params (Damage :type Float%20%28single-precision%29) (DamageType :type Damage%20Type%20Object%20Reference) (InstigatedBy :type Controller%20Object%20Reference) (DamageCauser :type Actor%20Object%20Reference))
  ;[1 1 1] ApplyDamage
  (Utilities|FlowControl|Sequence
    (:then_0
      (Utilities|Casting|CastToHumanDamageRanged DamageType)
      (Variables|Default|SetPushX 2e+02)
      (Variables|Default|SetPushZ 2e+02))
    (:then_1
      (Utilities|Casting|CastToHumanDamageMelee DamageType)
      (Variables|Default|SetPushX 4e+02)
      (Variables|Default|SetPushZ 3e+02))
    (:then_2
      (if (not (Variables|Lurker|GetisLurked?))
        (if (and (> Damage 0.0) (<= (Variables|Default|GetDamageTime) 0.0))
          (CallFunction|LaunchEnemyonHit DamageCauser)
          (Variables|Default|SetDamageTime (Variables|Default|GetDamageTime_const))
          (Variables|/Script/Engine.CharacterMovementComponent|SetMaxWalkSpeed (Variables|Character|GetCharacterMovement) 0.0)
          (Utilities|Time|SetTimerbyFunctionName 0 "ResetMovement" (Variables|Default|GetDamageStun))
          (bind _output_get (Variables|Default|SetHealth (- (Variables|Default|GetHealth) Damage)))
          (if (<= _output_get 0.0)
            (Actor|DestroyActor)))))))

(event EventChaseHuman
  (bind _returnvalue (Transformation|GetActorLocation))
  ;[1 1 1] Chace human override
  (if (Variables|Lurker|GetisLurked?)
    (bind _asenemy_big_controller (Utilities|Casting|CastToEnemyBigController (AI|GetAIController self)))
    (if (Variables|Default|GetisEnemyRight?)
      (AI|Navigation|MovetoLocation _asenemy_big_controller (Math|Vector|MakeVector (+ (.x _returnvalue) 1e+02) (.y _returnvalue) (.z _returnvalue)) 1.0 true false false)
      (else
        (AI|Navigation|MovetoLocation _asenemy_big_controller (Math|Vector|MakeVector (- (.x _returnvalue) 1e+02) (.y _returnvalue) (.z _returnvalue)) 1.0 true false false)))))

(event EventTick
  (params (DeltaSeconds :type Float%20%28single-precision%29))
  (|CallParentFunction DeltaSeconds)
  (CallFunction|TimeChange)
  (CallFunction|RotateCharge)
  (CallFunction|CheckforDamage))

(event EventOnLanded
  (params (Hit :type Hit%20Result%20Structure%20%28by%20ref%29))
  ;[1 1 1] On landed
  (if (Variables|Lurker|GetisInJump?)
    (Variables|Lurker|SetisInJump? false)
    (Variables|Lurker|SetLurkerCD (Variables|Lurker|GetLurkerCD_const))))

(event EventDamageHuman
  ;[1 1 1] Overrided functions
)

(fn ConstructionScript
  (|CallParentFunction))

(fn TimeChange
  (bind _jumpx (Variables|Lurker|GetJumpX))
  (bind _jumpz (Variables|Lurker|GetJumpZ))
  (bind _sprite (Variables|Default|GetSprite))
  (Utilities|FlowControl|Sequence
    (:then_0
      ;[1 1 1] LurkerCD update
      (bind _output_get (Variables|Lurker|SetLurkerCD (- (Variables|Lurker|GetLurkerCD) (Utilities|Time|GetWorldDeltaSeconds))))
      (if (Math|Boolean|ANDBoolean (<= _output_get 0.0) (Utilities|Enum|Equal(Enum) (Variables|Default|GetEnemyState) "NewEnumerator2") (not (Variables|Lurker|GetisLurked?)) (not (Variables|Lurker|GetisInJump?)))
        (if (Math|Boolean|Equal(Boolean) (Variables|Default|GetbisMovingRight) (Variables|Default|GetisEnemyRight?))
          (Variables|Lurker|SetisInJump? true)
          (Variables|Lurker|SetLurkerCD (Variables|Lurker|GetLurkerCD_const))
          (Components|Movement|StopMovementImmediately (Variables|Character|GetCharacterMovement))
          (if (Variables|Default|GetbisMovingRight)
            (Character|LaunchCharacter (Math|Vector|MakeVector _jumpx 0.0 _jumpz) false true)
            (else
              (Character|LaunchCharacter (Math|Vector|MakeVector (* _jumpx -1.0) 0.0 _jumpz) false true))))))
    (:then_1
      ;[1 1 1] Set is lurked
      (if (Math|Boolean|ANDBoolean (Utilities|Enum|Equal(Enum) (Variables|Default|GetEnemyState) "NewEnumerator2") (> (Variables|Lurker|GetLurkerCD) 0.0) (not (Variables|Lurker|GetisInJump?)))
        (if (not (Variables|Lurker|GetisLurked?))
          (Variables|Lurker|SetisLurked? true)
          (Development|SetHiddeninGame _sprite true false))
        (elif (Variables|Lurker|GetisLurked?)
          (Variables|Lurker|SetisLurked? false)
          (Development|SetHiddeninGame _sprite false false)
          (if (not (Utilities|Enum|Equal(Enum) (Variables|Default|GetEnemyState) "NewEnumerator2"))
            (Components|Movement|StopMovementImmediately (Variables|Character|GetCharacterMovement))))))
    (:then_2
      ;[1 1 1] Lurker is falling
      (if (and (AI|Components|NavMovement|IsFalling (Variables|Character|GetCharacterMovement)) (Variables|Lurker|GetisLurked?))
        (Variables|Lurker|SetLurkerCD 0.0)
        (if (not (Utilities|Enum|Equal(Enum) (Variables|Default|GetEnemyState) "NewEnumerator2"))
          (Components|Movement|StopMovementImmediately (Variables|Character|GetCharacterMovement)))))))

(fn ChargeStartCasting
  (bind _jumpx (Variables|Lurker|GetJumpX))
  (bind _jumpz (Variables|Lurker|GetJumpZ))
  (Variables|Lurker|SetLurkerCD (Variables|Lurker|GetLurkerCD_const))
  (if (Variables|Default|GetbisMovingRight)
    (Character|LaunchCharacter (Math|Vector|MakeVector _jumpx 0.0 _jumpz) true true)
    (else
      (Character|LaunchCharacter (Math|Vector|MakeVector (* _jumpx -1.0) 0.0 _jumpz) true true)))
  (Variables|Lurker|SetisLurked? true))

(fn RotateCharge
  (if (Utilities|Enum|Equal(Enum) (Variables|Default|GetEnemyState) "NewEnumerator2")
    (Utilities|FlowControl|Sequence
      (:then_0
        (if (and (Variables|Default|GetbisMovingRight) (not (Variables|Default|GetisEnemyRight?)))
          (Transformation|SetActorRotation "0,180.000000, 0")
          (Variables|Default|SetbisMovingRight false)))
      (:then_1
        (if (and (not (Variables|Default|GetbisMovingRight)) (Variables|Default|GetisEnemyRight?))
          (Transformation|SetActorRotation "0, 0, 0")
          (Variables|Default|SetbisMovingRight true))))))

(fn CheckforDamage
  (if (and (Variables|Lurker|GetisInJump?) (<= (Variables|Default|GetDamageTime) 0.0))
    (for _array_element (Collision|GetOverlappingActors (Variables|Default|GetDamageCollision) 0 :!class /Script/Engine.PrimitiveComponent)
      (bind _ashuman_character (Utilities|Casting|CastToHumanCharacter _array_element))
      (Game|Damage|ApplyDamage _ashuman_character 1.0 0 self))))