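; Ranged enemy child Blueprint (Slimeurod) that spits projectiles while chasing the human or the dog, with the inherited damage handlers overridden empty.
; Tick counts down a cooldown, then schedules FireProjectile on a short timer, which spawns the projectile at ThrowArrow, snaps it to a fixed Y plane and passes radius and wall flag.
; UpdateAnimation picks Paper2D flipbooks from movement, reusing the Climbing state for spitting and the run flipbook for jumping.
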(event EventBeginPlay
  (|CallParentFunction) ; This node is disabled and will not be called.\nDrag off pins to build functionality.
)

(event Collision|EventActorBeginOverlap
  (params (OtherActor :type Actor%20Object%20Reference))
  (|CallParentFunction OtherActor) ; This node is disabled and will not be called.\nDrag off pins to build functionality.
)

(event EventTick
  (params (DeltaSeconds :type Float%20%28single-precision%29))
  (|CallParentFunction DeltaSeconds)
  (CallFunction|TimeChange DeltaSeconds))

(event EventUpdateAnimation
  (bind _sprite (Variables|Default|GetSprite))
  ;[1 1 1] Handle Animation
  (Utilities|FlowControl|Sequence
    (:then_0
      ;[1 1 1] State machine
      (if (> (Math|Vector|VectorLength (Transformation|GetVelocity)) 0.0)
        (Variables|Default|SetState "NewEnumerator1")
        (elif (<= (Variables|Default|GetThrowAnimTime) 0.0)
          (Variables|Default|SetState "NewEnumerator0")
          (else
            (Variables|Default|SetState "NewEnumerator3")))))
    (:then_1
      (if (AI|Components|NavMovement|IsFalling (Variables|Character|GetCharacterMovement))
        (Variables|Default|SetState "NewEnumerator2")
        (Variables|Default|SetIsThrowing? false)))
    (:then_2
      (switch Utilities|FlowControl|Switch|SwitchonHumanState (Variables|Default|GetState)
        (:NewEnumerator0
          (Sprite|SetFlipbook _sprite "/Game/Sprites/Slime/Slimeurod_idle.Slimeurod_idle"))
        (:NewEnumerator1
          (Sprite|SetFlipbook _sprite "/Game/Sprites/Slime/Slimeurod_run.Slimeurod_run" :!label _label))
        (:NewEnumerator2
          (goto _label))
        (:NewEnumerator3
          (Sprite|SetFlipbook (Variables|Default|GetSprite) "/Game/Sprites/Slime/Slimeurod_spit.Slimeurod_spit"))))))

(event EventDamageHuman
  ;[1 1 1] Overrided damage handlers
)

(event EventDamageDog
  ;[1 1 1] Overrided damage handlers
)

(fn ConstructionScript
  (|CallParentFunction))

(fn FireProjectile
  (Variables|Default|SetThrowAnimTime 0.16)
  (bind _returnvalue (Game|SpawnActorfromClass "/Game/Blueprints/Enemy/Projectiles/EnemyRangedProjectile.EnemyRangedProjectile_C" (Transformation|GetWorldTransform (Variables|Default|GetThrowArrow)) "AlwaysSpawn" 0 0))
  (Audio|PlaySound2D "/Game/StarterContent/Audio/zvuki_dlya_igri/ydar_vraga.ydar_vraga")
  (Utilities|IsValid _returnvalue
    (:Is%20Valid
      (Transformation|SetActorLocation _returnvalue (Math|Vector|MakeVector (.x (Transformation|GetActorLocation _returnvalue)) 5.0 (.z (Transformation|GetActorLocation _returnvalue))) false false)
      (Components|Sphere|SetSphereRadius (Variables|/Game/Blueprints/Enemy/Projectiles/EnemyRangedProjectile.EnemyRangedProjectile_C|GetSphere _returnvalue) (Variables|Enemy|GetProjectileRadius) true)
      (Variables|/Game/Blueprints/Enemy/Projectiles/EnemyRangedProjectile.EnemyRangedProjectile_C|SetIsWall? _returnvalue (Variables|Enemy|GetIsWall?)))))

(fn TimeChange
  (params (Delta :type Float%20%28single-precision%29))
  (bind _output_get (Variables|Default|SetTimeThrow (Math|Float|Clamp(Float) (- (Variables|Default|GetTimeThrow) Delta) 0.0 123.0)))
  (Variables|Default|SetThrowAnimTime (Math|Float|Clamp(Float) (- (Variables|Default|GetThrowAnimTime) Delta) 0.0 123.0))
  (if (<= _output_get 0.0)
    (switch Utilities|FlowControl|Switch|SwitchonEnemyState (Variables|Default|GetEnemyState)
      (:NewEnumerator1
        _)
      (:NewEnumerator2
        _))
    (Utilities|Time|SetTimerbyFunctionName 0 "FireProjectile" 0.3)
    (Variables|Default|SetTimeThrow (Variables|Default|GetDamageDelay))))