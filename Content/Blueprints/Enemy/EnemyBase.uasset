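; Base 2D flipbook enemy character that animates by movement state and takes stunning hits.
; Tick derives idle, running or jumping from velocity and falling to pick the flipbook, and yaws the controller to face horizontal travel.
; Any damage halts walking for a stun timer and removes one health, destroying the actor at zero.
; It also carries jump input with a double jump and stores its spawn location as a patrol origin.
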(event Custom|UpdateAnimation
  (bind _sprite (Variables|Default|GetSprite))
  ;[1 1 1] Handle Animation
  (Utilities|FlowControl|Sequence
    (:then_0
      ;[1 1 1] State machine
      (if (> (Math|Vector|VectorLength (Transformation|GetVelocity)) 0.0)
        (Variables|Movement|SetState "NewEnumerator1")
        (else
          (Variables|Movement|SetState "NewEnumerator0"))))
    (:then_1
      (if (AI|Components|NavMovement|IsFalling (Variables|Character|GetCharacterMovement))
        (Variables|Movement|SetState "NewEnumerator2")
        (Variables|Throw|SetIsThrowing? false)))
    (:then_2
      (switch Utilities|FlowControl|Switch|SwitchonHumanState (Variables|Movement|GetState)
        (:NewEnumerator0
          (Sprite|SetFlipbook _sprite "/Game/Sprites/CharacterHuman/Character_Sprite_Idle.Character_Sprite_Idle"))
        (:NewEnumerator1
          (Sprite|SetFlipbook _sprite "/Game/Sprites/CharacterHuman/Character_Sprite_Run.Character_Sprite_Run"))
        (:NewEnumerator2
          (Sprite|SetFlipbook (Variables|Default|GetSprite) "/Game/Sprites/CharacterHuman/Character_Sprite_Jump.Character_Sprite_Jump"))))))

(event Game|Damage|EventAnyDamage
  (params (Damage :type Float%20%28single-precision%29) (DamageType :type Damage%20Type%20Object%20Reference) (InstigatedBy :type Controller%20Object%20Reference) (DamageCauser :type Actor%20Object%20Reference))
  (if (> Damage 0.0)
    (Variables|/Script/Engine.CharacterMovementComponent|SetMaxWalkSpeed (Variables|Character|GetCharacterMovement) 0.0)
    (Utilities|Time|SetTimerbyFunctionName 0 "ResetMovement" (Variables|Enemy|GetDamageStun))
    (bind _output_get (Variables|Enemy|SetHealth (- (Variables|Enemy|GetHealth) 1.0)))
    (if (<= _output_get 0.0)
      (Actor|DestroyActor))))

(event EventTick
  (params (DeltaSeconds :type Float%20%28single-precision%29))
  ;[1 1 1] Tick - Updates animation
  (CallFunction|UpdateAnimation)
  (Math|Float|CompareFloat (.X (Math|Vector|BreakVector (Variables|/Script/Engine.MovementComponent|GetVelocity (Pawn|GetMovementComponent)))) 0.0
    (:>
      (Pawn|SetControlRotation (Pawn|GetController) (Math|Rotator|MakeRotator 0.0 0.0 0.0) :!label _label))
    (:==
      (if (Variables|Movement|GetbisMovingRight)
        (goto _label)
        (else
          (Pawn|SetControlRotation (Pawn|GetController) (Math|Rotator|MakeRotator 0.0 0.0 1.8e+02) :!label _label_2))))
    (:<
      (goto _label_2))))

(event EventBeginPlay
  (Class|ActorComponent|SetIsReplicated (Variables|Default|GetSprite) true)
  (Variables|Movement|SetState "NewEnumerator0")
  (Variables|/Script/Engine.CharacterMovementComponent|SetMaxWalkSpeed (Variables|Character|GetCharacterMovement) (Variables|Enemy|GetMoveSpeed)))

(event EventOnLanded
  (params (Hit :type Hit%20Result%20Structure%20%28by%20ref%29))
  (Variables|Movement|SetState "NewEnumerator0")
  (Variables|Movement|SetdoubleJump false))

(event Input|ActionEvents|InputActionJump
  (params (Key :type Key%20Structure))
  ;[1 1 1] Handle Jump
  (:Pressed
    (Character|Jump)
    ;[1 1 1] DoubleJump
    (if (and (and (Utilities|Enum|Equal(Enum) (Variables|Movement|GetState) "NewEnumerator2") (not (Variables|Movement|GetdoubleJump))) (not (Variables|Default|GetWithDog?)))
      (Variables|Movement|SetdoubleJump true)
      (Character|LaunchCharacter "0, 0,550.000000" false true)))
  (:Released
    (Character|StopJumping)))

(fn ConstructionScript
  (Variables|Enemy|SetPatrolDefPosition (Transformation|GetActorLocation)))

(fn ResetMovement
  (Variables|/Script/Engine.CharacterMovementComponent|SetMaxWalkSpeed (Variables|Character|GetCharacterMovement) (Variables|Enemy|GetMoveSpeed)))