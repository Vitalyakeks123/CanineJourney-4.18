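; Ball actor that presses Button actors it touches.
; Each Tick it runs a multi sphere trace against WorldDynamic objects at its own location, sized by its Sphere component and ignoring itself.
; Every hit that casts to Button gets ActivateButtonViaBall called on it, so activation repeats each frame while overlapping rather than firing on an overlap event.
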(event EventBeginPlay)

(event Collision|EventActorBeginOverlap
  (params (OtherActor :type Actor%20Object%20Reference)))

(event EventTick
  (params (DeltaSeconds :type Float%20%28single-precision%29))
  (bind _returnvalue (Transformation|GetActorLocation))
  (bind _outhits (Collision|MultiSphereTraceForObjects _returnvalue _returnvalue (Variables|/Script/Engine.SphereComponent|GetSphereRadius (Variables|Default|GetSphere)) (Utilities|Array|MakeArray "ObjectTypeQuery2") false (Utilities|Array|MakeArray self) "None"))
  (for _array_element _outhits
    (bind _asbutton (Utilities|Casting|CastToButton (.HitActor (Collision|BreakHitResult _array_element))))
    (Default|ActivateButtonViaBall _asbutton)))

(fn ConstructionScript)