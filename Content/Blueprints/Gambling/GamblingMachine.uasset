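; Slot machine that drops into the level with a bounce, shaking the camera and launching the player and dog.
; A pulsing button shows when it is playable; each activation costs a coin and runs timed sounds, flipbook and GamblingWidget spin.
; SetPrize draws from limited empty, bomb and heal pools, choosing heart or paw by player-versus-dog health.
; The sixth play forces a special result; later activations spray wrenches.
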(event OnComponentBeginOverlap(Box)
  (params (OverlappedComponent :type Primitive%20Component%20Object%20Reference) (OtherActor :type Actor%20Object%20Reference) (OtherComp :type Primitive%20Component%20Object%20Reference) (OtherBodyIndex :type Integer) (bFromSweep :type Boolean) (SweepResult :type Hit%20Result%20Structure%20%28by%20ref%29))
  ;[1 1 1] Turn On/Off machine
  (Utilities|Casting|CastToHumanCharacter OtherActor)
  (Variables|Play|SetisNear? true))

(event OnComponentEndOverlap(Box)
  (params (OverlappedComponent :type Primitive%20Component%20Object%20Reference) (OtherActor :type Actor%20Object%20Reference) (OtherComp :type Primitive%20Component%20Object%20Reference) (OtherBodyIndex :type Integer))
  ;[1 1 1] Turn On/Off machine
  (Utilities|Casting|CastToHumanCharacter OtherActor)
  (Variables|Play|SetisNear? false))

(event Custom|DropMachine
  ;[1 1 1] Drop machine
  (Variables|Drop|SetisDroping? true)
  (Variables|Drop|SetSpeed 12.0)
  (Rendering|SetActorHiddenInGame false))

(event Custom|ActivateMachine
  (bind _returnvalue (Game|GetPlayerCharacter 0))
  (bind _ashuman_character (Utilities|Casting|CastToHumanCharacter _returnvalue))
  (bind _coinscount (Variables|/Game/Blueprints/Characters/HumanCharacter.HumanCharacter_C|GetCoinsCount _ashuman_character))
  ;[1 1 1] Activate machine
  (if (< (Variables|Play|GetPlayCount) 6)
    (if (and (not (Variables|Play|GetisPlaying?)) (> _coinscount 0))
      (bind _result (Math|Integer|DecrementInt _coinscount)
        (:%20%20
          (Math|Integer|DecrementInt (Variables|/Game/Blueprints/Characters/HumanCharacter.HumanCharacter_C|GetAllCoins _ashuman_character)
            (:%20%20
              (Default|CoinChange (Variables|/Game/Blueprints/Characters/HumanCharacter.HumanCharacter_C|GetHealthWidget _ashuman_character) _result)
              (Variables|Play|SetisPlaying? true)
              (Audio|SpawnSound2D "/Game/Sounds/slot_machine_coins.slot_machine_coins")
              (Utilities|Time|SetTimerbyFunctionName 0 "PullTheTrigger" 2.0)
              (bind _returnvalue_2 (UserInterface|CreateWidget "/Game/UI/GamblingWidget.GamblingWidget_C"))
              (bind _output_get (Variables|Default|SetGamblingWidget _returnvalue_2))
              (UserInterface|Viewport|AddtoViewport _output_get 0))))))
    (elif (and (not (Variables|Play|GetisWrenches?)) (not (Variables|Play|GetisPlaying?)))
      (Variables|Play|SetisWrenches? true)
      (Utilities|Time|SetTimerbyFunctionName 0 "StopWrenches" 2.0)
      (Utilities|Time|SetTimerbyFunctionName 0 "SpawnWrenches" 0.1 true))))

(event EventBeginPlay)

(event Collision|EventActorBeginOverlap
  (params (OtherActor :type Actor%20Object%20Reference)))

(event EventTick
  (params (DeltaSeconds :type Float%20%28single-precision%29))
  (CallFunction|AddSpeed DeltaSeconds)
  (CallFunction|Drop)
  (CallFunction|ChangeButtonSize DeltaSeconds))

(fn ConstructionScript
  (Variables|Gambling|SetStartPosition (Transformation|GetActorLocation)))

(fn AddSpeed
  (params (DeltaTime :type Float%20%28single-precision%29))
  (if (Variables|Drop|GetisDroping?)
    (Variables|Drop|SetSpeed (+ (Variables|Drop|GetSpeed) (* (Variables|Drop|GetDropSpeedBonus) DeltaTime)))))

(fn Drop
  (bind _returnvalue (Transformation|GetActorLocation))
  (if (Variables|Drop|GetisDroping?)
    (Transformation|Teleport (Math|Vector|MakeVector (.x _returnvalue) (.y _returnvalue) (- (.z _returnvalue) (Variables|Drop|GetSpeed))) "0, 0, 0")
    (if (and (<= (.z (Transformation|GetActorLocation)) (.z (Variables|Gambling|GetDropPosition))) (>= (Variables|Drop|GetSpeed) 0.0))
      (Variables|Drop|SetisDroping? false)
      (if (not (Variables|Drop|GetisSecondDrop?))
        (Variables|Drop|SetisSecondDrop? true)
        (Variables|Drop|SetSpeed -6.0)
        (Variables|Drop|SetisDroping? true)
        (Class|PlayerController|ClientPlayCameraShake (Game|GetPlayerController 0) "/Game/Blueprints/Gambling/GamblingCameraShake.GamblingCameraShake_C" 1.0 "CameraLocal" "0, 0, 0")
        (CallFunction|JumpAfterDrop 4.5e+02)
        (else
          (Class|PlayerController|ClientPlayCameraShake (Game|GetPlayerController 0) "/Game/Blueprints/Gambling/GamblingCameraAfterShake.GamblingCameraAfterShake_C" 1.0 "CameraLocal" "0, 0, 0")
          (CallFunction|JumpAfterDrop 1.5e+02)
          (Variables|Play|SetisReady? true))))))

(fn JumpAfterDrop
  (params (JumpForce :type Float%20%28single-precision%29))
  (bind _returnvalue (Game|GetPlayerCharacter 0))
  (bind _ashuman_character (Utilities|Casting|CastToHumanCharacter _returnvalue))
  (bind _dogreference (Variables|/Game/Blueprints/Characters/HumanCharacter.HumanCharacter_C|GetDogReference _ashuman_character))
  (if (AI|Components|NavMovement|IsFalling (Variables|/Script/Engine.Character|GetCharacterMovement _returnvalue))
    _
    (else
      (Character|LaunchCharacter _returnvalue (Math|Vector|MakeVector 0.0 0.0 JumpForce) false true)))
  (if (not (AI|Components|NavMovement|IsFalling (Variables|/Script/Engine.Character|GetCharacterMovement _dogreference)))
    (Character|LaunchCharacter _dogreference (Math|Vector|MakeVector 0.0 0.0 JumpForce) false true)))

(fn ChangeButtonSize
  (params (DeltaTime :type Float%20%28single-precision%29))
  (bind _returnvalue (* DeltaTime 0.7))
  (bind _r_button (Variables|Default|GetR-button))
  (bind _r_button_2 (Variables|Default|GetR-button))
  (bind _returnvalue_2 (Transformation|GetWorldScale _r_button))
  (if (Math|Boolean|ANDBoolean (Variables|Play|GetisReady?) (Variables|Play|GetisNear?) (not (Variables|Play|GetisPlaying?)) (< (Variables|Play|GetPlayCount) 6))
    (Rendering|SetVisibility _r_button_2 true false)
    (else
      (Rendering|SetVisibility _r_button_2 false false)))
  (if (Variables|Button|GetsetButtonBigger)
    (Transformation|SetWorldScale3D _r_button (Math|Vector|MakeVector (+ (.x _returnvalue_2) _returnvalue) (.y _returnvalue_2) (+ (.z _returnvalue_2) _returnvalue)))
    (if (>= (.x _returnvalue_2) 2.0)
      (Variables|Button|SetsetButtonBigger false))
    (else
      (Transformation|SetWorldScale3D _r_button (Math|Vector|MakeVector (- (.x _returnvalue_2) _returnvalue) (.y _returnvalue_2) (- (.z _returnvalue_2) _returnvalue)))
      (if (<= (.x _returnvalue_2) 1.5)
        (Variables|Button|SetsetButtonBigger true)))))

(fn PulltheTrigger
  (bind _paperflipbook (Variables|Default|GetPaperFlipbook))
  (Audio|PlaySound2D "/Game/Sounds/slot_machine_puller.slot_machine_puller")
  (Utilities|Time|SetTimerbyFunctionName 0 "DrumsActions" 3.0)
  (Sprite|SetFlipbook _paperflipbook "/Game/Sprites/Gambling/gambling-machine_activate.gambling-machine_activate")
  (Utilities|Time|SetTimerbyFunctionName 0 "ChangeAnimation" (- (Class|PaperFlipbookComponent|GetFlipbookLength _paperflipbook) 0.05))
  (CallFunction|SetPrize)
  (Default|SpinDrums (Variables|Default|GetGamblingWidget) (Variables|Play|GetPrizeType)))

(fn DrumsActions
  (Audio|PlaySound2D "/Game/Sounds/slot_machine_drums.slot_machine_drums"))

(fn ChangeAnimation
  (Sprite|SetFlipbook (Variables|Default|GetPaperFlipbook) "/Game/Sprites/Gambling/gambling-machine.gambling-machine")
  (Variables|Play|SetisPlaying? false)
  (Widget|RemovefromParent (Variables|Default|GetGamblingWidget))
  (switch int (Variables|Play|GetPrizeType)
    (:1
      (CallFunction|CreateHeart))
    (:2
      (CallFunction|CreatePaw))
    (:3
      (CallFunction|CreateBomb))))

(fn SetPrize
  (bind _result (Math|Integer|IncrementInt (Variables|Play|GetPlayCount))
    (:%20%20
      (if (== _result 6)
        (Variables|Play|SetPrizeType 4)
        (else
          (Variables|Play|SetisValidDrop false)
          (while (not (Variables|Play|GetisValidDrop))
            (switch int (Math|Random|RandomIntegerinRange 0 2)
              (:0
                (if (> (Variables|Play|GetEmptyDrops) 0)
                  (Variables|Play|SetisValidDrop true)
                  (Math|Integer|DecrementInt (Variables|Play|GetEmptyDrops)
                    (:%20%20
                      (Variables|Play|SetPrizeType 5)))))
              (:1
                (if (> (Variables|Play|GetBombDrop) 0)
                  (Variables|Play|SetisValidDrop true)
                  (Math|Integer|DecrementInt (Variables|Play|GetBombDrop)
                    (:%20%20
                      (Variables|Play|SetPrizeType 3)))))
              (:2
                (if (> (Variables|Play|GetHealDrops) 0)
                  (bind _ashuman_character (Utilities|Casting|CastToHumanCharacter (Game|GetPlayerCharacter 0)))
                  (if (< (Variables|/Game/Blueprints/Characters/HumanCharacter.HumanCharacter_C|GetHealth _ashuman_character) (Variables|/Game/Blueprints/Characters/DogCharacter.DogCharacter_C|GetHealth (Variables|/Game/Blueprints/Characters/HumanCharacter.HumanCharacter_C|GetDogReference _ashuman_character)))
                    (Variables|Play|SetPrizeType 1 :!label _label)
                    (else
                      (if (> (Variables|/Game/Blueprints/Characters/HumanCharacter.HumanCharacter_C|GetHealth _ashuman_character) (Variables|/Game/Blueprints/Characters/DogCharacter.DogCharacter_C|GetHealth (Variables|/Game/Blueprints/Characters/HumanCharacter.HumanCharacter_C|GetDogReference _ashuman_character)))
                        _
                        (elif (== (Math|Random|RandomIntegerinRange 0 1) 0)
                          (goto _label)
                          (else
                            _)))
                      (Variables|Play|SetPrizeType 2)))
                  (Math|Integer|DecrementInt (Variables|Play|GetHealDrops)
                    (:%20%20
                      (Variables|Play|SetisValidDrop true))))))))))))

(fn CreateBomb
  (bind _returnvalue (Transformation|GetActorLocation))
  (bind _returnvalue_2 (Game|SpawnActorfromClass "/Game/Blueprints/Gambling/GamblingBomb.GamblingBomb_C" (Math|Transform|MakeTransform (Math|Vector|MakeVector (.x _returnvalue) 1e+01 (+ (.z _returnvalue) 3e+01)) "0, 0, 0" "1.000000,1,1.000000") "AlwaysSpawn" 0 0))
  (if (> (.x (Transformation|GetActorLocation (Game|GetPlayerCharacter 0))) (.x (Transformation|GetActorLocation _returnvalue_2)))
    (Physics|AddImpulse (Variables|/Game/Blueprints/Gambling/GamblingBomb.GamblingBomb_C|GetBox _returnvalue_2) "75.000000, 0,275.000000" "None" true)
    (else
      (Physics|AddImpulse (Variables|/Game/Blueprints/Gambling/GamblingBomb.GamblingBomb_C|GetBox _returnvalue_2) "-75.000000, 0,275.000000" "None" true))))

(fn CreateHeart
  (bind _returnvalue (Transformation|GetActorLocation))
  (bind _returnvalue_2 (Game|SpawnActorfromClass "/Game/Blueprints/Pickables/Heart_Drop.Heart_Drop_C" (Math|Transform|MakeTransform (Math|Vector|MakeVector (.x _returnvalue) 5.0 (+ (.z _returnvalue) 3e+01)) "0, 0, 0" "1.000000,1,1.000000") "AlwaysSpawn" 0 0))
  (if (== (Math|Random|RandomIntegerinRange 0 1) 0)
    (Physics|AddImpulse (Variables|/Game/Blueprints/Pickables/PickableBase.PickableBase_C|GetSphere _returnvalue_2) "75.000000, 0,275.000000" "None" true)
    (else
      (Physics|AddImpulse (Variables|/Game/Blueprints/Pickables/PickableBase.PickableBase_C|GetSphere _returnvalue_2) "-75.000000, 0,275.000000" "None" true))))

(fn CreatePaw
  (bind _returnvalue (Transformation|GetActorLocation))
  (bind _returnvalue_2 (Game|SpawnActorfromClass "/Game/Blueprints/Pickables/Paw_Drop.Paw_Drop_C" (Math|Transform|MakeTransform (Math|Vector|MakeVector (.x _returnvalue) 5.0 (+ (.z _returnvalue) 3e+01)) "0, 0, 0" "1.000000,1,1.000000") "AlwaysSpawn" 0 0))
  (if (== (Math|Random|RandomIntegerinRange 0 1) 0)
    (Physics|AddImpulse (Variables|/Game/Blueprints/Pickables/PickableBase.PickableBase_C|GetSphere _returnvalue_2) "75.000000, 0,275.000000" "None" true)
    (else
      (Physics|AddImpulse (Variables|/Game/Blueprints/Pickables/PickableBase.PickableBase_C|GetSphere _returnvalue_2) "-75.000000, 0,275.000000" "None" true))))

(fn SpawnWrenches
  (bind _returnvalue (Transformation|GetActorLocation))
  (bind _returnvalue_2 (Game|SpawnActorfromClass "/Game/Blueprints/Gambling/GamblingWrench.GamblingWrench_C" (Math|Transform|MakeTransform (Math|Vector|MakeVector (.x _returnvalue) 5.0 (+ (.z _returnvalue) 3e+01)) (Math|Rotator|MakeRotator 0.0 (Math|Random|RandomFloatinRange -5e+01 5e+01) 0.0) "1.000000,1,1.000000") "AlwaysSpawn" 0 0))
  (if (== (Math|Random|RandomIntegerinRange 0 1) 0)
    (Physics|AddImpulse (Variables|/Game/Blueprints/Gambling/GamblingWrench.GamblingWrench_C|GetBox _returnvalue_2) (Math|Vector|MakeVector (Math|Random|RandomFloatinRange 4e+01 75.0) 0.0 (Math|Random|RandomFloatinRange 175.0 325.0)) "None" true)
    (else
      (Physics|AddImpulse (Variables|/Game/Blueprints/Gambling/GamblingWrench.GamblingWrench_C|GetBox _returnvalue_2) (Math|Vector|MakeVector (Math|Random|RandomFloatinRange -4e+01 -75.0) 0.0 (Math|Random|RandomFloatinRange 175.0 325.0)) "None" true))))

(fn StopWrenches
  (Variables|Play|SetisWrenches? false)
  (Utilities|Time|ClearTimerbyFunctionName 0 "SpawnWrenches"))