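; Timed gambling bomb that blinks until its lifetime expires, then explodes and damages nearby human characters.
; SetVisible and SetInvisible call each other through timers, toggling the flipbook sprite's alpha to create the blink.
; On destruction it spawns a GamblingBombExplosion and uses a pawn sphere trace to apply damage to each HumanCharacter hit.
; The box overlap only casts to HumanCharacter and triggers nothing.
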(event OnComponentBeginOverlap(Box)
  (params (OverlappedComponent :type Primitive%20Component%20Object%20Reference) (OtherActor :type Actor%20Object%20Reference) (OtherComp :type Primitive%20Component%20Object%20Reference) (OtherBodyIndex :type Integer) (bFromSweep :type Boolean) (SweepResult :type Hit%20Result%20Structure%20%28by%20ref%29))
  (Utilities|Casting|CastToHumanCharacter OtherActor))

(event EventBeginPlay
  (Utilities|Time|SetTimerbyFunctionName 0 "SetInvisible" 0.3)
  (Actor|SetLifeSpan (Variables|Default|GetLifeTime)))

(event Collision|EventActorBeginOverlap
  (params (OtherActor :type Actor%20Object%20Reference)))

(event EventTick
  (params (DeltaSeconds :type Float%20%28single-precision%29)))

(event EventDestroyed
  (bind _returnvalue (Transformation|GetActorLocation))
  (Game|SpawnActorfromClass "/Game/Blueprints/Gambling/GamblingBombExplosion.GamblingBombExplosion_C" (Math|Transform|MakeTransform (.location (Transformation|GetActorTransform)) "0, 0, 0" "2.500000,1,2.500000") "AlwaysSpawn" 0 0)
  (bind _outhits (Collision|MultiSphereTraceForObjects _returnvalue _returnvalue 7e+01 (Utilities|Array|MakeArray "ObjectTypeQuery3") false (Utilities|Array|MakeArray 0) "None"))
  (for _array_element _outhits
    (bind _ashuman_character (Utilities|Casting|CastToHumanCharacter (.HitActor (Collision|BreakHitResult _array_element))))
    (Game|Damage|ApplyDamage _ashuman_character 1.0 0 self)))

(fn ConstructionScript)

(fn SetVisible
  (Sprite|SetSpriteColor (Variables|Default|GetPaperFlipbook) "(R=1.000000,G=1.000000,B=1.000000,A=1.000000)")
  (Utilities|Time|SetTimerbyFunctionName 0 "SetInvisible" 0.3))

(fn SetInvisible
  (Sprite|SetSpriteColor (Variables|Default|GetPaperFlipbook) "(R=1.000000,G=1.000000,B=1.000000,A=0.000000)")
  (Utilities|Time|SetTimerbyFunctionName 0 "SetVisible" 0.2))