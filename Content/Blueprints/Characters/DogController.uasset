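; AI controller for a dog that follows the player or goes after a ball on command.
; ChangeFollow, Fetch and StopAllCommands set two state flags; Tick then re-issues moves toward the player or the first Ball found, searching every frame when not following the player.
; Moves change only the X coordinate and skip pathfinding, as in side-scrolling movement.
; Stopping moves the dog to its own location; reaching the ball triggers nothing yet.
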(event Custom|ChangeFollow
  (bind _returnvalue (Pawn|GetControlledPawn))
  (bind _returnvalue_2 (Transformation|GetActorLocation _returnvalue))
  (Variables|Default|SetFollowActor? false)
  (if (Variables|Default|GetCommandToMe)
    (Variables|Default|SetCommandToMe false)
    (AI|Navigation|MovetoLocation (Math|Vector|MakeVector (.x _returnvalue_2) (.y _returnvalue_2) (.z _returnvalue_2)) 2.0 true false false)
    (else
      (Variables|Default|SetCommandToMe true))))

(event Custom|Fetch
  (bind _returnvalue (Pawn|GetControlledPawn))
  (bind _returnvalue_2 (Transformation|GetActorLocation _returnvalue))
  (bind _outactors (Actor|GetAllActorsOfClass "/Game/Blueprints/Ball/Ball.Ball_C"))
  (if (> (Utilities|Array|Length _outactors) 0)
    (Variables|Default|SetCommandToMe false)
    (Variables|Default|SetFollowActor? true)
    (AI|Navigation|MovetoLocation (Math|Vector|MakeVector (.x (Transformation|GetActorLocation (Utilities|Array|Get(acopy) _outactors))) (.y _returnvalue_2) (.z _returnvalue_2)) 0.0 true false false)))

(event Custom|StopAllCommands
  (bind _returnvalue (Pawn|GetControlledPawn))
  (bind _returnvalue_2 (Transformation|GetActorLocation _returnvalue))
  (Variables|Default|SetFollowActor? false)
  (Variables|Default|SetCommandToMe false)
  (AI|Navigation|MovetoLocation (Math|Vector|MakeVector (.x _returnvalue_2) (.y _returnvalue_2) (.z _returnvalue_2)) 2.0 true false false))

(event EventBeginPlay)

(event EventTick
  (params (DeltaSeconds :type Float%20%28single-precision%29))
  (if (Variables|Default|GetCommandToMe)
    (CallFunction|FollowPlayer)
    (else
      (bind _outactors (Actor|GetAllActorsOfClass "/Game/Blueprints/Ball/Ball.Ball_C"))
      (CallFunction|FollowActor (Utilities|Array|Get(acopy) _outactors)))))

(fn ConstructionScript)

(fn FollowPlayer
  (bind _returnvalue (Pawn|GetControlledPawn))
  (bind _returnvalue_2 (Transformation|GetActorLocation _returnvalue))
  (AI|Navigation|MovetoLocation (Math|Vector|MakeVector (.x (Transformation|GetActorLocation (Game|GetPlayerCharacter 0))) (.y _returnvalue_2) (.z _returnvalue_2)) 2.0 true false false))

(fn FollowActor
  (params (Followed :type Actor%20Object%20Reference))
  (bind _returnvalue (Transformation|GetActorLocation Followed))
  (bind _returnvalue_2 (Pawn|GetControlledPawn))
  (bind _returnvalue_3 (Transformation|GetActorLocation _returnvalue_2))
  (if (Variables|Default|GetFollowActor?)
    (Utilities|IsValid Followed
      (:Is%20Valid
        (AI|Navigation|MovetoLocation (Math|Vector|MakeVector (.x _returnvalue) (.y _returnvalue_3) (.z _returnvalue_3)) 1.0 true false false)
        (if (<= (Math|Float|Absolute(Float) (- (.x _returnvalue) (.x _returnvalue_3))) 2.0)
          _)))))