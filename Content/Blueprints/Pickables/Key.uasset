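; Key pickup Blueprint that opens its referenced Gate when a HumanCharacter touches it.
; Sphere overlap calls Open on the Gate if it is valid, then destroys the key either way, and the Destroyed event plays a 2D sound.
; When the Box hits a WorldStatic component, it stops physics simulation on the Sphere, zeroes the actor rotation and prints a debug "Hello".
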(event OnComponentBeginOverlap(Sphere)
  (params (OverlappedComponent :type Primitive%20Component%20Object%20Reference) (OtherActor :type Actor%20Object%20Reference) (OtherComp :type Primitive%20Component%20Object%20Reference) (OtherBodyIndex :type Integer) (bFromSweep :type Boolean) (SweepResult :type Hit%20Result%20Structure%20%28by%20ref%29))
  (bind _gate (Variables|Default|GetGate))
  (Utilities|Casting|CastToHumanCharacter OtherActor)
  (Utilities|IsValid _gate
    (:Is%20Valid
      (Default|Open _gate))
    (:Is%20Not%20Valid
      _))
  (Actor|DestroyActor))

(event OnComponentHit(Box)
  (params (HitComponent :type Primitive%20Component%20Object%20Reference) (OtherActor :type Actor%20Object%20Reference) (OtherComp :type Primitive%20Component%20Object%20Reference) (NormalImpulse :type Vector :default "0, 0, 0") (Hit :type Hit%20Result%20Structure%20%28by%20ref%29))
  (if (Utilities|Enum|Equal(Enum) (Collision|GetCollisionObjectType OtherComp) "ECC_WorldStatic")
    (Physics|SetSimulatePhysics (Variables|Default|GetSphere) false)
    (Transformation|SetActorRotation "0, 0, 0")
    (Development|PrintString "Hello")))

(event EventBeginPlay)

(event Collision|EventActorBeginOverlap
  (params (OtherActor :type Actor%20Object%20Reference)))

(event EventTick
  (params (DeltaSeconds :type Float%20%28single-precision%29)))

(event EventDestroyed
  (Audio|PlaySound2D "/Game/StarterContent/Audio/zvuki_dlya_igri/hilka_pes3.hilka_pes3"))

(fn ConstructionScript
  (|CallParentFunction))