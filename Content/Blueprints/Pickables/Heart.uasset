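; Heart is a health pickup that heals a HumanCharacter who touches it.
; When its Sphere overlaps a HumanCharacter below max health, it adds Heal to Health, clamped to MaxHealth, and updates that character's HealthWidget.
; It then destroys itself and plays the Hilka 2D sound, so it stays in place if the character is already at full health.
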(event OnComponentBeginOverlap(Sphere)
  (params (OverlappedComponent :type Primitive%20Component%20Object%20Reference) (OtherActor :type Actor%20Object%20Reference) (OtherComp :type Primitive%20Component%20Object%20Reference) (OtherBodyIndex :type Integer) (bFromSweep :type Boolean) (SweepResult :type Hit%20Result%20Structure%20%28by%20ref%29))
  (bind _ashuman_character (Utilities|Casting|CastToHumanCharacter OtherActor))
  (if (< (Variables|/Game/Blueprints/Characters/HumanCharacter.HumanCharacter_C|GetHealth _ashuman_character) (Variables|/Game/Blueprints/Characters/HumanCharacter.HumanCharacter_C|GetMaxHealth _ashuman_character))
    (bind _output_get (Variables|/Game/Blueprints/Characters/HumanCharacter.HumanCharacter_C|SetHealth _ashuman_character (Math|Float|Clamp(Float) (+ (Variables|/Game/Blueprints/Characters/HumanCharacter.HumanCharacter_C|GetHealth _ashuman_character) (Variables|Default|GetHeal)) 0.0 (Variables|/Game/Blueprints/Characters/HumanCharacter.HumanCharacter_C|GetMaxHealth _ashuman_character))))
    (Default|ChangeHumanHealth (Variables|/Game/Blueprints/Characters/HumanCharacter.HumanCharacter_C|GetHealthWidget _ashuman_character) _output_get)
    (Actor|DestroyActor)
    (Audio|PlaySound2D "/Game/StarterContent/Audio/zvuki_dlya_igri/hilka.hilka")))

(event EventBeginPlay)

(event Collision|EventActorBeginOverlap
  (params (OtherActor :type Actor%20Object%20Reference)))

(event EventTick
  (params (DeltaSeconds :type Float%20%28single-precision%29)))

(fn ConstructionScript
  (|CallParentFunction))