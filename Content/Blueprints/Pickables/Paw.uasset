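; Paw is a pickup that restores one point of the dog's health, up to a cap of three.
; On sphere overlap by the human or the dog, it raises the dog's health, reached through the human's dog reference or directly.
; It then updates the health widget on the human character, destroys itself and plays a 2D sound.
; At full dog health the pickup stays in place.
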(event OnComponentBeginOverlap(Sphere)
  (params (OverlappedComponent :type Primitive%20Component%20Object%20Reference) (OtherActor :type Actor%20Object%20Reference) (OtherComp :type Primitive%20Component%20Object%20Reference) (OtherBodyIndex :type Integer) (bFromSweep :type Boolean) (SweepResult :type Hit%20Result%20Structure%20%28by%20ref%29))
  (bind _ashuman_character (Utilities|Casting|CastToHumanCharacter OtherActor)
    (:then
      (if (< (Variables|/Game/Blueprints/Characters/DogCharacter.DogCharacter_C|GetHealth (Variables|/Game/Blueprints/Characters/HumanCharacter.HumanCharacter_C|GetDogReference _ashuman_character)) 3.0)
        (bind _result (Math|Float|IncrementFloat (Variables|/Game/Blueprints/Characters/DogCharacter.DogCharacter_C|GetHealth (Variables|/Game/Blueprints/Characters/HumanCharacter.HumanCharacter_C|GetDogReference _ashuman_character)))
          (:%20%20
            (Default|ChangeDogHealth (Variables|/Game/Blueprints/Characters/HumanCharacter.HumanCharacter_C|GetHealthWidget _ashuman_character) _result)
            (Actor|DestroyActor)
            (Audio|PlaySound2D "/Game/StarterContent/Audio/zvuki_dlya_igri/hilka_pes3.hilka_pes3")))))
    (:CastFailed
      (bind _asdog_character (Utilities|Casting|CastToDogCharacter OtherActor))
      (if (< (Variables|/Game/Blueprints/Characters/DogCharacter.DogCharacter_C|GetHealth _asdog_character) 3.0)
        (bind _ashuman_character_2 (Utilities|Casting|CastToHumanCharacter (Game|GetPlayerCharacter 0)))
        (bind _result_2 (Math|Float|IncrementFloat (Variables|/Game/Blueprints/Characters/DogCharacter.DogCharacter_C|GetHealth _asdog_character))
          (:%20%20
            (Default|ChangeDogHealth (Variables|/Game/Blueprints/Characters/HumanCharacter.HumanCharacter_C|GetHealthWidget _ashuman_character_2) _result_2)
            (Actor|DestroyActor)
            (Audio|PlaySound2D "/Game/StarterContent/Audio/zvuki_dlya_igri/hilka_pes3.hilka_pes3")))))))

(event EventBeginPlay)

(event Collision|EventActorBeginOverlap
  (params (OtherActor :type Actor%20Object%20Reference)))

(event EventTick
  (params (DeltaSeconds :type Float%20%28single-precision%29)))

(fn ConstructionScript
  (|CallParentFunction))