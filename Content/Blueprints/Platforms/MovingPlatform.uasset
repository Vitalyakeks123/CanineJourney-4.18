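; Moving platform actor that travels back and forth along a list of Points, pausing for StopTime at each one.
; The construction script applies the cube's material and stores the actor's location as the first point.
; With at least two points, Tick counts down the pause, then teleports at constant speed in the X/Z plane toward Destination.
; On arrival within a small tolerance, SetNextPoint steps the index, recursively reversing direction at either end.
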(event EventBeginPlay
  (bind _points (Variables|Platform|GetPoints))
  (Variables|Default|SetCurrentStopTime (Variables|Platform|GetStopTime))
  (Variables|Default|SetPointsNumber (Utilities|Array|Length _points))
  (Variables|Default|SetDestination (Utilities|Array|Get(acopy) _points)))

(event Collision|EventActorBeginOverlap
  (params (OtherActor :type Actor%20Object%20Reference)))

(event EventTick
  (params (DeltaSeconds :type Float%20%28single-precision%29))
  (if (>= (Variables|Default|GetPointsNumber) 2)
    (bind _ismoving_ (CallFunction|ChangeStopTime DeltaSeconds))
    (if _ismoving_
      (CallFunction|MovePlatform DeltaSeconds))))

(fn ConstructionScript
  (Rendering|Material|SetMaterial (Variables|Default|GetCube) 0 (Variables|Platform|GetMaterial))
  (bind _output_get (Variables|Platform|SetStartPosition (Transformation|GetActorLocation)))
  (Utilities|Array|SetArrayElem (Variables|Platform|GetPoints) 0 _output_get true))

(fn MovePlatform
  (params (DeltaTime :type Float%20%28single-precision%29))
  (bind _returnvalue (Transformation|GetActorLocation))
  (bind _returnvalue_2 (Transformation|GetActorLocation))
  (bind _destination (Variables|Default|GetDestination))
  (bind _movespeed (Variables|Platform|GetMoveSpeed))
  (bind _destination_2 (Variables|Default|GetDestination))
  (bind _returnvalue_3 (Class|KismetMathLibrary|Vector2DInterptoConstant (Math|Vector2D|MakeVector2D (.x _returnvalue) (.z _returnvalue)) (Math|Vector2D|MakeVector2D (.x _destination) (.z _destination)) DeltaTime _movespeed))
  (Transformation|SetActorLocation (Math|Vector|MakeVector (.x _returnvalue_3) 0.0 (.y _returnvalue_3)) false true)
  (if (and (<= (Math|Float|Absolute(Float) (- (.x _returnvalue_2) (.x _destination_2))) 2.0) (<= (Math|Float|Absolute(Float) (- (.z _returnvalue_2) (.z _destination_2))) 2.0))
    (Variables|Default|SetCurrentStopTime (Variables|Platform|GetStopTime))
    (CallFunction|SetNextPoint)))

(fn ChangeStopTime
  (params (DeltaTime :type Float%20%28single-precision%29))
  (bind _output_get (Variables|Default|SetCurrentStopTime (Math|Float|Clamp(Float) (- (Variables|Default|GetCurrentStopTime) DeltaTime) 0.0 123123.0)))
  (if (<= _output_get 0.0)
    (return true)
    (else
      (return false))))

(fn SetNextPoint
  (if (Variables|Default|GetisMovingBack?)
    (bind _result (Math|Integer|DecrementInt (Variables|Default|GetCurrentIndex))
      (:%20%20
        (if (== _result -1)
          (Math|Integer|IncrementInt (Variables|Default|GetCurrentIndex)
            (:%20%20
              (Variables|Default|SetisMovingBack? false)
              (CallFunction|SetNextPoint)))
          (else
            (Variables|Default|SetDestination (Utilities|Array|Get(acopy) (Variables|Platform|GetPoints) (Variables|Default|GetCurrentIndex)))))))
    (else
      (bind _result_2 (Math|Integer|IncrementInt (Variables|Default|GetCurrentIndex))
        (:%20%20
          (if (== _result_2 (Variables|Default|GetPointsNumber))
            (Math|Integer|DecrementInt (Variables|Default|GetCurrentIndex)
              (:%20%20
                (Variables|Default|SetisMovingBack? true)
                (CallFunction|SetNextPoint)))
            (else
              (Variables|Default|SetDestination (Utilities|Array|Get(acopy) (Variables|Platform|GetPoints) (Variables|Default|GetCurrentIndex))))))))))