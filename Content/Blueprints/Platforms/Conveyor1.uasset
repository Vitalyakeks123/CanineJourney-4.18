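; Conveyor belt platform that carries human and dog characters along the world X axis while it is switched on.
; Each Tick it checks actors overlapping its Box and teleports those characters by Force, with IsLeft choosing the direction.
; The per-frame step is not scaled by delta time, so belt speed depends on frame rate.
; The construction script applies the Material variable to the Cube mesh.
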(event EventBeginPlay)

(event Collision|EventActorBeginOverlap
  (params (OtherActor :type Actor%20Object%20Reference))
  (if (Variables|Conveyor|GetIsOn?)
    _))

(event EventTick
  (params (DeltaSeconds :type Float%20%28single-precision%29))
  (if (Variables|Conveyor|GetIsOn?)
    (for _array_element (Collision|GetOverlappingActors (Variables|Default|GetBox) 0 :!class /Script/Engine.PrimitiveComponent)
      (bind _ashuman_character (Utilities|Casting|CastToHumanCharacter _array_element)
        (:then
          (CallFunction|MoveCharacter _ashuman_character))
        (:CastFailed
          (bind _asdog_character (Utilities|Casting|CastToDogCharacter _array_element))
          (CallFunction|MoveCharacter _asdog_character))))))

(fn ConstructionScript
  (Rendering|Material|SetMaterial (Variables|Default|GetCube) 0 (Variables|Conveyor|GetMaterial)))

(fn MoveCharacter
  (params (Character :type Character%20Object%20Reference))
  (bind _returnvalue (Transformation|GetActorRotation Character))
  (if (Variables|Conveyor|GetIsLeft?)
    (Transformation|Teleport Character (+ (* "-1.000000, 0, 0" (Variables|Conveyor|GetForce)) (Transformation|GetActorLocation Character)) _returnvalue)
    (else
      (Transformation|Teleport Character (+ (* "1.000000, 0, 0" (Variables|Conveyor|GetForce)) (Transformation|GetActorLocation Character)) _returnvalue))))