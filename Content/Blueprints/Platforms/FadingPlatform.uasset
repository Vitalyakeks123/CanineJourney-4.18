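; Fading platform that disappears a set time after a human or dog character overlaps it, then reappears.
; An overlap while online starts a SetOffline timer, unless one is already running.
; SetOffline hides the cube, disables its collision and schedules SetOnline, which shows it again with query-only collision.
; The construction script applies the configurable material to the cube.
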(event EventBeginPlay)

(event Collision|EventActorBeginOverlap
  (params (OtherActor :type Actor%20Object%20Reference))
  (Utilities|Casting|CastToHumanCharacter OtherActor
    (:then
      _)
    (:CastFailed
      (Utilities|Casting|CastToDogCharacter OtherActor)))
  (if (Variables|Default|GetisOnline)
    (if (not (Class|KismetSystemLibrary|IsTimerActive 0 "SetOffline"))
      (Utilities|Time|SetTimerbyFunctionName 0 "SetOffline" (Variables|Platform|GetOnlineTime)))))

(event EventTick
  (params (DeltaSeconds :type Float%20%28single-precision%29)))

(fn ConstructionScript
  (Rendering|Material|SetMaterial (Variables|Default|GetCube) 0 (Variables|Platform|GetMaterial)))

(fn SetOnline
  (Development|SetHiddeninGame (Variables|Default|GetCube) false false)
  (Collision|SetCollisionEnabled (Variables|Default|GetCube) "QueryOnly")
  (Variables|Default|SetisOnline true))

(fn SetOffline
  (Development|SetHiddeninGame (Variables|Default|GetCube) true false)
  (Utilities|Time|SetTimerbyFunctionName 0 "SetOnline" (Variables|Platform|GetOfflineTime))
  (Collision|SetCollisionEnabled (Variables|Default|GetCube) "NoCollision")
  (Variables|Default|SetisOnline false))