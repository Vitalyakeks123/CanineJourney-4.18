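; Platform actor that moves to a set position while the player character or its dog overlaps it, and returns to its start otherwise.
; Each tick, CheckOverlap picks the destination and MovePlatform teleports the actor toward it using constant-speed 2D interpolation on the X-Z plane.
; The construction script applies the cube's material and records the start position.
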(event EventBeginPlay)

(event Collision|EventActorBeginOverlap
  (params (OtherActor :type Actor%20Object%20Reference)))

(event EventTick
  (params (DeltaSeconds :type Float%20%28single-precision%29))
  (CallFunction|CheckOverlap)
  (CallFunction|MovePlatform DeltaSeconds))

(fn ConstructionScript
  (Rendering|Material|SetMaterial (Variables|Default|GetCube) 0 (Variables|Platform|GetMaterial))
  (Variables|Platform|SetStartPosition (Transformation|GetActorLocation)))

(fn MovePlatform
  (params (DeltaTime :type Float%20%28single-precision%29))
  (bind _returnvalue (Transformation|GetActorLocation))
  (bind _destination (Variables|Default|GetDestination))
  (bind _movespeed (Variables|Platform|GetMoveSpeed))
  (bind _returnvalue_2 (Class|KismetMathLibrary|Vector2DInterptoConstant (Math|Vector2D|MakeVector2D (.x _returnvalue) (.z _returnvalue)) (Math|Vector2D|MakeVector2D (.x _destination) (.z _destination)) DeltaTime _movespeed))
  (Transformation|SetActorLocation (Math|Vector|MakeVector (.x _returnvalue_2) 0.0 (.y _returnvalue_2)) false true))

(fn CheckOverlap
  (bind _returnvalue (Game|GetPlayerCharacter 0))
  (if (or (Collision|IsOverlappingActor _returnvalue :!class /Script/Engine.Actor) (Collision|IsOverlappingActor (Variables|/Game/Blueprints/Characters/HumanCharacter.HumanCharacter_C|GetDogReference (.AsHuman%20Character (Utilities|Casting|CastToHumanCharacter _returnvalue))) :!class /Script/Engine.Actor))
    (Variables|Default|SetDestination (Variables|Platform|GetMovePosition))
    (else
      (Variables|Default|SetDestination (Variables|Platform|GetStartPosition)))))