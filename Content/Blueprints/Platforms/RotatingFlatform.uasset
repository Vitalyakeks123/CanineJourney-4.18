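; Platform actor that flips in 90-degree pitch steps, either on a repeating timer or when a character leaves it.
; With IsAlways set, it turns each time the Interval countdown expires; otherwise, a HumanCharacter or un-picked DogCharacter ending overlap with its Box triggers a turn.
; Tick rotates it at a speed derived from RotateTime, tracking the accumulated angle and backing out any overshoot past 90 degrees.
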(event OnComponentEndOverlap(Box)
  (params (OverlappedComponent :type Primitive%20Component%20Object%20Reference) (OtherActor :type Actor%20Object%20Reference) (OtherComp :type Primitive%20Component%20Object%20Reference) (OtherBodyIndex :type Integer))
  (if (not (Variables|Platform|GetisAlways?))
    (if (not (Variables|Default|GetisRotating?))
      (Utilities|Casting|CastToHumanCharacter OtherActor
        (:then
          (Variables|Default|SetDeltaRot 0.0 :!label _label)
          (Variables|Default|SetisRotating? true))
        (:CastFailed
          (bind _asdog_character (Utilities|Casting|CastToDogCharacter OtherActor))
          (if (not (Variables|/Game/Blueprints/Characters/DogCharacter.DogCharacter_C|GetisPicked _asdog_character))
            (goto _label)))))))

(event EventBeginPlay
  (Variables|Default|SetSpeed (/ 9e+01 (Variables|Platform|GetRotateTime)))
  (Variables|Default|SetTime (Variables|Platform|GetInterval)))

(event EventTick
  (params (DeltaSeconds :type Float%20%28single-precision%29))
  (CallFunction|RotatePlatform)
  (CallFunction|ChangeTime))

(fn ConstructionScript
  (Rendering|Material|SetMaterial (Variables|Default|GetCube) 0 (Variables|Platform|GetMaterial)))

(fn RotatePlatform
  (bind _returnvalue (Utilities|Time|GetWorldDeltaSeconds))
  (bind _speed (Variables|Default|GetSpeed))
  (bind _returnvalue_2 (* _speed _returnvalue))
  (if (Variables|Default|GetisRotating?)
    (Variables|Default|SetDeltaRot (+ (Variables|Default|GetDeltaRot) _returnvalue_2))
    (Transformation|AddActorLocalRotation (Math|Rotator|MakeRotator 0.0 _returnvalue_2 0.0) false false)
    (if (>= (Math|Float|Absolute(Float) (Variables|Default|GetDeltaRot)) 9e+01)
      (Variables|Default|SetisRotating? false)
      (Transformation|AddActorLocalRotation (Math|Rotator|MakeRotator 0.0 (* (- (Variables|Default|GetDeltaRot) 9e+01) -1.0) 0.0) false false))))

(fn ChangeTime
  (if (not (Variables|Default|GetisRotating?))
    (bind _output_get (Variables|Default|SetTime (Math|Float|Clamp(Float) (- (Variables|Default|GetTime) (Utilities|Time|GetWorldDeltaSeconds)) 0.0 123.0)))
    (if (and (Variables|Platform|GetisAlways?) (<= _output_get 0.0))
      (Variables|Default|SetisRotating? true)
      (Variables|Default|SetDeltaRot 0.0)
      (Variables|Default|SetTime (Variables|Platform|GetInterval)))))