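; Blinking 2D platform that alternates between visible with query-only collision and hidden with no collision.
; SetOnline and SetOffline schedule each other by timer, using separate online and offline durations, so the cycle runs without Tick.
; The IsOn flag gates that scheduling, so an optional start delay holds the initial state until DelayEnd starts the cycle.
; The construction script applies the configurable sprite.
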(event EventBeginPlay
  (if (Variables|Platform|GethasDelay?)
    (Utilities|Time|SetTimerbyFunctionName 0 "DelayEnd" (Variables|Platform|GetDelay))
    (else
      (Variables|Default|SetIsOn? true)))
  (if (Variables|Platform|GetisOnline)
    (CallFunction|SetOnline)
    (else
      (CallFunction|SetOffline))))

(event Collision|EventActorBeginOverlap
  (params (OtherActor :type Actor%20Object%20Reference)))

(event EventTick
  (params (DeltaSeconds :type Float%20%28single-precision%29)))

(fn ConstructionScript
  (Rendering|Components|Sprite|SetSprite (Variables|Default|GetPaperSprite) (Variables|Platform|GetSprite)))

(fn SetOnline
  (bind _papersprite (Variables|Default|GetPaperSprite))
  (Development|SetHiddeninGame _papersprite false false)
  (Collision|SetCollisionEnabled _papersprite "QueryOnly")
  (Variables|Platform|SetisOnline true)
  (if (Variables|Default|GetIsOn?)
    (Utilities|Time|SetTimerbyFunctionName 0 "SetOffline" (Variables|Platform|GetOnlineTime))))

(fn SetOffline
  (bind _papersprite (Variables|Default|GetPaperSprite))
  (Development|SetHiddeninGame _papersprite true false)
  (Collision|SetCollisionEnabled _papersprite "NoCollision")
  (Variables|Platform|SetisOnline false)
  (if (Variables|Default|GetIsOn?)
    (Utilities|Time|SetTimerbyFunctionName 0 "SetOnline" (Variables|Platform|GetOfflineTime))))

(fn DelayEnd
  (Variables|Default|SetIsOn? true)
  (if (Variables|Platform|GetisOnline)
    (CallFunction|SetOnline)
    (else
      (CallFunction|SetOffline))))