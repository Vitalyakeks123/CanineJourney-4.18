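; A balance-scale platform that sinks toward its bottom position while the player stands on it, sending its linked Libra partner toward its top position.
; Each tick it checks for a grounded, overlapping player to set destinations, then moves at constant speed in X and Z.
; When neither linked platform is loaded, both destinations snap to their current locations, halting the pair.
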(event EventBeginPlay
  (if (Variables|Platform|GetisTop?)
    (Variables|Default|SetDestination (Variables|Platform|GetTopPosition))
    (else
      (Variables|Default|SetDestination (Variables|Platform|GetBotPosition)))))

(event Collision|EventActorBeginOverlap
  (params (OtherActor :type Actor%20Object%20Reference)))

(event EventTick
  (params (DeltaSeconds :type Float%20%28single-precision%29))
  (CallFunction|CheckOverlap)
  (CallFunction|MovePlatform DeltaSeconds))

(fn ConstructionScript
  (Rendering|Material|SetMaterial (Variables|Default|GetCube) 0 (Variables|Platform|GetMaterial))
  (Variables|Platform|SetStartPosition (Transformation|GetActorLocation)))

(fn MovePlatform
  (params (DeltaTime :type Float%20%28single-precision%29))
  (bind _returnvalue (Transformation|GetActorLocation))
  (bind _destination (Variables|Default|GetDestination))
  (bind _movespeed (Variables|Platform|GetMoveSpeed))
  (bind _returnvalue_2 (Class|KismetMathLibrary|Vector2DInterptoConstant (Math|Vector2D|MakeVector2D (.x _returnvalue) (.z _returnvalue)) (Math|Vector2D|MakeVector2D (.x _destination) (.z _destination)) DeltaTime _movespeed))
  (Transformation|SetActorLocation (Math|Vector|MakeVector (.x _returnvalue_2) 0.0 (.y _returnvalue_2)) false true))

(fn CheckOverlap
  (bind _returnvalue (Game|GetPlayerCharacter 0))
  (bind _libra (Variables|Platform|GetLibra))
  (bind _libra_2 (Variables|Platform|GetLibra))
  (if (and (Collision|IsOverlappingActor _returnvalue :!class /Script/Engine.Actor) (not (AI|Components|NavMovement|IsFalling (Variables|/Script/Engine.Character|GetCharacterMovement _returnvalue))))
    ;[1 1 1] Set isMoving
    (Variables|Default|SetDestination (Variables|Platform|GetBotPosition))
    (Variables|Default|SetisMoving? true)
    (Utilities|IsValid _libra_2
      (:Is%20Valid
        (Variables|LibraPlatform_C|SetDestination _libra_2 (Variables|LibraPlatform_C|GetTopPosition _libra_2))))
    (else
      (Variables|Default|SetisMoving? false)
      (Utilities|IsValid _libra
        (:Is%20Valid
          (if (not (Variables|LibraPlatform_C|GetisMoving? _libra))
            (Variables|Default|SetDestination (Transformation|GetActorLocation))
            (Variables|LibraPlatform_C|SetDestination _libra (Transformation|GetActorLocation _libra))))))))