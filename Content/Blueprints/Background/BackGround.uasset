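; Paper2D sprite background actor that creates parallax by shifting relative to camera movement, scaled by an offset multiplier.
; GetPlayerCamera caches the first PlayersCamera's position as the baseline.
; MoveWithOffset teleports by the passed actor's scaled delta, with Z scaling optional, then updates that baseline.
; The construction script applies the sprite and previews the offset; Tick is empty, and MoveToNextLocation's timed-move values feed only dead MovingBg code.
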(event Custom|MoveToNextLocation
  (params (CameraBlock :type Camera%20Block%20Object%20Reference) (Time :type Float%20%28single-precision%29))
  (bind _returnvalue (Transformation|GetActorLocation))
  (bind _returnvalue_2 (Transformation|GetActorLocation CameraBlock))
  (bind _offsetmultiplier (Variables|Background|GetOffSetMultiplier))
  (bind _returnvalue_3 (- (.x _returnvalue_2) (.x _returnvalue)))
  (bind _returnvalue_4 (- (.z _returnvalue_2) (.z _returnvalue)))
  (bind _returnvalue_5 (* _returnvalue_4 _offsetmultiplier))
  (bind _returnvalue_6 (* _returnvalue_3 _offsetmultiplier))
  (Variables|Default|SetMoveTime Time)
  (Variables|Default|SetMoveSpeedX (/ _returnvalue_6 (Variables|Default|GetMoveTime)))
  (Variables|Default|SetMoveSpeedZ (/ _returnvalue_5 (Variables|Default|GetMoveTime)))
  (Variables|Default|SetMoveToLocationX (+ (.x _returnvalue) _returnvalue_6))
  (Variables|Default|SetMoveToLocationZ (+ _returnvalue_5 (.z _returnvalue)))
  (Variables|Default|SetisMoving? true))

(event Custom|MoveWithOffset
  (params (Actor :type Actor%20Object%20Reference))
  (bind _returnvalue (Transformation|GetActorLocation Actor))
  (bind _returnvalue_2 (Transformation|GetActorLocation))
  (bind _offsetmultiplier (Variables|Background|GetOffSetMultiplier))
  ;[1 1 1] Move With Offset
  (Utilities|IsValid Actor
    (:Is%20Valid
      (Utilities|FlowControl|Sequence
        (:then_0
          (if (Variables|Background|GetisMovingZ?)
            (Transformation|Teleport (Math|Vector|MakeVector (- (.x _returnvalue_2) (* (- (.x (Variables|Default|GetPlayerPosition)) (.x _returnvalue)) _offsetmultiplier)) (.y _returnvalue_2) (+ (.z _returnvalue_2) (* (- (.z _returnvalue) (.z (Variables|Default|GetPlayerPosition))) _offsetmultiplier))) "0, 0, 0")
            (else
              (Transformation|Teleport (Math|Vector|MakeVector (- (.x _returnvalue_2) (* (- (.x (Variables|Default|GetPlayerPosition)) (.x _returnvalue)) _offsetmultiplier)) (.y _returnvalue_2) (+ (- (.z _returnvalue) (.z (Variables|Default|GetPlayerPosition))) (.z _returnvalue_2))) "0, 0, 0"))))
        (:then_1
          (Variables|Default|SetPlayerPosition (Transformation|GetActorLocation Actor)))))))

(event EventBeginPlay
  (CallFunction|GetPlayerCamera))

(event EventTick
  (params (DeltaSeconds :type Float%20%28single-precision%29)))

(fn ConstructionScript
  (bind _cameraoffset (Variables|Background|GetCameraOffset))
  (Rendering|Components|Sprite|SetSprite (Variables|Default|GetPaperSprite) (Variables|Background|GetSprite))
  (Utilities|IsValid _cameraoffset
    (:Is%20Valid
      (CallFunction|GetPlayerCamera)
      (CallFunction|MovewithOffset _cameraoffset))))

(fn MovingBg
  (bind _returnvalue (Game|GetPlayerController 0))
  (bind _returnvalue_2 (Viewport|GetViewportSize))
  (bind _returnvalue_3 (/ (.x _returnvalue_2) 2.0))
  (bind _returnvalue_4 (/ (.y _returnvalue_2) 2.0))
  (bind _worldlocation (Class|PlayerController|DeprojectScreenPositiontoWorld _returnvalue _returnvalue_3 _returnvalue_4))
  (Transformation|Teleport (Math|Vector|MakeVector (.x _worldlocation) -1e+02 (.z _worldlocation)) "0, 0, 0"))

(fn GetPlayerCamera
  (bind _outactors (Actor|GetAllActorsOfClass "/Game/Blueprints/Camera/PlayersCamera.PlayersCamera_C"))
  (bind _output_get (Variables|Default|SetPlayerReference (Utilities|Array|Get(acopy) _outactors)))
  (Variables|Default|SetPlayerPosition (Transformation|GetActorLocation _output_get)))