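; Player camera actor that carries static background sprites and drives the movement of scene background actors.
; The construction script assigns two configurable sprites to its StaticBackground components.
; The MoveBG event finds every BackGround actor and calls MoveWithOffset on each, passing the camera as reference.
; BeginPlay, overlap and Tick are unused, so background movement happens only when MoveBG is called.
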(event Custom|MoveBG
  (bind _outactors (Actor|GetAllActorsOfClass "/Game/Blueprints/Background/BackGround.BackGround_C"))
  (for _array_element _outactors
    (Default|MovewithOffset _array_element self)))

(event EventBeginPlay)

(event Collision|EventActorBeginOverlap
  (params (OtherActor :type Actor%20Object%20Reference)))

(event EventTick
  (params (DeltaSeconds :type Float%20%28single-precision%29)))

(fn ConstructionScript
  (Rendering|Components|Sprite|SetSprite (Variables|Default|GetStaticBackground) (Variables|Default|GetSprite1))
  (Rendering|Components|Sprite|SetSprite (Variables|Default|GetStaticBackground2) (Variables|Default|GetSprite2)))